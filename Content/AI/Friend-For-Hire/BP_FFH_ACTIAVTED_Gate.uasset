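; Gate actor in the Friend-For-Hire AI folder that can be activated to open.
; On BeginPlay it runs the parent logic and adds an activated gameplay tag to its tag container.
; Its OpenGate events set an OpeningGate flag and hide the actor in game, with no collision change or movement in this graph.
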(event `self.ReceiveBeginPlay`
  (`parent.ReceiveBeginPlay`)
  (`BlueprintGameplayTagLibrary.AddGameplayTag` (`self.TagContainer`) (`self.ActivatedTag`)))

(event `OpenGate`
  (set `self.OpeningGate` true))

(event `/Game/AI/Friend-For-Hire/BPI_FFH_Collect.open gate`
  (`self.SetActorHiddenInGame` true))

(fn `UserConstructionScript`
  (`parent.UserConstructionScript`))