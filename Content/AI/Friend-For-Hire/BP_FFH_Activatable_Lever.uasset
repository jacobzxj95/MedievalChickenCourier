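; BP_FFH_Activatable_Lever is a lever in the Friend-For-Hire folder that triggers a cutscene and moves a gate.
; It tags itself on BeginPlay; its custom event adds Lever.Activated, prints the hit actor and plays the YeOleWinterTon level sequence.
; After a delay, it teleports the first BP_FFH_ACTIAVTED_Gate found to a hardcoded location.
; Per-gate tag queries are unfinished and never run, so gate parameters are ignored.
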(event `self.ReceiveBeginPlay`
  (`BlueprintGameplayTagLibrary.AddGameplayTag` (`self.TagContainer`) (`self.LeverRefTag`)))

(event `Find Correct gate, apply change`
  (params (NewParam :type "GameplayTag Structure") (Gate2 :type "GameplayTag Structure") (`Hit actor` :type "Actor Object Reference"))
  (`KismetSystemLibrary.PrintString` (`KismetSystemLibrary.GetDisplayName` `Hit actor`))
  (`BlueprintGameplayTagLibrary.AddGameplayTag` (`self.TagContainer`) (struct :`TagName` "Lever.Activated"))
  (bind (_outactor _returnvalue) (`LevelSequencePlayer.CreateLevelSequencePlayer` "/Game/AI/Friend-For-Hire/LVL_Sequence_YeOleWinterTon.LVL_Sequence_YeOleWinterTon"))
  (`MovieSceneSequencePlayer.Play` _returnvalue)
  (`MovieSceneSequencePlayer.Play` (`LevelSequenceActor.SequencePlayer` _outactor))
  (`KismetSystemLibrary.Delay` 5.0)
  (bind _returnvalue_2 (`GameplayStatics.GetActorOfClass` "/Game/AI/Friend-For-Hire/BP_FFH_ACTIAVTED_Gate.BP_FFH_ACTIAVTED_Gate_C"))
  (`self.K2_SetActorLocation` _returnvalue_2 (9240.988281 4421.838867 793.570251) false false))

(fn `UserConstructionScript`)