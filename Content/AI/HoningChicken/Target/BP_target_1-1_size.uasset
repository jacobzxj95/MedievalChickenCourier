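; BP_target_1-1_size is a target actor that rewards hits from the honing chicken and hands control back to the main player character.
; When BP_AI_HoningChicken overlaps the Target component, it sends 75 to the game mode's currency message.
; It then hides the chicken and current player character, disables the latter's collision and possesses BP_PlayerChar.
; A DoOnce gates the sequence and resets at its end.
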(event `self.Target.OnComponentBeginOverlap`
  (params (OverlappedComponent :type "PrimitiveComponent Object Reference") (OtherActor :type "Actor Object Reference") (OtherComp :type "PrimitiveComponent Object Reference") (OtherBodyIndex :type Integer) (bFromSweep :type Boolean) (SweepResult :type "HitResult Structure (by ref)"))
  (if (== (`GameplayStatics.GetObjectClass` OtherActor) "/Game/AI/AICharacters/BP_AI_HoningChicken.BP_AI_HoningChicken_C")
    (`/Engine/EditorBlueprintResources/StandardMacros.DoOnce` false :!label _label
      (:`Completed`
        (message `/Game/Utility/Interfaces/BPI_UI.UpdateCurrency` (`GameplayStatics.GetGameMode`) 75)
        (`self.SetActorHiddenInGame` OtherActor true)
        (`self.SetActorHiddenInGame` (`GameplayStatics.GetPlayerCharacter` 0) true)
        (`self.SetActorEnableCollision` (`GameplayStatics.GetPlayerCharacter` 0) false)
        (bind _returnvalue (`GameplayStatics.GetActorOfClass` "/Game/Characters/BP_PlayerChar.BP_PlayerChar_C"))
        (`Controller.Possess` (`GameplayStatics.GetPlayerController` 0) _returnvalue)
        (goto _label :!via `Reset`)))))

(fn `UserConstructionScript`)