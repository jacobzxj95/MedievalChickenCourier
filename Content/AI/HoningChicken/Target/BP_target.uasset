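; BP_target is a hit target for the Honing Chicken that rewards currency feedback and progress when struck.
; When TargetCollision overlaps an exact BP_AI_HoningChicken, it sends Currency to the game mode's message update and spawns confetti at the target.
; It then raises the percentage bar on the chicken found by GetActorOfClass, rather than the overlapping actor.
; Disconnected quest, UI-message, hiding and possession-swap logic never runs.
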(event `self.ReceiveTick`
  (params (DeltaSeconds :type "Float (single-precision)")))

(event `self.Target.OnComponentBeginOverlap`
  (params (OverlappedComponent :type "PrimitiveComponent Object Reference") (OtherActor :type "Actor Object Reference") (OtherComp :type "PrimitiveComponent Object Reference") (OtherBodyIndex :type Integer) (bFromSweep :type Boolean) (SweepResult :type "HitResult Structure (by ref)")))

(event `self.Target Collision.OnComponentBeginOverlap`
  (params (OverlappedComponent :type "PrimitiveComponent Object Reference") (OtherActor :type "Actor Object Reference") (OtherComp :type "PrimitiveComponent Object Reference") (OtherBodyIndex :type Integer) (bFromSweep :type Boolean) (SweepResult :type "HitResult Structure (by ref)"))
  (if (== (`GameplayStatics.GetObjectClass` OtherActor) "/Game/AI/AICharacters/BP_AI_HoningChicken.BP_AI_HoningChicken_C")
    (message `/Game/Utility/Interfaces/BPI_UI.UpdateCurrency` (`GameplayStatics.GetGameMode`) (`self.Currency`))
    (`NiagaraFunctionLibrary.SpawnSystemAtLocation` "/Game/Art/VFX/VFX_Confetti.VFX_Confetti" (`self.K2_GetActorLocation`) (`self.K2_GetActorRotation`) (2.0 2.0 2.0))
    (bind _returnvalue (`GameplayStatics.GetActorOfClass` "/Game/AI/AICharacters/BP_AI_HoningChicken.BP_AI_HoningChicken_C"))
    (`/Engine/EditorBlueprintResources/StandardMacros.IsValid` _returnvalue
      (:`Is Valid`
        (`/Game/AI/AICharacters/BP_AI_HoningChicken.raise percentage bar` _returnvalue))
      (:`Is Not Valid`
        (`KismetSystemLibrary.PrintString` "Honing Chicken Ref ISN\"T VALID")))))

(event `self.ReceiveBeginPlay`)

(fn `UserConstructionScript`)