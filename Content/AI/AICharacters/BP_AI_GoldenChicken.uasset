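; Golden chicken AI character, a carryable quest item that extends its parent's pickup, drop and throw events.
; Pickup shows a UI message after a short delay, cleared on drop or throw; first pickup also rings church bells, starts intense music and signals the quest component.
; While stationary, it messages a villager every Tick, and thieves leaving its pickup overlap get a message.
; Its mechanic explanation popup pauses the game but describes a Pushback Chicken.
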(event `self.ReceiveBeginPlay`
  (`parent.ReceiveBeginPlay`)
  (bind _asbp_game_instance (cast `/Game/Utility/GameModes/BP_GameInstance` (`GameplayStatics.GetGameInstance`)))
  (set `self.As BP Game Instance` _asbp_game_instance))

(event `self.ReceiveTick`
  (params (DeltaSeconds :type "Float (single-precision)"))
  (`parent.ReceiveTick` DeltaSeconds)
  (if (== (`KismetMathLibrary.VSize` (`self.GetVelocity`)) 0.0)
    (bind _returnvalue (`GameplayStatics.GetActorOfClass` "/Game/Characters/BP_Villager.BP_Villager_C"))
    (`/Engine/EditorBlueprintResources/StandardMacros.IsValid` _returnvalue
      (:`Is Valid`
        (message `/Game/AI/BPI/BPI_Player_Chicken_interactions.HasGoldenChicken` _returnvalue)))))

(event `/Game/Utility/Interfaces/BPI_EPS.ItemPickedUp`
  (params (CurrentChicken :type "Actor Object Reference") (`CapturingChicken?` :type Boolean) (`HasChicken?` :type Boolean))
  (`parent.ItemPickedUp` CurrentChicken `CapturingChicken?` `HasChicken?`)
  (`KismetSystemLibrary.Delay` 0.1)
  (message `/Game/Utility/Interfaces/BPI_UI.TurnOnUI` (`GameplayStatics.GetGameMode`) "NewEnumerator12")
  (`/Engine/EditorBlueprintResources/StandardMacros.DoOnce` false
    (:`Completed`
      (`GameplayStatics.PlaySoundAtLocation` "/Game/SFX/QuestRelated/SC_ChurchBells.SC_ChurchBells" (`self.ChurchBellSoundLoc`) (struct) 1.0 1.0 0.0 null null null null)
      (bind _as_bp_game_instance (`self.As BP Game Instance`)
        (:`then`
          (`/Game/Utility/GameModes/BP_GameInstance.PlayIntenseMusic` _as_bp_game_instance)
          (`/Game/Components/ActorComponents/AC_Questitem.Send ID` (`self.AC_Questitem`) 0))
        (:`else`)))))

(event `/Game/Utility/Interfaces/BPI_EPS.ItemDropped`
  (params (DropLocation :type "Vector Structure"))
  (`parent.ItemDropped` DropLocation)
  (message `/Game/Utility/Interfaces/BPI_UI.TurnOffUI` (`GameplayStatics.GetGameMode`) "NewEnumerator12"))

(event `/Game/Utility/Interfaces/BPI_EPS.ItemThrown`
  (params (ThrowingForce :type "Float (double-precision)") (ThrowingDirection :type "Vector Structure") (StartingTransform :type "Transform Structure") (`CatapultLaunched?` :type Boolean) (StunDuration :type "Float (double-precision)"))
  (`parent.ItemThrown` ThrowingForce ThrowingDirection StartingTransform false 0.0)
  (message `/Game/Utility/Interfaces/BPI_UI.TurnOffUI` (`GameplayStatics.GetGameMode`) "NewEnumerator12"))

(event `self.Pickup.OnComponentEndOverlap`
  (params (OverlappedComponent :type "PrimitiveComponent Object Reference") (OtherActor :type "Actor Object Reference") (OtherComp :type "PrimitiveComponent Object Reference") (OtherBodyIndex :type Integer))
  (if (== (`GameplayStatics.GetObjectClass` OtherActor) "/Game/Characters/BP_Thief.BP_Thief_C")
    (message `/Game/AI/BPI/BPI_Player_Chicken_interactions.PickupChicken` OtherActor)))

(fn `Mechanic Explnation`
  (bind _returnvalue (`GameplayStatics.GetPlayerController` 0))
  (bind _returnvalue_2 (`|CreateWidget` "/Game/UI/W_LevelExplaination.W_LevelExplaination_C" _returnvalue))
  (set `/Game/UI/W_LevelExplaination.InputText` "This is a Pushback Chicken! Press the Right mouse button to activate a pushback effect that will knockback and stun nearby Thieves and Villagers. This ability can only be activated after your cooldown is up, so use it wisely!" _returnvalue_2)
  (`UserWidget.AddToViewport` _returnvalue_2 0)
  (`WidgetBlueprintLibrary.SetInputMode_UIOnlyEx` _returnvalue _returnvalue_2)
  (set `PlayerController.bShowMouseCursor` true _returnvalue)
  (`GameplayStatics.SetGamePaused` true))

(fn `UserConstructionScript`
  (`parent.UserConstructionScript`))