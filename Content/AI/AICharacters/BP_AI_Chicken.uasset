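; AI chicken character that runs BT_Chicken, flees to random points, and can be picked up, dropped, thrown or catapulted as a quest item.
; Pickup and release toggle movement, collision, the BeingHeld blackboard key and the quest waypoint icon, which a timer also hides by player distance.
; Thrown impacts trigger timeline squash-and-stretch scaled by hit normal and force.
; Catapulted hits on destructible shutters spawn a Chaos master field to break them.
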(event `self.ReceiveBeginPlay`
  (bind _returnvalue (`AIBlueprintHelperLibrary.GetAIController` (`self.GetOwner`)))
  ;[1 1 1] enable sensing updates
  (`parent.ReceiveBeginPlay`)
  (`/Engine/EditorBlueprintResources/StandardMacros.IsValid` _returnvalue
    (:`Is Valid`
      (`AIController.RunBehaviorTree` _returnvalue "/Game/AI/Trees/BT_Chicken.BT_Chicken")
      (bind _output_get (`/Game/Components/ActorComponents/AC_Questitem.CreateWidget` (`self.AC_Questitem`)))
      (`/Game/UI/Icons/W_MainObjectiveIcon.TurnOnObjectiveIcon` _output_get 2)
      (`WidgetComponent.SetWidget` (`self.Widget`) _output_get)
      (set `self.StartingScale` (`SceneComponent.RelativeScale3D` (`self.ChickenMesh`)))
      (if (`KismetArrayLibrary.Array_IsNotEmpty` (`self.Pre-GivenArray`))
        (set `/Game/Components/ActorComponents/AC_Questitem.ActorQuestIDS` (`self.Pre-GivenArray`) (`self.AC_Questitem`))
        (`/Game/Components/ActorComponents/AC_Questitem.On Off Waypoint` (`self.AC_Questitem`) (`self.Widget`) true)))))

(event `self.ReceiveTick`
  (params (DeltaSeconds :type "Float (single-precision)"))
  (bind _tags (`self.Tags`))
  (`parent.ReceiveTick` DeltaSeconds)
  ;[1 0.4158 0.9033] Add and remove the "Held" tag to/from the chicken depending on if it is picked up or not
  (if (`self.CratedChicken?`)
    (`|ExecutionSequence`
      (:`then_0`
        (`/Engine/EditorBlueprintResources/StandardMacros.DoOnce` false :!label _label
          (:`Completed`
            (bind _returnvalue (`KismetArrayLibrary.Array_Add` _tags))
            (`KismetArrayLibrary.Array_Set` (`self.Tags`) _returnvalue (`self.HeldTag`)))))
      (:`then_1`
        (goto _label_2 :!via `Reset`)))
    (else
      (`|ExecutionSequence`
        (:`then_0`
          (goto _label :!via `Reset`))
        (:`then_1`
          (`/Engine/EditorBlueprintResources/StandardMacros.DoOnce` false :!label _label_2
            (:`Completed`
              (`KismetArrayLibrary.Array_Remove` _tags (`KismetArrayLibrary.Array_LastIndex` _tags)))))))))

(event `Run From Player`
  ;[1 1 1] Charecter Spotted
  (if (not (`self.Isbeingheld?`))
    (`|AIMoveTo` self (`NavigationSystemV1.K2_GetRandomReachablePointInRadius` (`self.K2_GetActorLocation`) 2500.0 null null) null 5.0 true)))

(event `/Game/Utility/Interfaces/BPI_EPS.ItemPickedUp`
  (params (CurrentChicken :type "Actor Object Reference") (`CapturingChicken?` :type Boolean) (`HasChicken?` :type Boolean))
  ;[0 1 0.05664] Picked Up Interface
  (`AudioComponent.Stop` (`self.WingFlap`))
  (set `self.CratedChicken?` `CapturingChicken?`)
  (set `self.IsThrown` false)
  (`CharacterMovementComponent.SetMovementMode` (`self.CharacterMovement`) "MOVE_None" 0)
  (`/Engine/EditorBlueprintResources/StandardMacros.IsValid` (`AIBlueprintHelperLibrary.GetAIController` self)
    (:`Is Valid`
      (`self.SetActorEnableCollision` false)
      (`BlackboardComponent.SetValueAsBool` (`AIBlueprintHelperLibrary.GetBlackboard` (`AIBlueprintHelperLibrary.GetAIController` self)) "BeingHeld" true)
      (set `self.Isbeingheld?` true)
      (`self.Quest Enabled Waypoint Change` true)
      (`/Engine/EditorBlueprintResources/StandardMacros.DoOnce` false
        (:`Completed`
          (`/Game/Components/ActorComponents/AC_Questitem.Send ID` (`self.AC_Questitem`) 0))))))

(event `/Game/Utility/Interfaces/BPI_EPS.ItemDropped`
  (params (DropLocation :type "Vector Structure"))
  ;[0 1 0.05664] Upon Drop
  (`self.K2_SetActorLocation` DropLocation)
  (`CharacterMovementComponent.SetMovementMode` (`self.CharacterMovement`) "MOVE_Walking" 0)
  (`self.SetActorEnableCollision` true)
  (set `self.Isbeingheld?` false)
  (`BlackboardComponent.SetValueAsBool` (`AIBlueprintHelperLibrary.GetBlackboard` (`AIBlueprintHelperLibrary.GetAIController` self)) "BeingHeld" false)
  (`self.Run From Player`)
  (`GameplayStatics.PlaySoundAtLocation` "/Game/SFX/ChickenSounds/SFX_Animal_Chicken_Cluck_1.SFX_Animal_Chicken_Cluck_1" (`self.K2_GetActorLocation`) (struct) 1.0 1.0 0.0 null null null null)
  (`self.Quest Enabled Waypoint Change` false))

(event `StartOverlappingActorsTimer`
  ;[1 1 1] If the chicken falls into quicksand stop its wing flapping sound
  (bind _returnvalue (`KismetSystemLibrary.K2_SetTimerDelegate` (delegate `CheckOverlappingActors`) 0.1 true :!label _label_3))
  (set `self.OverlappingActorsTimerHandle` _returnvalue))

(event `/Game/Utility/Interfaces/BPI_EPS.ItemThrown`
  (params (ThrowingForce :type "Float (double-precision)") (ThrowingDirection :type "Vector Structure") (StartingTransform :type "Transform Structure") (`CatapultLaunched?` :type Boolean) (StunDuration :type "Float (double-precision)"))
  ;[0 1 0.05664] Thrown Interface
  (set `self.ThrowingForce` ThrowingForce)
  (bind _output_get (set `self.Catapult Launched?` `CatapultLaunched?`))
  (if (not _output_get)
    (`AudioComponent.Play` (`self.WingFlap`) 0.0)
    (else
      (bind _returnvalue (`GameplayStatics.SpawnSoundAttached` "/Game/SFX/ChickenSounds/SC_LaunchedChicken.SC_LaunchedChicken" (`self.ChickenMesh`) "None" (0.0 0.0 0.0) (struct) "KeepRelativeOffset" false 1.0 1.0 0.0 null null))
      (set `self.ChickenLaunchedSound` _returnvalue)))
  (`self.K2_DetachFromActor` "KeepWorld" "KeepWorld" "KeepWorld")
  (`CharacterMovementComponent.SetMovementMode` (`self.CharacterMovement`) "MOVE_Falling" 0)
  (`self.K2_SetActorLocation` (.location StartingTransform))
  (set `self.IsThrown` true)
  (`self.LaunchCharacter` (* ThrowingDirection ThrowingForce) true true)
  (`self.SetActorEnableCollision` true)
  (bind _niagara (`self.Niagara`)
    (:`then`
      (`NiagaraComponent.SetVariableVec3` _niagara "Wind Speed" (* (* (`self.GetActorForwardVector`) -1.0) 2000.0))
      (`ActorComponent.SetActive` (`self.Niagara`) true false))
    (:`else`
      _))
  (`self.Quest Enabled Waypoint Change` false)
  (goto _label_3))

(event `CheckOverlappingActors`
  ;[1 1 1] If the chicken falls into quicksand stop its wing flapping sound
  (for _array_element (`self.GetOverlappingActors` "/Script/Engine.Actor") :!label _label_4
    (if (== (`GameplayStatics.GetObjectClass` _array_element) "/Game/LevelObjects/LevelMechanics/BP_Quicksand.BP_Quicksand_C")
      (`AudioComponent.FadeOut` (`self.WingFlap`) 2.0 0.0 "Linear")
      (`self.BreakOverlappingActorSearch`)))
  (if (not (> (`KismetMathLibrary.VSize` (`MovementComponent.Velocity` (`self.CharacterMovement`))) 10.0))
    (`KismetSystemLibrary.K2_ClearAndInvalidateTimerHandle` (`self.OverlappingActorsTimerHandle`))))

(event `BreakOverlappingActorSearch`
  ;[1 1 1] If the chicken falls into quicksand stop its wing flapping sound
  (goto _label_4 :!via `Break`))

(event `self.OnLanded`
  (params (Hit :type "HitResult Structure (by ref)"))
  (`BlackboardComponent.SetValueAsBool` (`AIBlueprintHelperLibrary.GetBlackboard` (`AIBlueprintHelperLibrary.GetAIController` self)) "BeingHeld" false)
  (`self.K2_SetActorRotation` (struct))
  (`AudioComponent.Stop` (`self.WingFlap`))
  (set `self.IsThrown` false))

(event `SquashNStretch`
  (bind _charactermovement (`self.CharacterMovement`))
  (bind (_hitnormal_x _hitnormal_y _hitnormal_z) (`KismetMathLibrary.BreakVector` (`self.HitNormal`)))
  (bind _returnvalue (or (> _hitnormal_y 0.5) (< _hitnormal_y -0.5)))
  (bind _returnvalue_2 (or (> _hitnormal_x 0.5) (< _hitnormal_x -0.5)))
  ;[1 1 1] SquashAndStretch
  (`self.ResetNiagara`)
  (set `CharacterMovementComponent.GravityScale` 0.0 _charactermovement)
  (set `MovementComponent.Velocity` (0.0 0.0 0.0) _charactermovement)
  (set `self.IsThrown` false)
  (`GameplayStatics.PlaySoundAtLocation` "/Game/SFX/ChickenSounds/SC_ChickenSquash.SC_ChickenSquash" (`self.K2_GetActorLocation`) (struct) 1.0 1.0 0.0 null null null null)
  (set `self.EndingScale` (+ (`self.StartingScale`) (* (`KismetMathLibrary.MakeVector` (`KismetMathLibrary.SelectFloat` -0.4 0.0 (or _returnvalue _returnvalue_2)) (`KismetMathLibrary.SelectFloat` 0.4 0.0 (or _returnvalue_2 _returnvalue)) (`KismetMathLibrary.SelectFloat` -0.4 0.0 (or (> _hitnormal_z 0.5) (< _hitnormal_z -0.5)))) (`KismetMathLibrary.FClamp` (/ (`self.ThrowingForce`) 1250.0) 0.1))))
  (bind (_direction _alpha) (`Timeline|SquashAndStretch` :!via `PlayFromStart`)
    (:`Update`
      (`SceneComponent.SetRelativeScale3D` (`self.ChickenMesh`) (`KismetMathLibrary.VLerp` (`self.StartingScale`) (`self.EndingScale`) _alpha)))
    (:`Finished`
      (set `CharacterMovementComponent.GravityScale` 1.0 (`self.CharacterMovement`)))))

(event `/Game/Utility/Interfaces/BPI_Quest.TurnOnWaypoints`
  (params (ObjectiveID :type String) (`On/Off` :type Boolean))
  (bind _output_get (set `self.On/ Off` `On/Off`))
  (`KismetSystemLibrary.PrintString` (`KismetStringLibrary.Concat_StrStr` (`KismetSystemLibrary.GetDisplayName` self) "  " (`KismetStringLibrary.Conv_BoolToString` _output_get)))
  (`/Game/Components/ActorComponents/AC_Questitem.Check To Turn On Waypoints` (`self.AC_Questitem`) (`self.Widget`) _output_get ObjectiveID)
  (bind _returnvalue (`KismetSystemLibrary.K2_SetTimerDelegate` (delegate `CheckDistanceToPlayer`) 0.2 true))
  (set `self.IconDistanceToPlayerTimer` _returnvalue)
  (bind _asbp_player_char (cast `/Game/Characters/BP_PlayerChar` (`GameplayStatics.GetPlayerCharacter` 0)))
  (set `self.PlayerChar_Ref` _asbp_player_char))

(event `CheckDistanceToPlayer`
  (bind _widget (`self.Widget`))
  ;[0.05524 0.4612 1] If the player is far from the chicken, hide its icon
  (if (`self.On/ Off`)
    (bind _playerchar_ref (`self.PlayerChar_Ref`)
      (:`then`
        (if (> (`KismetMathLibrary.Vector_Distance` (`self.K2_GetActorLocation`) (`self.K2_GetActorLocation` _playerchar_ref)) 2700.0)
          (`SceneComponent.SetHiddenInGame` _widget true false)
          (else
            (`SceneComponent.SetHiddenInGame` _widget false false))))
      (:`else`))
    (else
      (`KismetSystemLibrary.K2_ClearAndInvalidateTimerHandle` (`self.IconDistanceToPlayerTimer`)))))

(event `ResetNiagara`
  (bind _niagara (`self.Niagara`))
  ;[1 1 1] SquashAndStretch
  (`SceneComponent.SetVisibility` _niagara false false)
  (`NiagaraComponent.ResetSystem` _niagara))

(event `self.ReceiveHit`
  (params (MyComp :type "PrimitiveComponent Object Reference") (Other :type "Actor Object Reference") (OtherComp :type "PrimitiveComponent Object Reference") (bSelfMoved :type Boolean) (HitLocation :type "Vector Structure") (HitNormal :type "Vector Structure") (NormalImpulse :type "Vector Structure") (Hit :type "HitResult Structure (by ref)"))
  (bind (_bblockinghit _binitialoverlap _time _distance _location _impactpoint _normal _impactnormal) (`GameplayStatics.BreakHitResult` Hit))
  (bind _returnvalue_location (`KismetMathLibrary.BreakTransform` (`KismetMathLibrary.Conv_VectorToTransform` _impactpoint)))
  ;[0.0582 0.05294 1] Chaos Damage for destroying objects like the wooden shutters in Coastalton.
  (set `self.HitNormal` HitNormal)
  (set `self.HitLocation` (`.ImpactPoint` (`GameplayStatics.BreakHitResult` Hit)))
  (if (`self.IsThrown`)
    (`self.SquashNStretch`))
  (`self.StartOverlappingActorsTimer`)
  (if (== (`GameplayStatics.GetObjectClass` Other) "/Game/LevelObjects/BP_DestructibleShutters.BP_DestructibleShutters_C")
    (if (`self.Catapult Launched?`)
      (bind _chickenlaunchedsound (`self.ChickenLaunchedSound`)
        (:`then`
          (`AudioComponent.Stop` _chickenlaunchedsound)
          (`GameplayStatics.PlaySoundAtLocation` "/Game/SFX/ChickenSounds/SC_ChickenBark.SC_ChickenBark" (`self.K2_GetActorLocation`) (struct) 1.0 1.0 0.3 null null null null)
          (bind _returnvalue (`|SpawnActorFromClass` "/Engine/EditorResources/FieldNodes/FS_MasterField.FS_MasterField_C" (`KismetMathLibrary.MakeTransform` (+ _returnvalue_location (* _impactnormal -3.0)) (struct) (0.7 0.7 0.7)) "Undefined" "OverrideRootScale" null null))
          (bind _output_get (set `self.MasterField_Ref` _returnvalue))
          (set `/Engine/EditorResources/FieldNodes/FS_MasterField.ActivationType` "NewEnumerator4" _output_get)
          (set `/Engine/EditorResources/FieldNodes/FS_MasterField.FieldLifespan` 0.1 _output_get)
          (set `/Engine/EditorResources/FieldNodes/FS_MasterField.Radial Magnitude` 10.0 _output_get)
          (`/Engine/EditorResources/FieldNodes/FS_MasterField.CE_Trigger` _output_get)
          (`/Engine/EditorBlueprintResources/StandardMacros.DoOnce` false :!label _label_5
            (:`Completed`
              (`GameplayStatics.PlaySoundAtLocation` "/Game/SFX/Mechanics/Catapult/SC_ShortExplosion.SC_ShortExplosion" (`self.K2_GetActorLocation`) (struct) 1.0 1.0 0.0 null null null null)
              (set `self.Catapult Launched?` false)
              (`KismetSystemLibrary.Delay` 0.1)
              (`self.ResetExplosionSound`))))
        (:`else`)))))

(event `ResetExplosionSound`
  ;[0.0582 0.05294 1] Chaos Damage for destroying objects like the wooden shutters in Coastalton.
  (goto _label_5 :!via `Reset`))

(fn `Quest Enabled Waypoint Change`
  (params (OnOff :type Boolean))
  (if (`/Game/Components/ActorComponents/AC_Questitem.IsQuestEnabled` (`self.AC_Questitem`))
    (if OnOff
      (`SceneComponent.SetHiddenInGame` (`self.Widget`) true false)
      (else
        (`SceneComponent.SetHiddenInGame` (`self.Widget`) false false))))
  (return))

(fn `UserConstructionScript`
  (`parent.UserConstructionScript`))