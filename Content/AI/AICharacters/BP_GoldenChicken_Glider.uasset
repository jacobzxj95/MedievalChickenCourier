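; Glider variant of the golden chicken pickup, with wing-flap feedback while the player carries it through the air.
; On pickup it hides its icon, plays church bells once and starts a looping timer that checks whether the player is falling.
; DoOnce gates switch WingFlap on and off as that state changes, and the timer clears after a drop or throw.
; Overlapping the courier wagon also hides the icon.
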(event `self.ReceiveBeginPlay`
  (`parent.ReceiveBeginPlay`))

(event `self.ReceiveTick`
  (params (DeltaSeconds :type "Float (single-precision)"))
  (`parent.ReceiveTick` DeltaSeconds))

(event `/Game/Utility/Interfaces/BPI_EPS.ItemPickedUp`
  (params (CurrentChicken :type "Actor Object Reference") (`CapturingChicken?` :type Boolean) (`HasChicken?` :type Boolean))
  (`parent.ItemPickedUp` CurrentChicken `CapturingChicken?` `HasChicken?`)
  (`SceneComponent.SetVisibility` (`self.ChickenIcon`) false false)
  (`|ExecutionSequence`
    (:`then_0`
      (`/Engine/EditorBlueprintResources/StandardMacros.DoOnce` false
        (:`Completed`
          (`GameplayStatics.PlaySoundAtLocation` "/Game/SFX/QuestRelated/SC_ChurchBells.SC_ChurchBells" (`self.WintertonBellLoc`) (struct) 1.0 1.0 0.0 null null null null)
          (bind _asbp_player_char (cast `/Game/Characters/BP_PlayerChar` (`GameplayStatics.GetPlayerCharacter` 0)))
          (set `self.PlayerChar_Ref` _asbp_player_char))))
    (:`then_1`
      (set `self.IsHeld?` true)
      (bind _returnvalue (`KismetSystemLibrary.K2_SetTimerDelegate` (delegate `IsGliding?`) 0.1 true))
      (set `self.IsGlidingTimerHandle` _returnvalue))))

(event `IsGliding?`
  (bind _wingflap (`self.WingFlap`))
  (if (`self.IsHeld?`)
    (bind _playerchar_ref (`self.PlayerChar_Ref`)
      (:`then`
        (if (`NavMovementComponent.IsFalling` (`Character.CharacterMovement` _playerchar_ref))
          (`|ExecutionSequence`
            (:`then_0`
              (`/Engine/EditorBlueprintResources/StandardMacros.DoOnce` false :!label _label
                (:`Completed`
                  (`AudioComponent.Play` _wingflap 0.0))))
            (:`then_1`
              (goto _label_2 :!via `Reset`)))
          (else
            (`|ExecutionSequence`
              (:`then_0`
                (goto _label :!via `Reset`))
              (:`then_1`
                (`/Engine/EditorBlueprintResources/StandardMacros.DoOnce` false :!label _label_2
                  (:`Completed`
                    (`AudioComponent.Stop` _wingflap))))))))
      (:`else`))
    (else
      (`KismetSystemLibrary.K2_ClearAndInvalidateTimerHandle` (`self.IsGlidingTimerHandle`)))))

(event `/Game/Utility/Interfaces/BPI_EPS.ItemDropped`
  (params (DropLocation :type "Vector Structure"))
  (`parent.ItemDropped` DropLocation)
  (set `self.IsHeld?` false))

(event `/Game/Utility/Interfaces/BPI_EPS.ItemThrown`
  (params (ThrowingForce :type "Float (double-precision)") (ThrowingDirection :type "Vector Structure") (StartingTransform :type "Transform Structure") (`CatapultLaunched?` :type Boolean) (StunDuration :type "Float (double-precision)"))
  (`parent.ItemThrown` ThrowingForce ThrowingDirection StartingTransform false 0.0)
  (set `self.IsHeld?` false))

(event `self.Pickup.OnComponentBeginOverlap`
  (params (OverlappedComponent :type "PrimitiveComponent Object Reference") (OtherActor :type "Actor Object Reference") (OtherComp :type "PrimitiveComponent Object Reference") (OtherBodyIndex :type Integer) (bFromSweep :type Boolean) (SweepResult :type "HitResult Structure (by ref)"))
  (if (== OtherActor (`GameplayStatics.GetPlayerPawn` 0))
    _
    (elif (== (`GameplayStatics.GetObjectClass` OtherActor) "/Game/LevelObjects/BP_CourierWagon.BP_CourierWagon_C")
      (`SceneComponent.SetHiddenInGame` (`self.ChickenIcon`) true false))))

(event `self.Pickup.OnComponentEndOverlap`
  (params (OverlappedComponent :type "PrimitiveComponent Object Reference") (OtherActor :type "Actor Object Reference") (OtherComp :type "PrimitiveComponent Object Reference") (OtherBodyIndex :type Integer))
  (if (== (`GameplayStatics.GetObjectClass` OtherActor) "/Game/LevelObjects/BP_CourierWagon.BP_CourierWagon_C")
    (`SceneComponent.SetHiddenInGame` (`self.ChickenIcon`) false false)))

(fn `UserConstructionScript`
  (`parent.UserConstructionScript`))