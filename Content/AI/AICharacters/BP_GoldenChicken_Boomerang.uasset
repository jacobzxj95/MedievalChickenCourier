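; Throwable golden chicken AI character that flies like a boomerang back toward the player.
; While thrown, Tick drives flying movement, turning toward the instigator with forward projectile velocity and mesh spin, then after a delay issues an AI move to the player.
; Pickup and overlaps stop flight, BeingHeld syncs to the blackboard, and dropping turns every BP_Thief into a villager.
; Curve-path helpers and the explanation popup are unused.
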(event `self.ReceiveTick`
  (params (DeltaSeconds :type "Float (single-precision)"))
  (bind _mesh (`self.Mesh`))
  (`parent.ReceiveTick` DeltaSeconds)
  (if (`self.IsThrown`)
    (if (`self.movingAway`)
      (bind _asbp_player_char (cast `/Game/Characters/BP_PlayerChar` (`GameplayStatics.GetPlayerCharacter` 0)))
      (`/Game/Characters/BP_PlayerChar.ClearArc` _asbp_player_char)
      (`CharacterMovementComponent.SetMovementMode` (`self.CharacterMovement`) "MOVE_Flying" 0)
      (`self.K2_SetActorRotation` (`KismetMathLibrary.RInterpTo_Constant` (`self.K2_GetActorRotation` self) (`KismetMathLibrary.FindLookAtRotation` (`self.K2_GetActorLocation` self) (`self.K2_GetActorLocation` (`self.GetInstigator`))) DeltaSeconds 200.0) true)
      (set `MovementComponent.Velocity` (* (`self.GetActorForwardVector`) 1000.0) (`self.ProjectileMovement`))
      (`SceneComponent.K2_AddRelativeRotation` _mesh (struct :`Yaw` 30.0) false false)
      (`KismetSystemLibrary.Delay` 5.0)
      (set `self.movingAway` false)
      (`MovementComponent.StopMovementImmediately` (`self.ProjectileMovement`))
      (`SceneComponent.K2_AddRelativeRotation` :`self` _mesh)
      (else
        (`MovementComponent.StopMovementImmediately` (`self.ProjectileMovement`))
        (if (not (`self.movingAway`))
          (`self.Return to player`)
          (set `self.movingAway` true))))))

(event `self.ChickenMesh.OnComponentBeginOverlap`
  (params (OverlappedComponent :type "PrimitiveComponent Object Reference") (OtherActor :type "Actor Object Reference") (OtherComp :type "PrimitiveComponent Object Reference") (OtherBodyIndex :type Integer) (bFromSweep :type Boolean) (SweepResult :type "HitResult Structure (by ref)"))
  (if (== (`GameplayStatics.GetObjectClass` OtherActor) (`GameplayStatics.GetPlayerCharacter` 0))
    (set `self.IsThrown` false)
    (`BlackboardComponent.SetValueAsBool` (`AIBlueprintHelperLibrary.GetBlackboard` (`AIBlueprintHelperLibrary.GetAIController` self)) "BeingHeld" true)))

(event `/Game/Utility/Interfaces/BPI_EPS.ItemThrown`
  (params (ThrowingForce :type "Float (double-precision)") (ThrowingDirection :type "Vector Structure") (StartingTransform :type "Transform Structure") (`CatapultLaunched?` :type Boolean) (StunDuration :type "Float (double-precision)"))
  (`parent.ItemThrown` ThrowingForce ThrowingDirection StartingTransform `CatapultLaunched?` 0.0)
  (set `self.IsThrown` true)
  (set `self.movingAway` true)
  (bind _asbp_player_char (cast `/Game/Characters/BP_PlayerChar` (`GameplayStatics.GetPlayerCharacter` 0)))
  (`/Game/Characters/BP_PlayerChar.RemoveProjectilePath` _asbp_player_char))

(event `/Game/Utility/Interfaces/BPI_EPS.ItemPickedUp`
  (params (CurrentChicken :type "Actor Object Reference") (`CapturingChicken?` :type Boolean) (`HasChicken?` :type Boolean))
  (`parent.ItemPickedUp` CurrentChicken `CapturingChicken?` `HasChicken?`)
  (set `self.movingAway` false)
  (set `self.IsThrown` false)
  (`MovementComponent.StopMovementImmediately` (`self.ProjectileMovement`))
  (`CharacterMovementComponent.SetMovementMode` (`self.CharacterMovement`) "MOVE_None" 0))

(event `/Game/Utility/Interfaces/BPI_EPS.ItemDropped`
  (params (DropLocation :type "Vector Structure"))
  (`parent.ItemDropped` DropLocation)
  (set `self.IsThrown` false)
  (`BlackboardComponent.SetValueAsBool` (`AIBlueprintHelperLibrary.GetBlackboard` (`AIBlueprintHelperLibrary.GetAIController` self)) "BeingHeld" false)
  (bind _outactors (`GameplayStatics.GetAllActorsOfClass` "/Game/Characters/BP_Thief.BP_Thief_C"))
  (for _array_element _outactors
    (`/Game/Characters/BP_Thief.Thief Becomes Villager` _array_element)))

(event `self.Pickup.OnComponentBeginOverlap`
  (params (OverlappedComponent :type "PrimitiveComponent Object Reference") (OtherActor :type "Actor Object Reference") (OtherComp :type "PrimitiveComponent Object Reference") (OtherBodyIndex :type Integer) (bFromSweep :type Boolean) (SweepResult :type "HitResult Structure (by ref)"))
  (if (== (`GameplayStatics.GetObjectClass` OtherActor) (`GameplayStatics.GetPlayerCharacter` 0))
    (`MovementComponent.StopMovementImmediately` (`self.ProjectileMovement`))
    (`CharacterMovementComponent.SetMovementMode` (`self.CharacterMovement`) "MOVE_Falling" 0)
    (`|ExecutionSequence`
      (:`then_0`
        (`/Engine/EditorBlueprintResources/StandardMacros.DoOnce` false))
      (:`then_1`
        (set `self.IsThrown` false)
        (`self.Reset Projectile Movement`)))))

(fn `Curve Control Point`
  (bind (_x _y) (`KismetMathLibrary.BreakRotIntoAxes` (`KismetMathLibrary.FindLookAtRotation` (`self.MidPoint`) (`self.Target Location`))))
  (set `self.Curved Point` (+ (`self.MidPoint`) (`KismetMathLibrary.RotateAngleAxis` (* (`KismetMathLibrary.RandomFloatInRange` (`self.Min Curve Radius`) (`self.Max Curve Radius`)) _y) (`KismetMathLibrary.RandomFloatInRange` (`self.Min Angle`) (`self.Max angle`)) _x)))
  (return))

(fn `Curve Mid Point`
  (set `self.MidPoint` (+ (* (- (`self.Target Location`) (`self.K2_GetActorLocation`)) (`KismetMathLibrary.RandomFloatInRange` (`self.Min Curve Distance Point`) (`self.Max Curve Distance Point`))) (`self.K2_GetActorLocation`))))

(fn `Get Location`
  (params (u :type "Vector Structure") (t :type "Float (double-precision)"))
  (returns (location :type "Vector Structure"))
  (return (+ (* u t) (0.0 0.0 0.0) (0.0 0.0 0.0) (* 0.5 (`MovementComponent.GetGravityZ` (`self.CharacterMovement`)) t t))))

(fn `Line Trace For Curve Locations`
  (bind _returnvalue (`self.K2_GetActorLocation`))
  (bind _outhit (`KismetSystemLibrary.LineTraceSingleForObjects` _returnvalue (* _returnvalue (`KismetMathLibrary.GetForwardVector` (`self.K2_GetActorRotation`))) (`|MakeArray` "ObjectTypeQuery1" :!type "EObjectTypeQuery Enum") false (`|MakeArray` self :!type "Actor Object Reference")))
  (bind (_bblockinghit _binitialoverlap _time _distance _location _impactpoint _normal _impactnormal _physmat _hitactor _hitcomponent _hitbonename _bonename _hititem _elementindex _faceindex _tracestart _traceend) (`GameplayStatics.BreakHitResult` _outhit))
  (set `self.Target Location` (`KismetMathLibrary.SelectVector` _location _traceend)))

(fn `MechanicExplnation`
  (bind _returnvalue (`GameplayStatics.GetPlayerController` 0))
  (bind _returnvalue_2 (`|CreateWidget` "/Game/UI/W_LevelExplaination.W_LevelExplaination_C" _returnvalue))
  (set `/Game/UI/W_LevelExplaination.InputText` (`self.Mechanic Text`) _returnvalue_2)
  (`UserWidget.AddToViewport` _returnvalue_2 0)
  (`WidgetBlueprintLibrary.SetInputMode_UIOnlyEx` _returnvalue _returnvalue_2)
  (set `PlayerController.bShowMouseCursor` true _returnvalue)
  (`GameplayStatics.SetGamePaused` true))

(fn `Reset Projectile Movement`
  (bind _projectilemovement (`self.ProjectileMovement`))
  (`ProjectileMovementComponent.ResetInterpolation` _projectilemovement)
  (`MovementComponent.StopMovementImmediately` _projectilemovement)
  (`CharacterMovementComponent.SetMovementMode` (`self.CharacterMovement`) "MOVE_None" 0))

(fn `Return to player`
  (`AIController.MoveToLocation` (`AIBlueprintHelperLibrary.GetAIController` self) (`self.K2_GetActorLocation` (`GameplayStatics.GetPlayerCharacter` 0)) -1.0 true false false false null true))

(fn `UserConstructionScript`
  (`parent.UserConstructionScript`))