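; Animation notify that plays surface-dependent footstep sounds for the Thief AI character.
; On notify, it line-traces 200 units down from the owning actor's location on the Visibility channel.
; The hit's physical surface type selects a matching sound cue, played at the actor's location, with small cobblestone roads reusing the stone cue.
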(fn `Received_Notify`
  (params (MeshComp :type "SkeletalMeshComponent Object Reference") (Animation :type "AnimSequenceBase Object Reference") (EventReference :type "AnimNotifyEventReference Structure (by ref)"))
  (returns (ReturnValue :type Boolean))
  (bind _returnvalue (`ActorComponent.GetOwner` MeshComp))
  (bind _returnvalue_2 (`Actor.K2_GetActorLocation` _returnvalue))
  (bind (_outhit _returnvalue_3) (`KismetSystemLibrary.LineTraceSingle` _returnvalue_2 (+ _returnvalue_2 (* (`Actor.GetActorUpVector` _returnvalue) -200.0)) "TraceTypeQuery1"))
  (if _returnvalue_3
    (switch `EPhysicalSurface` (`GameplayStatics.GetSurfaceType` _outhit)
      (:`SurfaceType1`
        (`GameplayStatics.PlaySoundAtLocation` "/Game/SFX/CharacterSounds/Footsteps/Grass/SC_Footsteps_Grass.SC_Footsteps_Grass" _returnvalue_2 (struct) 1.0 1.0 0.0 null null null null))
      (:`SurfaceType2`
        (`GameplayStatics.PlaySoundAtLocation` "/Game/SFX/CharacterSounds/Footsteps/Stone_Rock/SC_FootSteps_Stone.SC_FootSteps_Stone" _returnvalue_2 (struct) 1.0 1.0 0.0 null null null null))
      (:`SurfaceType3`
        (`GameplayStatics.PlaySoundAtLocation` "/Game/SFX/CharacterSounds/Footsteps/Gravel_LooseRock/SC_Footsteps_Gravel.SC_Footsteps_Gravel" _returnvalue_2 (struct) 1.0 1.0 0.0 null null null null))
      (:`SurfaceType4`
        (`GameplayStatics.PlaySoundAtLocation` "/Game/SFX/CharacterSounds/Footsteps/Sand/SC_Footsteps_Sand.SC_Footsteps_Sand" _returnvalue_2 (struct) 1.0 1.0 0.0 null null null null))
      (:`SurfaceType5`
        (`GameplayStatics.PlaySoundAtLocation` "/Game/SFX/CharacterSounds/Footsteps/Dirt/SC_Footsteps_Dirt.SC_Footsteps_Dirt" _returnvalue_2 (struct) 1.0 1.0 0.0 null null null null))
      (:`SurfaceType6`
        (`GameplayStatics.PlaySoundAtLocation` "/Game/SFX/CharacterSounds/Footsteps/Water/SC_Footsteps_Water.SC_Footsteps_Water" _returnvalue_2 (struct) 1.0 1.0 0.0 null null null null))
      (:`SurfaceType7`
        (`GameplayStatics.PlaySoundAtLocation` "/Game/SFX/CharacterSounds/Footsteps/Mud/SC_Footsteps_Mud.SC_Footsteps_Mud" _returnvalue_2 (struct) 1.0 1.0 0.0 null null null null))
      (:`SurfaceType8`
        (`GameplayStatics.PlaySoundAtLocation` "/Game/SFX/CharacterSounds/Footsteps/Wood/SC_Footsteps_Wood.SC_Footsteps_Wood" _returnvalue_2 (struct) 1.0 1.0 0.0 null null null null))
      (:`SurfaceType9`
        (`GameplayStatics.PlaySoundAtLocation` "/Game/SFX/CharacterSounds/Footsteps/Snow/ShallowSnow/SC_Footsteps_ShallowSnow.SC_Footsteps_ShallowSnow" _returnvalue_2 (struct) 1.0 1.0 0.0 null null null null))
      (:`SurfaceType10`
        (`GameplayStatics.PlaySoundAtLocation` "/Game/SFX/CharacterSounds/Footsteps/Leaves_Branches_Hay/SC_Footsteps_Leaves_Hay_Branches.SC_Footsteps_Leaves_Hay_Branches" _returnvalue_2 (struct) 1.0 1.0 0.0 null null null null))
      (:`SurfaceType11`
        (`GameplayStatics.PlaySoundAtLocation` "/Game/SFX/CharacterSounds/Footsteps/Snow/DeepSnow/SC_DeepSnow.SC_DeepSnow" _returnvalue_2 (struct) 1.0 1.0 0.0 null null null null))
      (:`SurfaceType12`
        (`GameplayStatics.PlaySoundAtLocation` "/Game/SFX/CharacterSounds/Footsteps/Ice/SC_IceFootsteps.SC_IceFootsteps" _returnvalue_2 (struct) 1.0 1.0 0.0 null null null null))
      (:`SurfaceType13`
        (`GameplayStatics.PlaySoundAtLocation` "/Game/SFX/CharacterSounds/Footsteps/Stone_Rock/SC_FootSteps_Stone.SC_FootSteps_Stone" _returnvalue_2 (struct) 1.0 1.0 0.0 null null null null)))
    (return false)))