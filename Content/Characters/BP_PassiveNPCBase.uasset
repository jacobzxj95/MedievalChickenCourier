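; BP_PassiveNPCBase is a passive NPC base Blueprint that handles the start and end of player interactions.
; On start, it stores the player character and, if ShouldMoveCamera is set, blends the view to itself, notifies the player and hides a UI message.
; Ending unconditionally notifies the player, returns the view to them and restores the message.
; QuestInteraction is a stub returning an empty string.
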(event `/Game/Utility/Interfaces/BPI_Interaction.InteractionStarted`
  (params (PlayerCharacter :type "/Game/Characters/BP_PlayerChar Object Reference") (HeldObject :type "Actor Object Reference"))
  ;[1 1 1] InteractionStarted
  (set `self.PlayerCharacter` PlayerCharacter)
  (if (`self.ShouldMoveCamera`)
    (`PlayerController.SetViewTargetWithBlend` (`GameplayStatics.GetPlayerController` 0) self 1.2 "VTBlend_Linear" 0.0 false)
    (`/Game/Characters/BP_PlayerChar.Interaction Start/ Ended` (`self.PlayerCharacter`) true)
    (message `/Game/Utility/Interfaces/BPI_UI.TurnOffUI` (`GameplayStatics.GetGameMode`) "NewEnumerator0")))

(event `/Game/Utility/Interfaces/BPI_Interaction.InteractionEnded`
  (bind _playercharacter (`self.PlayerCharacter`))
  ;[1 1 1] Ending Interaction
  (`/Game/Characters/BP_PlayerChar.Interaction Start/ Ended` _playercharacter false)
  (`PlayerController.SetViewTargetWithBlend` (`GameplayStatics.GetPlayerController` 0) _playercharacter 0.0 "VTBlend_Linear" 0.0 false)
  (message `/Game/Utility/Interfaces/BPI_UI.TurnOnUI` (`GameplayStatics.GetGameMode`) "NewEnumerator0"))

(fn `QuestInteraction`
  (returns (ObjectiveID :type String))
  (return ""))

(fn `UserConstructionScript`)