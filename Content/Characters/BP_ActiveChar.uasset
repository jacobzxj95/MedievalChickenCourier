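; BP_ActiveChar is a character that holds one item, such as a chicken or chicken crate, and supports stealing and handing it over.
; When stolen from, it detaches any Chicken-tagged item, messages the stealer with it and briefly sets a recently-robbed flag, cleared by timer.
; When receiving, it snaps the item to a crate or chicken mesh socket, playing a sound for non-crates.
; GiveItem releases and returns the held item.
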(event `ResetRecentlyStolenFrom`
  (set `self.WasRecentlyStolenFrom` false))

(event `/Game/Utility/Interfaces/BPI_Stealing.UpdateStolen`
  (params (`Who'sStealing` :type "Actor Object Reference"))
  ;[1 1 1] Stealing
  (`self.UpdateWhenStolen` `Who'sStealing`))

(event `/Game/Utility/Interfaces/BPI_Stealing.UpdateStealer`
  (params (ItemStolen :type "Actor Object Reference"))
  ;[1 1 1] Stealing
  (`self.UpdateWhenStealing` ItemStolen))

(fn `GiveItem`
  (returns (TempCurrentItem1 :type "Actor Object Reference"))
  (locals (TempCurrentItem :type "Actor Object Reference"))
  (bind _current_item (`self.Current Item`)
    (:`then`
      (`self.K2_DetachFromActor` _current_item "KeepWorld" "KeepRelative" "KeepWorld")
      (set `local.TempCurrentItem` (`self.Current Item`))
      (set `self.Current Item` null)
      (set `self.Is Holding?` false)
      (return (`local.TempCurrentItem`)))
    (:`else`)))

(fn `UpdateWhenStealing`
  (params (ObjectStolen :type "Actor Object Reference"))
  (set `self.Current Item` ObjectStolen)
  (set `self.Is Holding?` true)
  (if (!= (`GameplayStatics.GetObjectClass` ObjectStolen) "/Game/LevelObjects/BP_ChickenCrate.BP_ChickenCrate_C")
    (`self.K2_AttachToComponent` (`self.Current Item`) (`self.Mesh`) "ChickenLoc" "SnapToTarget" "SnapToTarget" "KeepWorld" true)
    (`GameplayStatics.PlaySoundAtLocation` (`self.WhenStealing`) (`self.K2_GetActorLocation`) (struct) 1.0 1.0 0.0 null null null null)
    (else
      (`self.K2_AttachToComponent` (`self.Current Item`) (`self.Mesh`) "ChickenCrate" "SnapToTarget" "SnapToTarget" "KeepWorld" true))))

(fn `UpdateWhenStolen`
  (params (TheStealer :type "Object Object Reference"))
  (bind _current_item (`self.Current Item`))
  (`/Engine/EditorBlueprintResources/StandardMacros.IsValid` _current_item
    (:`Is Valid`
      (if (`self.ActorHasTag` _current_item "Chicken")
        (`self.K2_DetachFromActor` (`self.Current Item`) "KeepRelative" "KeepRelative" "KeepRelative")
        (message `/Game/Utility/Interfaces/BPI_Stealing.UpdateStealer` TheStealer (`self.Current Item`))
        (set `self.Current Item` null)
        (set `self.Is Holding?` false)
        (`GameplayStatics.PlaySoundAtLocation` (`self.WhenStolenFromSound`) (`self.K2_GetActorLocation`) (struct) 1.0 1.0 0.0 null null null null)
        (set `self.WasRecentlyStolenFrom` true)
        (`KismetSystemLibrary.K2_SetTimer` null "ResetRecentlyStolenFrom" 0.1)))))

(fn `UserConstructionScript`)