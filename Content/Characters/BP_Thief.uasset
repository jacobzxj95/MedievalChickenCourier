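; BP_Thief is an AI character that steals chickens from the player and carries them to the nearest BP_ThiefChickenReturn.
; It starts as a villager and becomes a hooded, faster thief on stealing, swapping mesh, AnimBP and blackboard flag.
; BT_Thief and pawn sensing drive it, while overlaps and AI moves handle stealing, grabbing thrown chickens and delivery, retrying failed turn-ins.
; Stuns make it release its chicken and pause before behaviors resume.
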(event `self.ReceiveBeginPlay`
  ;[0.4603 0.54 0 1 162] Collapsed nodes for thief states
  ;;[1 0.451 0.4627 1 82] On Begin Play, run behaviors
  (`self.Thief_Becomes_Villager` self)
  (`self.RunBehaviorTree,enablesenseing`)
  (bind _outactors (`GameplayStatics.GetAllActorsOfClass` "/Game/LevelObjects/BP_ThiefChickenReturn.BP_ThiefChickenReturn_C"))
  (bind _output_get (set `self.BP Thief Chicken Return Array` _outactors))
  (set `self.Startng Turnin Array` _output_get)
  (bind _outactors_2 (`GameplayStatics.GetAllActorsOfClass` "/Game/AI/AICharacters/BP_AI_Chicken.BP_AI_Chicken_C"))
  (set `self.BP AI Chickens` _outactors_2))

(event `Stunned BY Pushback`
  (bind _current_item (`self.Current Item`))
  ;[0.4603 0.54 0 1 162] Collapsed nodes for thief states
  ;;[1 0.451 0.4627 1 202] STUNNED
  ;;;[1 0.451 0.4627 1 40] Stunned BY Pushback
  (`/Engine/EditorBlueprintResources/StandardMacros.IsValid` _current_item
    (:`Is Valid`
      (`self.K2_DetachFromActor` _current_item "KeepRelative" "KeepRelative" "KeepRelative")
      (message `/Game/Utility/Interfaces/BPI_EPS.ItemDropped` _current_item (`self.K2_GetActorLocation`))
      (set `self.Current Item` null)
      (set `self.Is Holding?` false)
      (set `CharacterMovementComponent.MaxWalkSpeed` 0.0 (`self.CharacterMovement`))
      (`SceneComponent.SetHiddenInGame` (`self.StunnedWidget`) false false)
      (`GameplayStatics.PlaySoundAtLocation` "/Game/SFX/CharacterSounds/Theif/SC_HitSounds.SC_HitSounds" (`self.K2_GetActorLocation`) (struct) 0.75 1.0 0.0 null null null null)
      (`KismetSystemLibrary.Delay` 3.0)
      (set `CharacterMovementComponent.MaxWalkSpeed` 475.0 (`self.CharacterMovement`)))))

(event `Stunned`
  (bind _current_item (`self.Current Item`))
  ;[0.4603 0.54 0 1 162] Collapsed nodes for thief states
  ;;[1 0.451 0.4627 1 202] STUNNED
  ;;;[1 0.451 0.4627 1 40] Stunned State
  (`self.PlayAnimMontage` "/Game/Art/CharecterAnimations/AnimSequences/Thieves/Stunned/AM_DizzyIdle.AM_DizzyIdle")
  (set `self.IsStunned?` true)
  (`/Engine/EditorBlueprintResources/StandardMacros.IsValid` _current_item
    (:`Is Valid`
      (`SceneComponent.SetHiddenInGame` (`self.ChickenIcon`) true false)
      (`self.K2_DetachFromActor` _current_item "KeepRelative" "KeepRelative" "KeepRelative")
      (message `/Game/Utility/Interfaces/BPI_EPS.ItemThrown` _current_item 1000.0 (`self.GetActorForwardVector`) (`self.GetTransform`) false 0.0)
      (set `self.Current Item` null)
      (set `self.Is Holding?` false))
    (:`Is Not Valid`
      _))
  (set `CharacterMovementComponent.MaxWalkSpeed` 0.0 (`self.CharacterMovement`))
  (`SceneComponent.SetHiddenInGame` (`self.StunnedWidget`) false false)
  (`GameplayStatics.PlaySoundAtLocation` "/Game/SFX/CharacterSounds/Theif/SC_HitSounds.SC_HitSounds" (`self.K2_GetActorLocation`) (struct) 0.75 1.0 0.0 null null null null)
  (`KismetSystemLibrary.Delay` (`self.StunDuration`))
  (`self.StopAnimMontage` "/Game/Art/CharecterAnimations/AnimSequences/Thieves/Stunned/AM_DizzyIdle.AM_DizzyIdle")
  (set `self.StunDuration` 3.0)
  (set `CharacterMovementComponent.MaxWalkSpeed` 475.0 (`self.CharacterMovement`))
  (`SceneComponent.SetHiddenInGame` (`self.StunnedWidget`) true false)
  (set `self.IsStunned?` false)
  (`SceneComponent.SetHiddenInGame` (`self.ChickenIcon`) true false)
  (`self.Upon Stolen reset behaviors`))

(event `/Game/Utility/Interfaces/BPI_Hit.HitByProjectile`
  (params (StunDuration :type "Float (double-precision)"))
  ;[0.4603 0.54 0 1 162] Collapsed nodes for thief states
  ;;[1 0.451 0.4627 1 202] STUNNED
  ;;;[1 0.451 0.4627 1 40] BPI HIT
  (set `self.StunDuration` StunDuration)
  (`self.Stunned`))

(event `Upon Stolen reset behaviors`
  ;[0.4603 0.54 0 1 162] Collapsed nodes for thief states
  ;;[1 0.451 0.4627 1 202] STEALING
  ;;;[1 0.451 0.4627 1 34] when player has stolen chicken from thief
  (`AIBlueprintHelperLibrary.SimpleMoveToLocation` (`AIBlueprintHelperLibrary.GetAIController` self) (`NavigationSystemV1.K2_GetRandomReachablePointInRadius` (`self.K2_GetActorLocation`) 3000.0 null null))
  (`self.Reset return behavior`)
  (`SceneComponent.SetHiddenInGame` (`self.StunnedWidget`) true false)
  (`SceneComponent.SetHiddenInGame` (`self.ChickenIcon`) true false))

(event `self.Egg Loc Check.OnComponentBeginOverlap`
  (params (OverlappedComponent :type "PrimitiveComponent Object Reference") (OtherActor :type "Actor Object Reference") (OtherComp :type "PrimitiveComponent Object Reference") (OtherBodyIndex :type Integer) (bFromSweep :type Boolean) (SweepResult :type "HitResult Structure (by ref)"))
  ;[0.4603 0.54 0 1 162] Collapsed nodes for thief states
  ;;[1 0.451 0.4627 1 202] STEALING
  ;;;[1 0.451 0.4627 1 58] on overlap,run stealing checks
  (if (and (== OtherActor (`GameplayStatics.GetPlayerPawn` 0)) (not (`self.Is Holding?`)) (not (`self.IsStunned?`)))
    (message `/Game/Utility/Interfaces/BPI_Stealing.UpdateStolen` OtherActor self)
    (`KismetSystemLibrary.PrintString` "Hello")
    (elif (and (not (`self.Is Holding?`)) (`self.TryingToStealThrownChicken`) (== OtherActor (`self.Nearest Chicken`)))
      (set `self.TryingToStealThrownChicken` false)
      (message `/Game/Utility/Interfaces/BPI_EPS.ItemPickedUp` (`self.Nearest Chicken`) null false false)
      (`self.UpdateWhenStealing` (`self.Nearest Chicken`))
      (`KismetSystemLibrary.Delay` 0.2)
      (if (`self.Is Holding?`)
        (`self.Villager_Becomes_Thief`)
        (`self.Attempt chicken return, with interuptions`)))))

(event `self.Grab Thrown Chicken`
  (params (ChickenThrown :type "Actor Object Reference"))
  (bind _nearest_chicken (`self.Nearest Chicken`))
  ;[0.4603 0.54 0 1 162] Collapsed nodes for thief states
  ;;[1 0.451 0.4627 1 202] STEALING
  ;;;[1 0.451 0.4627 1 74] find and grab nearest chicken
  (bind _output_get (set `self.Nearest Chicken` ChickenThrown))
  (`/Engine/EditorBlueprintResources/StandardMacros.IsValid` _output_get
    (:`Is Valid`
      (if (<= (`self.GetDistanceTo` _output_get) 10000.0)
        (set `self.TryingToStealThrownChicken` true)
        (`KismetSystemLibrary.PrintString` (`KismetSystemLibrary.GetDisplayName` _nearest_chicken))
        (`|AIMoveTo` self (0.0 0.0 0.0) _nearest_chicken
          (:`OnSuccess`
            (set `self.TryingToStealThrownChicken` false)))))
    (:`Is Not Valid`
      (set `self.Nearest Chicken` null))))

(event `ChickenReturned`
  (bind _returnvalue (`AIBlueprintHelperLibrary.GetAIController` (`self.GetOwner`)))
  ;[0.4603 0.54 0 1 162] Collapsed nodes for thief states
  ;;[1 0.451 0.4627 1 98] STATE SWITCHES
  ;;;[1 0.451 0.4627 1 58] called from within "BP_ReturnChicken" sets thief behaviors to their previous state
  (`BlackboardComponent.SetValueAsBool` (`AIBlueprintHelperLibrary.GetBlackboard` _returnvalue) "ISHOLDINGCHICKEN" false)
  (`AIController.RunBehaviorTree` _returnvalue "/Game/AI/Trees/BT_Thief.BT_Thief")
  (`PawnSensingComponent.SetSensingUpdatesEnabled` (`self.AICPawnSensing`) true)
  (`SceneComponent.SetHiddenInGame` (`self.ChickenIcon`) true false)
  (`self.Upon Stolen reset behaviors`)
  (bind _outactors (`GameplayStatics.GetAllActorsOfClass` "BP_Thief_C"))
  (for _array_element _outactors
    (`self.Thief_Becomes_Villager` _array_element)))

(event `Attempt chicken return, with interuptions`
  (bind _selectthiefarrayelement (`self.SelectThiefArrayElement`))
  ;[0.4603 0.54 0 1 162] Collapsed nodes for thief states
  ;;[1 0.451 0.4627 1 202] STEALING
  ;;;[1 0.451 0.4627 1 42] move to nearest thrown or dropped chicken
  (`/Engine/EditorBlueprintResources/StandardMacros.DoOnce` false :!label _label
    (:`Completed`
      (`self.GetNearestThiefTurnin`)
      (`KismetSystemLibrary.PrintString` (`KismetSystemLibrary.GetDisplayName` _selectthiefarrayelement))
      (`AITask_MoveTo.AIMoveTo` (`AIBlueprintHelperLibrary.GetAIController` self) (0.0 0.0 0.0) _selectthiefarrayelement -1.0 "Default" "Disable" true true false "Enable"
        (:`OnRequestFailed`
          (`KismetArrayLibrary.Array_RemoveItem` (`self.BP Thief Chicken Return Array`) (`self.SelectThiefArrayElement`))
          (set `self.SelectThiefArrayElement` null)
          (`self.GetNearestThiefTurnin`)
          (`self.Reset return behavior`)
          (`self.Attempt chicken return, with interuptions`))
        (:`OnMoveFinished`
          (set `self.BP Thief Chicken Return Array` (`self.Startng Turnin Array`)))))))

(event `/Game/Utility/Interfaces/BPI_Stealing.UpdateStealer`
  (params (ItemStolen :type "Actor Object Reference"))
  ;[0.4603 0.54 0 1 162] Collapsed nodes for thief states
  ;;[1 0.451 0.4627 1 202] STEALING
  ;;;[1 0.451 0.4627 1 98] THIEF STEALS CHICKEN
  (`parent.UpdateStealer` ItemStolen)
  (`GameplayStatics.PlaySoundAtLocation` "/Game/SFX/ChickenSounds/ES_Chicken_Growl_-_SFX_Producer.ES_Chicken_Growl_-_SFX_Producer" (`self.K2_GetActorLocation`) (struct) 1.0 1.0 0.0 null null null null)
  (message `/Game/Utility/Interfaces/BPI_UI.TurnOffUI` (`GameplayStatics.GetGameMode`) "NewEnumerator2")
  (if (`self.Check for golden chicken ` ItemStolen)
    (message `/Game/Utility/Interfaces/BPI_UI.TurnOffUI` (`GameplayStatics.GetGameMode`) "NewEnumerator12"))
  (bind _outactors (`GameplayStatics.GetAllActorsOfClass` "BP_Thief_C"))
  (for _array_element _outactors
    (if (`/Game/Characters/BP_ActiveChar.Is Holding?` _array_element)
      (`self.Villager_Becomes_Thief` _array_element)
      (`self.Attempt chicken return, with interuptions`)
      (`AIController.RunBehaviorTree` (`AIBlueprintHelperLibrary.GetAIController` self) "/Game/AI/Trees/BT_Thief.BT_Thief")
      (`SceneComponent.SetHiddenInGame` (`self.ChickenIcon`) false false)
      (else
        (`self.Thief Becomes Villager` _array_element)))))

(event `self.Thief_Becomes_Villager`
  ;[0.4603 0.54 0 1 162] Collapsed nodes for thief states
  ;;[1 0.451 0.4627 1 98] STATE SWITCHES
  ;;;[1 0.451 0.4627 1 50] change thief to villager State
  (`self.Thief Becomes Villager`))

(event `Reset return behavior`
  ;[0.4603 0.54 0 1 162] Collapsed nodes for thief states
  ;;[1 0.451 0.4627 1 202] STEALING
  ;;;[1 0.451 0.4627 1 42] move to nearest thrown or dropped chicken
  (goto _label :!via `Reset`))

(event `self.Villager_Becomes_Thief`
  ;[0.4603 0.54 0 1 162] Collapsed nodes for thief states
  ;;[1 0.451 0.4627 1 98] STATE SWITCHES
  ;;;[1 0.451 0.4627 1 50] Reset to thief State
  (`self.Villager Becomes Thief`))

(event `/Game/Utility/Interfaces/BPI_Stealing.UpdateStolen`
  (params (`Who'sStealing` :type "Actor Object Reference"))
  ;[0.4603 0.54 0 1 162] Collapsed nodes for thief states
  ;;[1 0.451 0.4627 1 202] STEALING
  ;;;[1 0.451 0.4627 1 98] PLAYER STEALS CHICKEN
  (`parent.UpdateStolen` `Who'sStealing`)
  (if (`self.WasRecentlyStolenFrom`)
    (`self.Stunned`)
    (`SceneComponent.SetVisibility` (`self.ChickenIcon`) false false)))

(fn `BPI_PickupChicken`
  (params (ActorToGiveTo :type "Actor Object Reference")))

(fn `GetNearestThiefTurnin`
  (bind _bp_thief_chicken_return_array (`self.BP Thief Chicken Return Array`))
  (bind (_distance _returnvalue) (`GameplayStatics.FindNearestActor` (`self.K2_GetActorLocation` self) _bp_thief_chicken_return_array))
  (`/Engine/EditorBlueprintResources/StandardMacros.IsValid` (`self.SelectThiefArrayElement`)
    (:`Is Valid`
      (return))
    (:`Is Not Valid`
      (for _array_element _bp_thief_chicken_return_array
        (if (== _array_element _returnvalue)
          (set `self.SelectedThiefTurnin` _returnvalue)
          (break)))
      (set `self.SelectThiefArrayElement` _array_element)
      (return))))

(fn `RunBehaviorTree,enablesenseing`
  (returns (BlackboardComponent :type "BlackboardComponent Object Reference"))
  (bind _returnvalue (`AIBlueprintHelperLibrary.GetAIController` (`self.GetOwner`)))
  (bind _astheif_aic (cast `/Game/AI/AICharacters/Theif/Theif_AIC` _returnvalue)
    (:`then`
      (bind _blackboardcomponent (`AIController.UseBlackboard` _returnvalue "/Game/AI/BlackBoards/BB_ChickenAI.BB_ChickenAI"))
      (`AIController.RunBehaviorTree` _returnvalue "/Game/AI/Trees/BT_Thief.BT_Thief")
      (bind _pawnsensing (`/Game/AI/AIC/AIC_Base.PawnSensing` _astheif_aic))
      (`PawnSensingComponent.SetSensingUpdatesEnabled` _pawnsensing true)
      (set `self.AICPawnSensing` _pawnsensing)
      (return _blackboardcomponent))
    (:`CastFailed`
      (`KismetSystemLibrary.PrintText` "Wrong AIC for Thief set!" true true (struct :`R` 0.704167 :`B` 0.010588 :`A` 1.0)))))

(fn `SphereTraceforchicken`)

(fn `StealFromPlayer`
  (params (Object :type "Object Object Reference")))

(fn `Thief Becomes Villager`
  (bind _mesh (`self.Mesh`))
  (bind _returnvalue (`AIBlueprintHelperLibrary.GetBlackboard` (`AIBlueprintHelperLibrary.GetAIController` self)))
  (`SkeletalMeshComponent.SetSkeletalMeshAsset` _mesh "/Game/Meshes/Characters/Thief/HoodDown/thief_nohood__1_.thief_nohood__1_")
  (`SkeletalMeshComponent.SetAnimInstanceClass` _mesh "/Game/Art/CharecterAnimations/ABP_Thieves.ABP_Thieves_C")
  (`/Engine/EditorBlueprintResources/StandardMacros.IsValid` _returnvalue
    (:`Is Valid`
      (`BlackboardComponent.SetValueAsBool` _returnvalue "playerhaschicken" false)
      (set `CharacterMovementComponent.MaxWalkSpeed` 350.0 (`self.CharacterMovement`)))))

(fn `UpdateWhenStealing`
  (params (ObjectStolen :type "Actor Object Reference"))
  (`parent.UpdateWhenStealing` ObjectStolen))

(fn `UpdateWhenStolen`
  (params (TheStealer :type "Object Object Reference"))
  (`parent.UpdateWhenStolen` TheStealer))

(fn `UserConstructionScript`
  (`parent.UserConstructionScript`))

(fn `Villager Becomes Thief`
  (bind _mesh (`self.Mesh`))
  (`SkeletalMeshComponent.SetSkeletalMeshAsset` _mesh "/Game/Meshes/Characters/Thief/Hooded/thief_hood__1_.thief_hood__1_")
  (`SkeletalMeshComponent.SetAnimInstanceClass` _mesh "/Game/Art/CharecterAnimations/ABP_HoodedThieves.ABP_HoodedThieves_C")
  (`BlackboardComponent.SetValueAsBool` (`AIBlueprintHelperLibrary.GetBlackboard` (`AIBlueprintHelperLibrary.GetAIController` self)) "playerhaschicken" true)
  (set `CharacterMovementComponent.MaxWalkSpeed` 600.0 (`self.CharacterMovement`)))