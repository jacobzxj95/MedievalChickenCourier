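; Vendor character the player can interact with, which also introduces and spawns a hireable friend NPC.
; Interaction start and end extend parent logic by swapping game-mode UI messages.
; Escape blends the view target to the vendor and calls InteractionStartEnded on the player.
; SpawnIntoWorld runs once, spawning BP_Friend_for_hire at FFHSpawnLoc and, a second later, pausing the game behind an explanation widget.
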(event `Key|Escape`
  (params (Key :type "Key Structure"))
  (:`Pressed`
    (set `self.PlayerCharacterREF` (stale `/Game/Utility/Interfaces/BPI_Interaction.InteractionStarted` PlayerCharacter))
    (if true
      (`PlayerController.SetViewTargetWithBlend` (`GameplayStatics.GetPlayerController` 0) self 1.2 "VTBlend_Linear" 0.0 false)
      (`/Game/Characters/BP_PlayerChar.Interaction Start/ Ended` (`self.PlayerCharacterREF`) true)
      (message `/Game/Utility/Interfaces/BPI_UI.TurnOffUI` (`GameplayStatics.GetGameMode`) "NewEnumerator0"))))

(event `/Game/Utility/Interfaces/BPI_Interaction.InteractionStarted`
  (params (PlayerCharacter :type "/Game/Characters/BP_PlayerChar Object Reference") (HeldObject :type "Actor Object Reference"))
  (bind _returnvalue (`GameplayStatics.GetGameMode`))
  (`parent.InteractionStarted` PlayerCharacter null)
  (message `/Game/Utility/Interfaces/BPI_UI.TurnOnUI` _returnvalue "NewEnumerator3")
  (message `/Game/Utility/Interfaces/BPI_UI.TurnOffUI` _returnvalue "NewEnumerator0"))

(event `/Game/Utility/Interfaces/BPI_Interaction.InteractionEnded`
  (`parent.InteractionEnded`)
  (message `/Game/Utility/Interfaces/BPI_UI.TurnOnUI` (`GameplayStatics.GetGameMode`) "NewEnumerator0")
  (message `/Game/Utility/Interfaces/BPI_UI.TurnOffUI` (`GameplayStatics.GetGameMode`) "NewEnumerator3"))

(event `Spawn into world(Call in Editor)`)

(event `/Game/AI/Friend-For-Hire/BPI_Friend_For_Hire.Spawn into world`
  (bind _returnvalue (`GameplayStatics.GetPlayerController` 0))
  (`/Engine/EditorBlueprintResources/StandardMacros.DoOnce` false
    (:`Completed`
      (`|ExecutionSequence`
        (:`then_0`
          (`KismetSystemLibrary.Delay` 1.0)
          (bind _returnvalue_2 (`|CreateWidget` "/Game/UI/W_LevelExplaination.W_LevelExplaination_C" _returnvalue))
          (set `/Game/UI/W_LevelExplaination.InputText` (`self.Friend For hire Explnation`) _returnvalue_2)
          (`UserWidget.AddToViewport` _returnvalue_2 0)
          (`WidgetBlueprintLibrary.SetInputMode_UIOnlyEx` _returnvalue _returnvalue_2)
          (set `PlayerController.bShowMouseCursor` true _returnvalue)
          (`GameplayStatics.SetGamePaused` true))
        (:`then_1`
          (`GameplayStatics.GetActorOfClass` "BP_Vendor_C")
          (bind _returnvalue_3 (`|SpawnActorFromClass` "/Game/AI/AICharacters/BP_Friend_for_hire.BP_Friend_for_hire_C" (`SceneComponent.K2_GetComponentToWorld` (`self.FFH Spawn Loc`)) "Undefined" "OverrideRootScale" null null))
          (`/Engine/EditorBlueprintResources/StandardMacros.IsValid` _returnvalue_3
            (:`Is Valid`
              (`KismetSystemLibrary.PrintString` "BP Friend for hire is valid")
              (`self.SetActorHiddenInGame` _returnvalue_3 false)
              (`self.SetActorEnableCollision` _returnvalue_3 true))
            (:`Is Not Valid`
              (`KismetSystemLibrary.PrintString` "BP Friend for hire is NOT valid" true true (struct :`R` 1.0 :`G` 0.032468 :`A` 1.0)))))))))

(fn `UserConstructionScript`)