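; BP_WagerMan is an interactable Wager Man character that opens the Wager UI when the player interacts with him.
; A DoOnce limits this to one interaction, calling the parent logic, then after a short delay showing the UI through the game mode.
; Ending the interaction turns that UI message off.
; InteractVolume overlaps toggle the "E" prompt for the player pawn, which stops appearing once HasInteracted is set.
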(event `/Game/Utility/Interfaces/BPI_Interaction.InteractionEnded`
  ;[0.1823 0.1256 0.04851] Turn off the UI when the Interaction is ended
  (`parent.InteractionEnded`)
  (message `/Game/Utility/Interfaces/BPI_UI.TurnOffUI` (`GameplayStatics.GetGameMode`) "NewEnumerator9"))

(event `/Game/Utility/Interfaces/BPI_Interaction.InteractionStarted`
  (params (PlayerCharacter :type "/Game/Characters/BP_PlayerChar Object Reference") (HeldObject :type "Actor Object Reference"))
  ;[0.2604 0.208 0.1788] Turn on the Wager UI when the interaction is started
  (`/Engine/EditorBlueprintResources/StandardMacros.DoOnce` false
    (:`Completed`
      (`parent.InteractionStarted` PlayerCharacter null)
      (`KismetSystemLibrary.Delay` 1.3)
      (message `/Game/Utility/Interfaces/BPI_UI.TurnOnUI` (`GameplayStatics.GetGameMode`) "NewEnumerator9")
      (set `self.HasInteracted?` true)
      ;[0.1931 1 0.4723] Show and hide the "E" interaction message when in range of the Wager man
      (`SceneComponent.SetHiddenInGame` (`self.E to Interact`) true false :!label _label))))

(event `self.InteractVolume.OnComponentEndOverlap`
  (params (OverlappedComponent :type "PrimitiveComponent Object Reference") (OtherActor :type "Actor Object Reference") (OtherComp :type "PrimitiveComponent Object Reference") (OtherBodyIndex :type Integer))
  ;[0.1931 1 0.4723] Show and hide the "E" interaction message when in range of the Wager man
  (if (== OtherActor (`GameplayStatics.GetPlayerPawn` 0))
    (goto _label)))

(event `self.InteractVolume.OnComponentBeginOverlap`
  (params (OverlappedComponent :type "PrimitiveComponent Object Reference") (OtherActor :type "Actor Object Reference") (OtherComp :type "PrimitiveComponent Object Reference") (OtherBodyIndex :type Integer) (bFromSweep :type Boolean) (SweepResult :type "HitResult Structure (by ref)"))
  ;[0.1931 1 0.4723] Show and hide the "E" interaction message when in range of the Wager man
  (if (== (`GameplayStatics.GetPlayerPawn` 0) OtherActor)
    (if (not (`self.HasInteracted?`))
      (`SceneComponent.SetHiddenInGame` (`self.E to Interact`) false false))))

(fn `UserConstructionScript`
  (`parent.UserConstructionScript`))