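; BP_WagonMan is an interactable character, apparently an NPC, built on a parent class that supplies the interaction logic.
; When the player pawn enters its InteractionSphere, it plays the Goldencurior sound at its own location.
; Starting an interaction calls the parent handler, then hides the Billboard, which this Blueprint never shows again.
; Interaction end and construction only forward to the parent, and leaving the sphere triggers nothing.
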(event `/Game/Utility/Interfaces/BPI_Interaction.InteractionStarted`
  (params (PlayerCharacter :type "/Game/Characters/BP_PlayerChar Object Reference") (KBrownChar :type "/Game/KristianB/BP_ChickenCourier Object Reference"))
  ;[0 1 0.05664] InteractionStarted
  (`parent.InteractionStarted` PlayerCharacter null)
  (`SceneComponent.SetHiddenInGame` (`self.Billboard`) true false))

(event `self.InteractionSphere.OnComponentBeginOverlap`
  (params (OverlappedComponent :type "PrimitiveComponent Object Reference") (OtherActor :type "Actor Object Reference") (OtherComp :type "PrimitiveComponent Object Reference") (OtherBodyIndex :type Integer) (bFromSweep :type Boolean) (SweepResult :type "HitResult Structure (by ref)"))
  ;[1 1 1] Interaction button
  (if (== OtherActor (`GameplayStatics.GetPlayerPawn` 0))
    (`GameplayStatics.PlaySoundAtLocation` "/Game/SFX/CharacterSounds/FellowCourier/goldencurior.goldencurior" (`self.K2_GetActorLocation`) (struct) 1.0 1.0 0.0 null null null null)))

(event `/Game/Utility/Interfaces/BPI_Interaction.InteractionEnded`
  ;[0 1 0.05664] InteractionStarted
  (`parent.InteractionEnded`))

(event `self.InteractionSphere.OnComponentEndOverlap`
  (params (OverlappedComponent :type "PrimitiveComponent Object Reference") (OtherActor :type "Actor Object Reference") (OtherComp :type "PrimitiveComponent Object Reference") (OtherBodyIndex :type Integer))
  ;[1 1 1] Interaction button
  (if (== OtherActor (`GameplayStatics.GetPlayerPawn` 0))
    _))

(fn `UserConstructionScript`
  (`parent.UserConstructionScript`))