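; BP_Villager is an NPC character that runs BT_BASE_NPC when possessed and can carry a stealable item.
; Construction picks a woman, young man or old man mesh, animation class and walk speed.
; Projectile hits drop the item, launch the villager and briefly stun it, while steal events defer to the parent.
; HitBox overlaps with Buyer- or Seller-tagged actors pause the game; lose-condition events are empty, and swarm logic is disconnected.
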(event `self.HitBox.OnComponentBeginOverlap`
  (params (OverlappedComponent :type "PrimitiveComponent Object Reference") (OtherActor :type "Actor Object Reference") (OtherComp :type "PrimitiveComponent Object Reference") (OtherBodyIndex :type Integer) (bFromSweep :type Boolean) (SweepResult :type "HitResult Structure (by ref)"))
  ;[0.8745 0.1608 0] on begin overlap,if actor has "playerCharecter" tag, report touch event,play sound at location, and call event "FacePlayer"
  (bind _returnvalue (message `GameplayTagAssetInterface.HasMatchingGameplayTag` OtherActor (struct :`TagName` "buyer")))
  (if _returnvalue
    (`GameplayStatics.SetGamePaused` true)
    (else
      (bind _returnvalue_2 (message `GameplayTagAssetInterface.HasMatchingGameplayTag` OtherActor (struct :`TagName` "Seller")))
      (if _returnvalue_2
        (`GameplayStatics.SetGamePaused` true)))))

(event `Villager attmpts lose condition`
  ;[1 1 1] Lose condition logic
  ;;[0.8745 0.1608 0] Villager attempts lose condition
)

(event `self.ReceivePossessed`
  (params (NewController :type "Controller Object Reference"))
  ;[0.8745 0.1608 0] all villagers move to player unpon picking up golden chicken
  (bind _asaicontroller (cast `AIController` NewController))
  (`AIController.RunBehaviorTree` _asaicontroller "/Game/AI/Trees/BT_BASE_NPC.BT_BASE_NPC"))

(event `self.ReceiveBeginPlay`)

(event `/Game/Utility/Interfaces/BPI_Hit.HitByProjectile`
  (params (StunDuration :type "Float (double-precision)"))
  (bind (_returnvalue_x _returnvalue_y _returnvalue_z) (`KismetMathLibrary.BreakVector` (`self.GetActorForwardVector`)))
  (bind _returnvalue (+ 100.0 _returnvalue_x _returnvalue_y _returnvalue_z))
  ;[0.8745 0.1608 0] when hit by projectile, drop current item
  (message `/Game/Utility/Interfaces/BPI_EPS.ItemDropped` (`self.Current Item`) (`self.K2_GetActorLocation`))
  (set `self.Current Item` null)
  (set `self.Is Holding?` false)
  (`self.Stunned`)
  (`self.LaunchCharacter` (`KismetMathLibrary.MakeVector` _returnvalue _returnvalue _returnvalue) true true))

(event `LoseCondition_Villager`
  ;[1 1 1] Lose condition logic
  ;;[0.8745 0.1608 0] buffer for lose condition, villager
)

(event `/Game/Utility/Interfaces/BPI_Stealing.UpdateStealer`
  (params (ItemStolen :type "Actor Object Reference"))
  ;[0.8745 0.1608 0] Player Steals from villager
  (`parent.UpdateStealer` ItemStolen))

(event `/Game/Utility/Interfaces/BPI_Stealing.UpdateStolen`
  (params (`Who'sStealing` :type "Actor Object Reference"))
  ;[0.8745 0.1608 0] Villager steals from player
  (`parent.UpdateStolen` `Who'sStealing`))

(event `Stunned`
  (bind _current_item (`self.Current Item`))
  ;[0.6941 0.1176 0.1176] Stunned State
  (set `self.IsStunned?` false)
  (`/Engine/EditorBlueprintResources/StandardMacros.IsValid` _current_item
    (:`Is Valid`
      (`GameplayStatics.PlaySoundAtLocation` "/Game/SFX/Mechanics/Throw_Hit_Drop/ES_Comic_Tube_Doink_-_SFX_Producer.ES_Comic_Tube_Doink_-_SFX_Producer" (`self.K2_GetActorLocation`) (struct) 1.0 1.0 0.0 null null null null)
      (`SceneComponent.SetHiddenInGame` (`self.Chicken icon`) true false)
      (`self.K2_DetachFromActor` _current_item "KeepRelative" "KeepRelative" "KeepRelative")
      (message `/Game/Utility/Interfaces/BPI_EPS.ItemDropped` _current_item (`self.K2_GetActorLocation`))
      (set `self.Current Item` null)
      (set `self.Is Holding?` false))
    (:`Is Not Valid`
      _))
  (set `CharacterMovementComponent.MaxWalkSpeed` 0.0 (`self.CharacterMovement`))
  (`SceneComponent.SetHiddenInGame` (`self.Stunned Widget`) false false)
  (`GameplayStatics.PlaySoundAtLocation` "/Game/SFX/CharacterSounds/Theif/SC_HitSounds.SC_HitSounds" (`self.K2_GetActorLocation`) (struct) 0.75 1.0 0.0 null null null null)
  (`KismetSystemLibrary.Delay` 3.0)
  (set `CharacterMovementComponent.MaxWalkSpeed` 350.0 (`self.CharacterMovement`))
  (`SceneComponent.SetHiddenInGame` (`self.Stunned Widget`) true false)
  (set `self.IsStunned?` false)
  (`SceneComponent.SetHiddenInGame` (`self.Chicken icon`) true false))

(fn `PickupChicken`
  (returns (`Currently being held` :type Boolean))
  (return false))

(fn `UserConstructionScript`
  (bind _mesh (`self.Mesh`))
  (bind _mesh_2 (`self.Mesh`))
  (bind _mesh_3 (`self.Mesh`))
  (switch `int` (`self.SkeletalMesh`)
    (:`0`
      ;[1 1 1] Woman
      (`SkeletalMeshComponent.SetSkeletalMeshAsset` _mesh_2 "/Game/Meshes/Characters/Villagers/Female/Villager_woman__1_.Villager_woman__1_")
      (`SkeletalMeshComponent.SetAnimInstanceClass` _mesh_2 "/Game/Art/CharecterAnimations/ABP_VillagerW.ABP_VillagerW_C")
      (set `CharacterMovementComponent.MaxWalkSpeed` 250.0 (`self.CharacterMovement`) :!label _label))
    (:`1`
      ;[1 1 1] Young man
      (`SkeletalMeshComponent.SetSkeletalMeshAsset` _mesh_3 "/Game/Meshes/Characters/Villagers/MaleYoung/Villager_young__1_.Villager_young__1_")
      (`SkeletalMeshComponent.SetAnimInstanceClass` _mesh_3 "/Game/Art/CharecterAnimations/ABP_VillagerM.ABP_VillagerM_C")
      (goto _label))
    (:`2`
      ;[1 1 1] Old man
      (`SkeletalMeshComponent.SetSkeletalMeshAsset` _mesh "/Game/Meshes/Characters/Villagers/MaleOld/Villager_old__1_.Villager_old__1_")
      (`SkeletalMeshComponent.SetAnimInstanceClass` _mesh "/Game/Art/CharecterAnimations/ABP_VillagerOM.ABP_VillagerOM_C")
      (set `CharacterMovementComponent.MaxWalkSpeed` 125.0 (`self.CharacterMovement`)))))