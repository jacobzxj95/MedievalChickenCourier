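; Quest giver NPC that offers a quest and accepts turned-in items, with mesh and animations chosen by type.
; Interaction opens the quest through ACQuestGiver once until reset, and checks held items through ACQuestTurnin when enabled, moving stored chickens.
; Overlap plays a wave and shows the interact prompt.
; An overhead icon follows quest acceptance, GM_MVP quest-load events and objective waypoint toggles.
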(event `self.ReceiveBeginPlay`
  (bind _mesh (`self.Mesh`))
  (switch `int` (`self.QuestGiverType`)
    (:`0`
      (`SkeletalMeshComponent.PlayAnimation` _mesh "/Game/Meshes/Characters/OldLady/Idle__1_.Idle__1_" true))
    (:`1`
      (`SkeletalMeshComponent.PlayAnimation` _mesh "/Game/Art/CharecterAnimations/AnimSequences/QuestGivers/Leofric/Neutral_Idle.Neutral_Idle" true))
    (:`2`
      _))
  (bind _output_get (`/Game/Components/ActorComponents/AC_QuestTurnin.CreateWidget` (`self.AC_QuestTurnin`)))
  (set `self.Above Character Ref` _output_get)
  (`WidgetComponent.SetWidget` (`self.TurnInIcon`) _output_get)
  (`/Game/UI/Icons/W_MainObjectiveIcon.TurnOnObjectiveIcon` _output_get 1)
  (bind _asgm_mvp (cast `/Game/Maps/GameModes/GM_MVP` (`GameplayStatics.GetGameMode`)))
  (add `/Game/Maps/GameModes/GM_MVP.QuestDataLoad` _asgm_mvp (delegate `QuestHasBeenLoaded`)))

(event `QuestHasBeenLoaded`
  (params (QuestRowName :type Name))
  (if (== (`.RowName` (break `DataTableRowHandle` (`/Game/Components/ActorComponents/AC_QuestGiver.QuestToGive` (`self.AC_QuestGiver`)))) QuestRowName)
    (`SceneComponent.SetHiddenInGame` (`self.TurnInIcon`) true false)
    (set `self.CloseDoOnce` true)
    (set `self.ShouldMoveCamera` false)
    (set `self.QuestEnabled` true)))

(event `QuestAccepted?`
  (params (`Accepted/NotAccepted` :type Boolean))
  ;[0 1 0.05664] InteractionStarted
  (if `Accepted/NotAccepted`
    (`SceneComponent.SetHiddenInGame` (`self.TurnInIcon`) true false)
    (else
      (`self.Reset`)
      (set `self.ShouldMoveCamera` true))))

(event `Reset`
  ;[0 1 0.05664] InteractionStarted
  (goto _label :!via `Reset`))

(event `self.InteractionStarted`
  (params (PlayerCharacter :type "/Game/Characters/BP_PlayerChar Object Reference") (HeldObject :type "Actor Object Reference"))
  (bind _ac_questturnin (`self.AC_QuestTurnin`))
  ;[0 1 0.05664] InteractionStarted
  (`parent.InteractionStarted` PlayerCharacter null)
  (`|ExecutionSequence`
    (:`then_0`
      (`/Engine/EditorBlueprintResources/StandardMacros.DoOnce` (`self.CloseDoOnce`) :!label _label
        (:`Completed`
          (`self.QuestInteraction`)
          (set `self.ShouldMoveCamera` false)
          (add `/Game/UI/Dialogue/W_QuestDialogue.QuestInteraction` (`/Game/Components/ActorComponents/AC_QuestGiver.QuestWidget` (`self.AC_QuestGiver`)) (delegate `QuestAccepted?`)))))
    (:`then_1`
      (if (`self.QuestEnabled`)
        (if (!= HeldObject null)
          (bind _isquestitem (`/Game/Components/ActorComponents/AC_QuestTurnin.Actor to Check` _ac_questturnin HeldObject))
          (if _isquestitem
            (switch `/Game/Utility/Enums/E_TurnInActions` (`self.What to do with turned in item`)
              (:`NewEnumerator0`
                (`/Game/Components/ActorComponents/AC_QuestTurnin.MoveActorToLocation` _ac_questturnin (`SceneComponent.K2_GetComponentLocation` (`self.ChickenMovementLocation`)) true))))
          (else
            (`GameplayStatics.PlaySound2D` "/Game/SFX/UISounds/IncorrectInput.IncorrectInput" 1.0 1.0 0.0 null null)))))))

(event `self.InteractionSphere.OnComponentBeginOverlap`
  (params (OverlappedComponent :type "PrimitiveComponent Object Reference") (OtherActor :type "Actor Object Reference") (OtherComp :type "PrimitiveComponent Object Reference") (OtherBodyIndex :type Integer) (bFromSweep :type Boolean) (SweepResult :type "HitResult Structure (by ref)"))
  (bind _mesh (`self.Mesh`))
  ;[1 1 1] Interaction button
  (if (== OtherActor (`GameplayStatics.GetPlayerPawn` 0))
    (`|ExecutionSequence`
      (:`then_0`
        (switch `int` (`self.QuestGiverType`)
          (:`0`
            (`SkeletalMeshComponent.PlayAnimation` _mesh "/Game/Meshes/Characters/OldLady/Waving.Waving" false)
            (`KismetSystemLibrary.Delay` 0.6)
            (`SkeletalMeshComponent.PlayAnimation` _mesh "/Game/Meshes/Characters/OldLady/Idle__1_.Idle__1_" true))
          (:`1`
            (`SkeletalMeshComponent.PlayAnimation` _mesh "/Game/Art/CharecterAnimations/AnimSequences/QuestGivers/Leofric/Waving.Waving" false)
            (`KismetSystemLibrary.Delay` 0.7)
            (`SkeletalMeshComponent.PlayAnimation` _mesh "/Game/Art/CharecterAnimations/AnimSequences/QuestGivers/Leofric/Neutral_Idle.Neutral_Idle" true))
          (:`2`
            (`SkeletalMeshComponent.PlayAnimation` _mesh "/Game/Art/CharecterAnimations/AnimSequences/QuestGivers/OldLady/OldLady_Waving_Anim.OldLady_Waving_Anim" true)
            (`KismetSystemLibrary.Delay` 0.7)
            (`SkeletalMeshComponent.PlayAnimation` _mesh "/Game/Art/CharecterAnimations/AnimSequences/QuestGivers/OldLady/OldLady_Idle_Anim.OldLady_Idle_Anim" true))))
      (:`then_1`
        (bind _asgm_mvp (cast `/Game/Maps/GameModes/GM_MVP` (`GameplayStatics.GetGameMode`)))
        (`Widget.SetVisibility` (`/Game/UI/W_HUD.EtoInteract` (`/Game/Maps/GameModes/GM_MVP.PlayerHUD` _asgm_mvp)) "Visible")))))

(event `self.InteractionEnded`
  ;[0 1 0.05664] InteractionStarted
  (`parent.InteractionEnded`))

(event `self.InteractionSphere.OnComponentEndOverlap`
  (params (OverlappedComponent :type "PrimitiveComponent Object Reference") (OtherActor :type "Actor Object Reference") (OtherComp :type "PrimitiveComponent Object Reference") (OtherBodyIndex :type Integer))
  ;[1 1 1] Interaction button
  (if (== OtherActor (`GameplayStatics.GetPlayerPawn` 0))
    (`Widget.SetVisibility` (`/Game/UI/W_HUD.EtoInteract` (`/Game/Maps/GameModes/GM_MVP.PlayerHUD` (stale `self.InteractionSphere.OnComponentBeginOverlap` _asgm_mvp))) "Hidden")))

(event `/Game/Utility/Interfaces/BPI_Quest.TurnOnWaypoints`
  (params (ObjectiveID :type String) (`On/Off` :type Boolean))
  (bind _turninicon (`self.TurnInIcon`))
  (for _array_element (`/Game/Components/ActorComponents/AC_QuestTurnin.ObjectiveName` (`self.AC_QuestTurnin`))
    (if (`KismetStringLibrary.EqualEqual_StrStr` ObjectiveID _array_element)
      (if `On/Off`
        (`KismetSystemLibrary.DelayUntilNextTick`)
        (`SceneComponent.SetHiddenInGame` _turninicon false false)
        (`/Game/UI/Icons/W_MainObjectiveIcon.TurnOnObjectiveIcon` (`self.Above Character Ref`) 0)
        (set `self.QuestEnabled` true)
        (else
          (`SceneComponent.SetHiddenInGame` _turninicon true false)
          (set `self.QuestEnabled` false))))))

(fn `QuestInteraction`
  (returns (ObjectiveID :type String))
  (bind _objectiveid (`/Game/Components/ActorComponents/AC_QuestGiver.QuestInteraction` (`self.AC_QuestGiver`)))
  (return _objectiveid))

(fn `UserConstructionScript`
  (`parent.UserConstructionScript`)
  (switch `int` (`self.QuestGiverType`)
    (:`0`
      (`SkeletalMeshComponent.SetSkeletalMeshAsset` (`self.Mesh`) "/Game/Meshes/Characters/OldLady/Idle.Idle"))
    (:`1`
      (`SkeletalMeshComponent.SetSkeletalMeshAsset` (`self.Mesh`) "/Game/Meshes/Characters/FellowCouriers/LeoFric__1_.LeoFric__1_"))))