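; Quest manager that runs one quest, loading its details from DT_QuestInfo and tracking progress through stages and objectives.
; Objective ID updates advance progress, send UI messages through the GameMode and save completed quests, while "SUB" updates count toward failure.
; Waypoints toggle on BPI_Quest actors whose turn-in or item components match the objective, except for secret quests.
; Golden chicken quests spawn their chicken upon reaching the final stage.
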(event `EvaluteStageWhenLoaded`
  (bind (_questgivername _dialoguetext _queststages) (break `/Game/Utility/Struct/STR_QuestDetails` (`self.QuestDetails`)))
  (if (not (`KismetArrayLibrary.Array_IsValidIndex` _queststages (+ (`KismetArrayLibrary.Array_Find` _queststages (`self.CurrentStage`)) 1)))
    (`self.SpawnGoldenChicken`)))

(event `self.ReceiveBeginPlay`
  (bind ((`QuestStages_7_B3E19BA34577D0A5172858847C21D2F1` _queststages) (`IsSecret_12_997409714C1FE5970EE995B7DD81B4C0` _issecret)) (break `/Game/Utility/Struct/STR_QuestDetails` (`self.QuestDetails`)))
  ;[1 1 1] When the quest is created, set the variables
  (bind _returnvalue (`GameplayStatics.GetCurrentLevelName` true))
  (set `self.Level Quest Is In` _returnvalue)
  ;[1 1 1] Check to see if a save game exsists
  (bind _returnvalue_2 (`|GetDataTableRow` "/Game/Utility/DT_QuestInfo.DT_QuestInfo" (`self.QuestRowID`))
    (:`then`
      (set `self.QuestDetails` _returnvalue_2)
      (set `self.Is this QuestSecret` _issecret)
      (bind _output_get (set `self.CurrentStage` (`|GetArrayItem` _queststages (`self.CurrentStageNum`))))
      (set `self.ObjectiveLossCondition` (`.LossCondition_20_191E6C644659182B726D1DB575F335C5` (break `/Game/Utility/Struct/STR_ObjectiveDetails` (`|GetArrayItem` (`.Objectives_25_1EF6A4194D11E168DBD54CB3AA140CC2` (break `/Game/Utility/Struct/STR_StageDetails` _output_get))))))
      (`self.TellQuestActorsToTurnOn/OffWaypoints` true)
      (add `self.Quest Failed` (delegate `Quest Failed_Event`)))))

(event `Quest Failed_Event` :!signature `self.Quest Failed`
  (params (Loss :type String))
  (`self.TellQuestActorsToTurnOn/OffWaypoints` false)
  (message `/Game/Utility/Interfaces/BPI_UI.TurnOffUI` (`GameplayStatics.GetGameMode`) "NewEnumerator0"))

(event `/Game/Utility/Interfaces/BPI_Quest.QuestUpdate`
  (params (ObjectiveID :type String))
  ;[1 1 1] Update the quest info
  (`self.UpdateQuestInfo` ObjectiveID))

(fn `CurObjectiveDetails`
  (params (`Previous/Current` :type Boolean))
  (returns (`Current Objective` :type "/Game/Utility/Struct/STR_ObjectiveDetails Structure (by ref)"))
  (return (`|GetArrayItem` (`.Objectives_25_1EF6A4194D11E168DBD54CB3AA140CC2` (break `/Game/Utility/Struct/STR_StageDetails` (`self.CurrentStage`))) (`KismetMathLibrary.SelectInt` (- (`self.CurrentObjectiveNum`) 1) (`self.CurrentObjectiveNum`) `Previous/Current`))))

(fn `SpawnGoldenChicken`
  (bind _returnvalue (`GameplayStatics.GetActorOfClass` "/Game/LevelObjects/QuestRelated/BP_GoldenChickerSpawnLocation.BP_GoldenChickerSpawnLocation_C"))
  (bind _returnvalue_2 (`|SpawnActorFromClass` (`.GoldenChickenType_23_A50DFF054B28B98B69DDDB970DBE51FC` (break `/Game/Utility/Struct/STR_QuestDetails` (`self.QuestDetails`))) (`KismetMathLibrary.MakeTransform` (`SceneComponent.K2_GetComponentLocation` (`Actor.RootComponent` _returnvalue))) "Undefined" "OverrideRootScale" self null))
  (`/Game/LevelObjects/QuestRelated/BP_GoldenChickerSpawnLocation.Animate The Cock` _returnvalue _returnvalue_2))

(fn `TellQuestActorsToTurnOn/OffWaypoints`
  (params (`On/Off` :type Boolean) (`Previous/Current` :type Boolean))
  ;[1 1 1] If not a secret quest turn on waypoints
  (if (not (`self.Is this QuestSecret`))
    (bind _outactors (`GameplayStatics.GetAllActorsWithInterface` "/Game/Utility/Interfaces/BPI_Quest.BPI_Quest_C"))
    (for _array_element _outactors
      (switch `/Game/Utility/Enums/E_StepType` (`.ObjectiveType_13_434CD30B4087BA0F3DC7F1B3A89D7407` (break `/Game/Utility/Struct/STR_ObjectiveDetails` (`self.CurObjectiveDetails` (`local.Previous/Current`))))
        (:`NewEnumerator0`
          (bind _returnvalue (`self.GetComponentByClass` _array_element "/Game/Components/ActorComponents/AC_QuestTurnin.AC_QuestTurnin_C"))
          (`/Engine/EditorBlueprintResources/StandardMacros.IsValid` _returnvalue :!label _label
            (:`Is Valid`
              (for _array_element_2 (`/Game/Components/ActorComponents/AC_QuestTurnin.ObjectiveName` _returnvalue)
                (if (`KismetStringLibrary.EqualEqual_StrStr` _array_element_2 (`.ObjectiveID_12_1EAEAB4C4B67269B52536BAF19FAA687` (break `/Game/Utility/Struct/STR_ObjectiveDetails` (`self.CurObjectiveDetails` (`local.Previous/Current`)))))
                  (message `/Game/Utility/Interfaces/BPI_Quest.TurnOnWaypoints` _array_element (`.ObjectiveID_12_1EAEAB4C4B67269B52536BAF19FAA687` (break `/Game/Utility/Struct/STR_ObjectiveDetails` (`self.CurObjectiveDetails` (`local.Previous/Current`)))) `On/Off` :!label _label_2))))))
        (:`NewEnumerator1`
          (bind _returnvalue_2 (`self.GetComponentByClass` _array_element "/Game/Components/ActorComponents/AC_Questitem.AC_Questitem_C"))
          (`/Engine/EditorBlueprintResources/StandardMacros.IsValid` _returnvalue_2 :!label _label_3
            (:`Is Valid`
              (for _array_element_3 (`/Game/Components/ActorComponents/AC_Questitem.ActorQuestIDS` _returnvalue_2)
                (if (`KismetStringLibrary.EqualEqual_StrStr` _array_element_3 (`.ObjectiveID_12_1EAEAB4C4B67269B52536BAF19FAA687` (break `/Game/Utility/Struct/STR_ObjectiveDetails` (`self.CurObjectiveDetails` (`local.Previous/Current`)))))
                  (goto _label_2))))))
        (:`NewEnumerator2`
          (`|ExecutionSequence`
            (:`then_0`
              (goto _label))
            (:`then_1`
              (goto _label_3))))))
    (return)
    (else
      (return))))

(fn `UpdateQuestInfo`
  (params (CheckingOBJID :type String))
  (bind _returnvalue (`GameplayStatics.GetGameMode`))
  (bind (_current_objective_objectivename _current_objective_objectivedescription _current_objective_objectivetype _current_objective_objectiveid) (break `/Game/Utility/Struct/STR_ObjectiveDetails` (`self.CurObjectiveDetails` true)))
  (bind _currentobjectivenum (`self.CurrentObjectiveNum`))
  (bind ((`Objectives_25_1EF6A4194D11E168DBD54CB3AA140CC2` _objectives)) (break `/Game/Utility/Struct/STR_StageDetails` (`self.CurrentStage`)))
  (bind ((`CompletionReward_15_BBC272474F79DB67EF7CC299C30286D1` _completionreward) (`IsGoldenChickenQuest_17_9512DF304F1ED28EA9BD8E8772247193` _isgoldenchickenquest)) (break `/Game/Utility/Struct/STR_QuestDetails` (`self.QuestDetails`)))
  (bind _returnvalue_2 (- (`self.ObjectiveLossCondition`) 1))
  (bind _returnvalue_3 (`KismetMathLibrary.Clamp` (+ (`self.CurrentObjectiveNum`) 1) 0 (- (`KismetArrayLibrary.Array_Length` (`.Objectives_25_1EF6A4194D11E168DBD54CB3AA140CC2` (break `/Game/Utility/Struct/STR_StageDetails` (`self.CurrentStage`)))) 1)))
  ;[1 1 1] Is the update coming from something with the current objectiveID
  (if (`KismetArrayLibrary.Array_IsValidIndex` _objectives _currentobjectivenum)
    (if (`KismetStringLibrary.EqualEqual_StrStr` CheckingOBJID (`.ObjectiveID_12_1EAEAB4C4B67269B52536BAF19FAA687` (break `/Game/Utility/Struct/STR_ObjectiveDetails` (`|GetArrayItem` _objectives _currentobjectivenum))))
      (bind _result (`/Engine/EditorBlueprintResources/StandardMacros.IncrementInt` (`BlueprintMapLibrary.Map_Find` (`self.CurrentObjectiveProgress`) (`local.CheckingOBJID`)))
        (:`  `
          (if (<= (`.Quantity_16_9D94EDA64A4CAC90391433AE0F575027` (break `/Game/Utility/Struct/STR_ObjectiveDetails` (`self.CurObjectiveDetails` false))) _result)
            ;[1 1 1] Check to see if the current objective is complete
            (if (not (== (`self.CurrentObjectiveNum`) (`KismetArrayLibrary.Array_LastIndex` (`.Objectives_25_1EF6A4194D11E168DBD54CB3AA140CC2` (break `/Game/Utility/Struct/STR_StageDetails` (`self.CurrentStage`))))))
              (if (`KismetArrayLibrary.Array_IsValidIndex` (`.Objectives_25_1EF6A4194D11E168DBD54CB3AA140CC2` (break `/Game/Utility/Struct/STR_StageDetails` (`self.CurrentStage`))) _returnvalue_3)
                (bind _output_get (set `self.CurrentObjectiveNum` _returnvalue_3))
                (set `self.ObjectiveLossCondition` (`.LossCondition_20_191E6C644659182B726D1DB575F335C5` (break `/Game/Utility/Struct/STR_ObjectiveDetails` (`|GetArrayItem` (`.Objectives_25_1EF6A4194D11E168DBD54CB3AA140CC2` (break `/Game/Utility/Struct/STR_StageDetails` (`self.CurrentStage`))) _output_get))))
                (if (not (`self.Is this QuestSecret`))
                  (`self.ObjectiveCompleted` _current_objective_objectiveid)
                  (message `/Game/Utility/Interfaces/BPI_UI.ObjectiveCompleted` (`GameplayStatics.GetGameMode`) (`self.CurObjectiveDetails` false))
                  (`GameplayStatics.PlaySound2D` "/Game/SFX/QuestRelated/kazoocelebration.kazoocelebration" 1.0 1.0 0.0 null null)
                  (`|ExecutionSequence`
                    (:`then_0`
                      (`self.TellQuestActorsToTurnOn/OffWaypoints` false true))
                    (:`then_1`
                      (`self.TellQuestActorsToTurnOn/OffWaypoints` true)))))
              (elif (not (`self.Is this QuestSecret`))
                (bind _was_last_stage (`self.UpdateQuestStage`))
                (if _was_last_stage
                  (message `/Game/Utility/Interfaces/BPI_UI.QuestCompleted` _returnvalue _isgoldenchickenquest)
                  (message `/Game/Utility/Interfaces/BPI_UI.UpdateCurrency` _returnvalue _completionreward :!label _label)
                  (`self.TellQuestActorsToTurnOn/OffWaypoints` false)
                  (`self.QuestCompleted` self)
                  (bind _game_instance (message `/Game/Utility/Interfaces/BPI_UI.Pass Out Game Instance Ref` (`GameplayStatics.GetGameMode`)))
                  (`/Game/Utility/GameModes/BP_GameInstance.SaveCompletedQuests` _game_instance (`self.QuestRowID`))
                  (else
                    (message `/Game/Utility/Interfaces/BPI_UI.StageCompleted` (`GameplayStatics.GetGameMode`) (`self.CurrentStage`))))
                (else
                  (goto _label))))
            (else
              ;[1 1 1] Update current objective progress and update the UI
              (if (not (`self.Is this QuestSecret`))
                (`BlueprintMapLibrary.Map_Add` (`self.CurrentObjectiveProgress`) (`local.CheckingOBJID`) _result)
                (message `/Game/Utility/Interfaces/BPI_UI.Update UI Upon Turnin` (`GameplayStatics.GetGameMode`) _result (`self.CurObjectiveDetails` false))
                (`GameplayStatics.PlaySound2D` "/Game/SFX/QuestTick.QuestTick" 1.0 1.0 0.0 null null))))))
      (elif (and (`KismetStringLibrary.EqualEqual_StrStr` CheckingOBJID "SUB") (not (`.IsSecret_12_997409714C1FE5970EE995B7DD81B4C0` (break `/Game/Utility/Struct/STR_QuestDetails` (`self.QuestDetails`)))))
        (if (`KismetStringLibrary.EqualEqual_StrStr` "goldenChicken" (`.ObjectiveID_12_1EAEAB4C4B67269B52536BAF19FAA687` (break `/Game/Utility/Struct/STR_ObjectiveDetails` (`self.CurObjectiveDetails` false))))
          (`self.Quest Failed` "GoldenChicken")
          (`self.TellQuestActorsToTurnOn/OffWaypoints` false)
          (elif (<= _returnvalue_2 0)
            (`self.Quest Failed` "Thieves")
            (else
              (bind _output_get_2 (set `self.ObjectiveLossCondition` _returnvalue_2))
              (message `/Game/Utility/Interfaces/BPI_UI.LossCondition` (`GameplayStatics.GetGameMode`) _output_get_2))))))))

(fn `UpdateQuestStage`
  (returns (`Was Last Stage` :type Boolean))
  (locals (TempCurrentStage :type Integer))
  (bind ((`QuestGiverName_26_FA10CE0E4EF0CD66FDF818BFB9FBF03B` _questgivername) (`QuestStages_7_B3E19BA34577D0A5172858847C21D2F1` _queststages)) (break `/Game/Utility/Struct/STR_QuestDetails` (`self.QuestDetails`)))
  (if (not (== (`self.CurrentStageNum`) (`KismetArrayLibrary.Array_LastIndex` _queststages)))
    (`self.TellQuestActorsToTurnOn/OffWaypoints` false)
    (`/Engine/EditorBlueprintResources/StandardMacros.IncrementInt` (`self.CurrentStageNum`)
      (:`  `
        (if (and (not (`KismetArrayLibrary.Array_IsValidIndex` _queststages (+ (`self.CurrentStageNum`) 1))) (`.IsGoldenChickenQuest_17_9512DF304F1ED28EA9BD8E8772247193` (break `/Game/Utility/Struct/STR_QuestDetails` (`self.QuestDetails`))))
          (`self.SpawnGoldenChicken`))
        (bind _output_get (set `self.CurrentStage` (`|GetArrayItem` (`.QuestStages_7_B3E19BA34577D0A5172858847C21D2F1` (break `/Game/Utility/Struct/STR_QuestDetails` (`self.QuestDetails`))) (`self.CurrentStageNum`))))
        (bind _output_get_2 (set `self.CurrentObjectiveNum` 0))
        (bind ((`ObjectiveID_12_1EAEAB4C4B67269B52536BAF19FAA687` _objectiveid) (`LossCondition_20_191E6C644659182B726D1DB575F335C5` _losscondition)) (break `/Game/Utility/Struct/STR_ObjectiveDetails` (`|GetArrayItem` (`.Objectives_25_1EF6A4194D11E168DBD54CB3AA140CC2` (break `/Game/Utility/Struct/STR_StageDetails` _output_get)) _output_get_2)))
        (set `self.ObjectiveLossCondition` _losscondition)
        (`self.StageCompleted` _objectiveid)
        (`self.TellQuestActorsToTurnOn/OffWaypoints` true)
        (return false)))
    (else
      (return true))))

(fn `UserConstructionScript`)