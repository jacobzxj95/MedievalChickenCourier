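; SaveGame Blueprint that stores quest progress, player data, object turn-in states and the last loaded level.
; Quest saves record completed IDs, each level's quest and a per-quest stage, objective and progress struct, with maps also tracking object turn-ins.
; Each save function writes the whole object to the QuestSaveData, PlayerSaveData or ObjectData slot.
; ClearQuestData empties quest maps in memory without saving, leaving completed quests intact.
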(fn `ClearQuestData`
  (`BlueprintMapLibrary.Map_Clear` (`self.LevelQuests`))
  (`BlueprintMapLibrary.Map_Clear` (`self.QuestProgress`))
  (`BlueprintMapLibrary.Map_Clear` (`self.HasQuestObjectBeenTurned`)))

(fn `SaveLastLoadedLevel`
  (params (LevelName :type String))
  (set `self.LevelName` LevelName)
  (`GameplayStatics.SaveGameToSlot` self "PlayerSaveData"))

(fn `SaveObjectData`
  (params (`Object Name` :type Name) (TurninStatus :type Boolean))
  (`BlueprintMapLibrary.Map_Add` (`self.Has Object Been Turned in`) (`KismetStringLibrary.Conv_NameToString` `Object Name`) TurninStatus)
  (`GameplayStatics.SaveGameToSlot` self "ObjectData"))

(fn `SavePlayerData`
  (params (`Data to save` :type "/Game/Utility/Struct/STR_PlayerSaveData Structure"))
  (set `self.PlayerSaveData` `Data to save`)
  (`GameplayStatics.SaveGameToSlot` self "PlayerSaveData"))

(fn `SaveQuestDetails`
  (params (`Quest Actor` :type "/Game/RodgerL/BP_QuestManager Object Reference") (HasQuestCompleted :type Boolean))
  (bind _questrowid (`/Game/RodgerL/BP_QuestManager.QuestRowID` `Quest Actor`))
  (if HasQuestCompleted
    (`KismetArrayLibrary.Array_AddUnique` (`self.CompletedQuests`) _questrowid))
  (`BlueprintMapLibrary.Map_Add` (`self.LevelQuests`) (`/Game/RodgerL/BP_QuestManager.Level Quest Is In` `Quest Actor`) _questrowid)
  (`BlueprintMapLibrary.Map_Add` (`self.QuestProgress`) _questrowid (make `/Game/Utility/Struct/STR_SaveData` :`Quest Progress` (`/Game/RodgerL/BP_QuestManager.CurrentObjectiveProgress` `Quest Actor`) :`CurrentStage` (`/Game/RodgerL/BP_QuestManager.CurrentStage` `Quest Actor`) :`CurrentObjective` (`/Game/RodgerL/BP_QuestManager.CurrentObjectiveNum` `Quest Actor`) :`Has Been Set` true))
  (`GameplayStatics.SaveGameToSlot` self "QuestSaveData")
  (return))

(fn `SaveQuestObjectData`
  (params (`Object Name` :type Name) (TurninLocation :type "Vector Structure"))
  (`BlueprintMapLibrary.Map_Add` (`self.HasQuestObjectBeenTurned`) (`KismetStringLibrary.Conv_NameToString` `Object Name`) TurninLocation)
  (`GameplayStatics.SaveGameToSlot` self "QuestSaveData"))