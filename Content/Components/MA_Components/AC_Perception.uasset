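; Actor component that makes AI-audible noise for its owner, intended for sprinting.
; RunningNoise emits a full-loudness noise at the owner's location through a PawnNoiseEmitter, alerting AI within hearing range.
; The Hearing test event and Tick are empty.
; A disconnected draft that scales loudness from audio attenuation settings and distance never runs.
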(event `Running Noise`
  (bind _returnvalue (`self.GetOwner`))
  ;[0.599 0 0.05185] AI Perception:NOISE
  ;;[1 1 1] toggle sprint, make noise; will alert AI if within range
  (`PawnNoiseEmitterComponent.MakeNoise` (`self.PawnNoiseEmitter`) _returnvalue 1.0 (`Actor.K2_GetActorLocation` _returnvalue)))

(event `Hearing`
  ;[0.599 0 0.05185] AI Perception:NOISE
  ;;[1 1 1] Testing pawn sensing,make noise, will alert AI if within range
)