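; Actor component that lets the player pick up and drop items tagged "Interactable", holding one at a time.
; On PickUp Item input, it attaches the first tagged actor overlapping the player to the mesh's sword socket.
; On Drop Item input, it traces downward from the player and, on a hit, detaches the held item and places it at the hit location.
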(event `InputAction|PickUp Item`
  (params (Key :type "Key Structure"))
  ;[0.8784 0.03529 0.04706] on input, get all overlapping actors, search for tag "Interactable" If actor has tag, set as current item, attach actor to component, set is holding weapon to true
  (:`Pressed`
    (if (not (`self.Is Holding Weapon?`))
      (for _array_element (`Actor.GetOverlappingActors` (`GameplayStatics.GetPlayerCharacter` 0) "/Script/Engine.Actor")
        (if (`Actor.ActorHasTag` _array_element "Interactable")
          (bind _output_get (set `self.Current Item` _array_element))
          (`Actor.K2_AttachToComponent` _output_get (`self.Mesh`) "sword_socket" "SnapToTarget" "SnapToTarget" "SnapToTarget" true)
          (set `self.Is Holding Weapon?` true)
          (break))))))

(event `InputAction|Drop Item`
  (params (Key :type "Key Structure"))
  (bind _current_item (`self.Current Item`))
  ;[0.8784 0.03529 0.04706] on input, check if player is holding weapon, line trace from player location,subtracting from the z value,if line trace hits solid object detach current item from actor and set actor transform
  (:`Pressed`
    (if (`self.Is Holding Weapon?`)
      (bind (_outhit _returnvalue) (`KismetSystemLibrary.LineTraceSingle` (`Actor.K2_GetActorLocation` (`GameplayStatics.GetPlayerCharacter` 0)) (- (`Actor.K2_GetActorLocation` (`GameplayStatics.GetPlayerCharacter` 0)) (0.0 0.0 500.0)) "TraceTypeQuery1"))
      (if _returnvalue
        (`Actor.K2_DetachFromActor` _current_item "KeepWorld" "KeepWorld" "KeepWorld")
        (`Actor.K2_SetActorTransform` _current_item (`KismetMathLibrary.MakeTransform` (`.Location` (`GameplayStatics.BreakHitResult` _outhit))) false false)
        (set `self.Is Holding Weapon?` false)))))