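; Actor component that lets a walking character vault over obstacles in front of it.
; VaultLinetrace line-traces forward at knee height, then sphere-traces down to find the wall top and check its height and thickness.
; Tick lerps the owner above that point, then launches player character 0 forward.
; The thickness-aware VaultTick, with its CancelVault reset, is never run, and EndHit is never assigned here.
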(event `self.ReceiveTick`
  (params (DeltaSeconds :type "Float (single-precision)"))
  (bind _returnvalue (`self.GetOwner`))
  (bind (_middlehit_x _middlehit_y _middlehit_z) (`KismetMathLibrary.BreakVector` (`self.MiddleHit`)))
  (bind _returnvalue_2 (`KismetMathLibrary.MakeVector` _middlehit_x _middlehit_y (+ _middlehit_z 100.0)))
  (if (`self.VaultingCheck`)
    (`Actor.K2_SetActorLocation` _returnvalue (`KismetMathLibrary.VLerp` (`Actor.K2_GetActorLocation` _returnvalue) _returnvalue_2 DeltaSeconds) false false)
    (if (== (`Actor.K2_GetActorLocation` (`self.GetOwner`)) _returnvalue_2 :`ErrorTolerance` 45.0)
      (`Character.LaunchCharacter` (`GameplayStatics.GetPlayerCharacter` 0) (* (`Actor.GetActorForwardVector` (`self.GetOwner`)) 500.0) true true)
      (set `self.VaultingCheck` false))))

(event `VaultLinetrace`
  (bind _returnvalue (`self.GetOwner`))
  (bind _returnvalue_2 (+ (- (`Actor.K2_GetActorLocation` _returnvalue) (0.0 0.0 20.0)) (`KismetMathLibrary.SelectVector` (0.0 0.0 0.0) (* (`Actor.GetActorForwardVector` (`self.GetOwner`)) (`self.StartingLocationMod`)) (`self.ShouldCheckFarther`))))
  (bind _returnvalue_3 (+ (`self.Wall Location`) (* (`KismetMathLibrary.GetForwardVector` (`KismetMathLibrary.MakeRotFromX` (`self.Wall Normal`))) -10.0)))
  ;[0 1 0.05664] Checking to see if there is a surface at about knee height in front of the character
  (if (`|EnumEquality` (`CharacterMovementComponent.MovementMode` (`Actor.GetComponentByClass` _returnvalue "/Script/Engine.CharacterMovementComponent")) "MOVE_Walking")
    (bind (_outhit _returnvalue_4) (`KismetSystemLibrary.LineTraceSingle` :`Start` _returnvalue_2 :`End` (+ _returnvalue_2 (* (`Actor.GetActorForwardVector` (`self.GetOwner`)) (`self.LineLength`))) :`TraceChannel` "TraceTypeQuery4" :`DrawDebugType` "Persistent"))
    (if _returnvalue_4
      (set `self.SomethingHit` true)
      (bind (_bblockinghit _binitialoverlap _time _distance _location _impactpoint _normal) (`GameplayStatics.BreakHitResult` _outhit))
      (set `self.Wall Location` _location)
      (set `self.Wall Normal` _normal)
      ;[0 1 0.05664] Check for middle point of wall
      (bind (_outhit_2 _returnvalue_5) (`KismetSystemLibrary.SphereTraceSingle` :`Start` (+ _returnvalue_3 (0.0 0.0 200.0)) :`End` _returnvalue_3 :`Radius` 20.0 :`TraceChannel` "TraceTypeQuery4" :`bTraceComplex` true :`DrawDebugType` "Persistent" :`TraceHitColor` (struct :`R` 0.277204 :`G` 0.100721 :`B` 1.0 :`A` 1.0)))
      (if _returnvalue_5
        (bind _output_get (set `self.MiddleHit` (`.Location` (`GameplayStatics.BreakHitResult` _outhit_2))))
        (`KismetSystemLibrary.PrintString` (`KismetStringLibrary.Conv_VectorToString` _output_get))
        (`|ExecutionSequence`
          (:`then_0`
            ;[0 1 0.05664] Check if the top of the wall is a valid vault location
            (if (< (* (.z (- (`self.Wall Location`) (`self.MiddleHit`))) -1.0) (`self.HeightValue`))
              (set `self.ShouldVault` true)
              (else
                (set `self.ShouldVault` false))))
          (:`then_1`
            (`|ExecutionSequence`
              (:`then_0`
                ;[1 1 1] Checking to see how high the wall is
                (if (< (.z (- (`self.MiddleHit`) (`self.EndHit`))) 30.0)
                  (set `self.IsWallThick` true)
                  (else
                    (set `self.IsWallThick` false))))
              (:`then_1`
                (if (`self.ShouldVault`)
                  (set `self.VaultingCheck` true))))))))))

(fn `CancelVault`
  (bind _returnvalue (`self.GetOwner`))
  (set `self.VaultingCheck` false)
  (set `self.VaultingSpeed` 0.0)
  (`Actor.SetActorEnableCollision` _returnvalue true)
  (`CharacterMovementComponent.SetMovementMode` (`Actor.GetComponentByClass` _returnvalue "/Script/Engine.CharacterMovementComponent") "MOVE_Walking" 0)
  (set `self.SomethingHit` false)
  (return))

(fn `Vault Tick`
  (params (Tick :type "Float (single-precision)"))
  (locals (`SecondLerp?` :type Boolean))
  (bind (_middlehit_x _middlehit_y _middlehit_z) (`KismetMathLibrary.BreakVector` (`self.MiddleHit`)))
  (if (`self.VaultingCheck`)
    (if (`self.IsWallThick`)
      (set `self.VaultingSpeed` (+ (`self.VaultingSpeed`) 0.1))
      (`Actor.K2_SetActorLocation` (`self.GetOwner`) (`KismetMathLibrary.VLerp` (`Actor.K2_GetActorLocation` (`self.GetOwner`)) (`KismetMathLibrary.MakeVector` _middlehit_x _middlehit_y (+ _middlehit_z 174.0)) Tick) false false)
      (if (> (`self.VaultingSpeed`) 7.0)
        (`KismetSystemLibrary.PrintString` "true")
        (set `self.VaultingSpeed` (+ (`self.VaultingSpeed`) 0.1))
        (`Actor.K2_SetActorLocation` (`self.GetOwner`) (`KismetMathLibrary.VLerp` (`Actor.K2_GetActorLocation` (`self.GetOwner`)) (`self.EndHit`) (`local.Tick`)) false false)
        (if (> (`self.VaultingSpeed`) 30.0)
          (`self.CancelVault` :!label _label)
          (return)))
      (else
        (set `self.VaultingSpeed` (+ (`self.VaultingSpeed`) 0.1))
        (`Actor.K2_SetActorLocation` (`self.GetOwner`) (`KismetMathLibrary.VLerp` (`Actor.K2_GetActorLocation` (`self.GetOwner`)) (`self.EndHit`) Tick) false false)
        (if (> (`self.VaultingSpeed`) 5.0)
          (goto _label))))))