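; Quest turn-in component that lets its owner accept quest items for its listed objectives.
; ActorToCheck matches an item's quest IDs against those objectives, then notifies quest managers, clears the item's waypoint, turns thieves into villagers and plays a sound.
; Helpers take the player's held item, drop it at a location tagged Delivered with effects, and create an objective icon widget.
; CheckTurninAllowance signals completion whenever the allowance is positive; SendActorName is an empty stub.
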(fn `Actor to Check`
  (params (OverlappedActor :type "Actor Object Reference"))
  (returns (IsQuestItem :type Boolean))
  (locals (Increment :type Integer))
  (bind _returnvalue (`Actor.GetComponentByClass` OverlappedActor "/Game/Components/ActorComponents/AC_Questitem.AC_Questitem_C"))
  ;[1 1 1] Check to see if the given item has a quest item component, if not get the fuck out
  (`/Engine/EditorBlueprintResources/StandardMacros.IsValid` OverlappedActor
    (:`Is Valid`
      (if (and (`KismetSystemLibrary.IsValid` OverlappedActor) (`KismetSystemLibrary.IsValid` _returnvalue) (not (`KismetArrayLibrary.Array_Contains` (`self.GivenItems`) OverlappedActor)))
        (bind _outactors (`GameplayStatics.GetAllActorsOfClass` "/Game/RodgerL/BP_QuestManager.BP_QuestManager_C"))
        (set `self.SendToQuestManagers` _outactors)
        ;[1 1 1] Loop through the actors ID array and compare it, one by one to the delivery volumes
        (for _array_element (`/Game/Components/ActorComponents/AC_Questitem.ActorQuestIDS` _returnvalue) :!label _label
          (if (== _array_element (`|GetArrayItem` (`self.ObjectiveName`) (`local.Increment`)))
            (`KismetArrayLibrary.Array_AddUnique` (`self.GivenItems`) OverlappedActor)
            (for _array_element_2 (`self.SendToQuestManagers`)
              (if (`self.ShouldCountActor`)
                (message `/Game/Utility/Interfaces/BPI_Quest.QuestUpdate` _array_element_2 _array_element)))
            (message `/Game/Utility/Interfaces/BPI_Quest.TurnOnWaypoints` (`local.OverlappedActor`) _array_element false)
            (bind _outactors_2 (`GameplayStatics.GetAllActorsOfClass` "/Game/Characters/BP_Thief.BP_Thief_C"))
            (for _array_element_3 _outactors_2
              (message `/Game/AI/BPI/BPI_Villager_Switch_States.Thief_Becomes_Villager` _array_element_3))
            (`GameplayStatics.PlaySoundAtLocation` (`self.QuestTurnInSound`) (`Actor.K2_GetActorLocation` (`self.GetOwner`)) (struct) 1.0 1.0 0.0 null null null null)
            (return true)))
        (bind _output_get (set `local.Increment` (+ (`local.Increment`) 1)))
        (if (`KismetArrayLibrary.Array_IsValidIndex` (`self.ObjectiveName`) _output_get)
          (goto _label)
          (else
            (return false)))
        (else
          (return false))))))

(fn `CheckTurninAllowance`
  (locals (CheckingNum :type Integer))
  (if (> (`self.TurnInAllowance`) 0)
    (bind _output_get (set `local.CheckingNum` (+ (`self.TurnInAllowance`) 1)))
    (if (>= _output_get (`self.TurnInAllowance`))
      (`self.TurninFinished`)
      (for _array_element (`self.ObjectiveName`)
        (message `/Game/Utility/Interfaces/BPI_Quest.TurnOnWaypoints` (`self.GetOwner`) _array_element false))
      (return)
      (else
        (return)))
    (else
      (return))))

(fn `CreateWidget`
  (returns (Output_Get :type "/Game/UI/Icons/W_MainObjectiveIcon Object Reference"))
  (bind _returnvalue (`|CreateWidget` "/Game/UI/Icons/W_MainObjectiveIcon.W_MainObjectiveIcon_C" (`GameplayStatics.GetPlayerController` 0)))
  (bind _output_get (set `self.TurninIcon` _returnvalue))
  (set `/Game/UI/Icons/W_MainObjectiveIcon.OwningActor` (`self.GetOwner`) _output_get)
  (return _output_get))

(fn `MoveActorToLocation`
  (params (NewLocation :type "Vector Structure") (ShouldPlayVFX :type Boolean))
  (locals (`Held Actor` :type "Actor Object Reference"))
  (bind _currentactor (`self.PassOutActorReference`))
  (`/Engine/EditorBlueprintResources/StandardMacros.IsValid` _currentactor
    (:`Is Valid`
      (bind _output_get (set `local.Held Actor` _currentactor))
      (`self.MoveActorToLocationFunction` _output_get NewLocation)
      (if (`local.ShouldPlayVFX`)
        (`NiagaraFunctionLibrary.SpawnSystemAtLocation` (`self.QuestTurninVFX`) NewLocation))
      (return))))

(fn `MoveActorToLocationFunction`
  (params (ActorToMove :type "Actor Object Reference") (DropLocation :type "Vector Structure"))
  (message `/Game/Utility/Interfaces/BPI_EPS.ItemDropped` ActorToMove DropLocation)
  (`KismetArrayLibrary.Array_Add` (`Actor.Tags` ActorToMove) "Delivered")
  (`GameplayStatics.PlaySoundAtLocation` "/Game/SFX/QuestRelated/kazoocelebration.kazoocelebration" DropLocation (struct) 1.0 1.0 0.0 null null null null))

(fn `PassOutActorReference`
  (returns (CurrentActor :type "Actor Object Reference"))
  (bind _asbp_player_char (cast `/Game/Characters/BP_PlayerChar` (`GameplayStatics.GetPlayerCharacter` 0)))
  (`/Engine/EditorBlueprintResources/StandardMacros.IsValid` (`/Game/Characters/BP_ActiveChar.Current Item` _asbp_player_char)
    (:`Is Valid`
      (bind _tempcurrentitem1 (`/Game/Characters/BP_ActiveChar.GiveItem` _asbp_player_char))
      (return _tempcurrentitem1))
    (:`Is Not Valid`
      (return null))))

(fn `SendActorName`
  (params (`Object To Save` :type "Actor Object Reference") (VectorToSave :type "Vector Structure"))
  (return))