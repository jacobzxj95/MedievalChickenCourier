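; Actor component that serves as a quest log, starting, tracking and completing quests.
; AddNewQuest records the quest ID, spawns a BP_QuestManager actor with that row ID and save data, binds its completion event and fires QuestStarted.
; CompleteQuest removes and destroys the manager but leaves its ID in CurrentActiveQuest, which QueryActiveQuest checks.
; QuestFailed is an empty stub.
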(fn `AddNewQuest`
  (params (QuestID :type Name) (LoadedData :type "/Game/Utility/Struct/STR_SaveData Structure"))
  (returns (`Newly Added Quest` :type "/Game/RodgerL/BP_QuestManager Object Reference"))
  (`KismetArrayLibrary.Array_AddUnique` (`self.CurrentActiveQuest`) QuestID)
  (bind _returnvalue (`|SpawnActorFromClass` "/Game/RodgerL/BP_QuestManager.BP_QuestManager_C" (`KismetMathLibrary.MakeTransform` (0.0 0.0 -100.0)) "Undefined" "OverrideRootScale" null QuestID LoadedData null))
  (add `/Game/RodgerL/BP_QuestManager.QuestCompleted` _returnvalue (`|CreateDelegate` :!event `BoundQuestEvent`))
  (`KismetArrayLibrary.Array_Add` (`self.CurrentQuests`) _returnvalue)
  (`self.Quest Started` _returnvalue)
  (`KismetSystemLibrary.PrintString` "event called" true true (struct :`G` 0.66 :`B` 1.0 :`A` 1.0) 10.0)
  (return _returnvalue))

(fn `BoundQuestEvent`
  (params (Manager :type "/Game/RodgerL/BP_QuestManager Object Reference"))
  (`self.CompleteQuest` Manager))

(fn `CompleteQuest`
  (params (`Quest That Was Completed` :type "/Game/RodgerL/BP_QuestManager Object Reference (by ref)"))
  (if (`KismetArrayLibrary.Array_Contains` (`self.CurrentQuests`) `Quest That Was Completed`)
    (`KismetArrayLibrary.Array_RemoveItem` (`self.CurrentQuests`) `Quest That Was Completed`)
    (`Actor.K2_DestroyActor` `Quest That Was Completed`)))

(fn `QueryActiveQuest`
  (params (QuestID :type Name))
  (returns (`HasQuest?` :type Boolean))
  (return (`KismetArrayLibrary.Array_Contains` (`self.CurrentActiveQuest`) QuestID)))

(fn `Quest Failed`)