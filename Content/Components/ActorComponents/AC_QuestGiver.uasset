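; AC_QuestGiver is an actor component that lets its owner offer a quest to the player.
; It creates a W_QuestDialogue widget at BeginPlay, then fills it from the QuestToGive data table row and shows it with mouse cursor and UI input.
; QuestInteraction opens the dialogue unless the player's quest turn-in component reports the quest active, and returns the owner's display name.
; A helper hides quest marker actors.
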(event `self.ReceiveBeginPlay`
  (bind _returnvalue (`|CreateWidget` "/Game/UI/Dialogue/W_QuestDialogue.W_QuestDialogue_C"))
  (set `self.QuestWidget` _returnvalue))

(fn `DisplayQuest`
  (bind _returnvalue (`GameplayStatics.GetPlayerController` 0))
  (bind (_questtogive_datatable _questtogive_rowname) (break `DataTableRowHandle` (`self.QuestToGive`)))
  (bind _questwidget (`self.QuestWidget`))
  (bind _questwidget_2 (`self.QuestWidget`))
  (bind _returnvalue_2 (`|GetDataTableRow` _questtogive_datatable _questtogive_rowname)
    (:`then`
      (set `/Game/UI/Dialogue/W_QuestDialogue.BPQuestGiver` (`self.GetOwner`) _questwidget)
      (set `/Game/UI/Dialogue/W_QuestDialogue.Quest ID` _questtogive_rowname _questwidget)
      (set `/Game/UI/Dialogue/W_QuestDialogue.QuestData` _returnvalue_2 _questwidget)
      (`UserWidget.AddToViewport` _questwidget_2 0)
      (set `PlayerController.bShowMouseCursor` true _returnvalue)
      (`WidgetBlueprintLibrary.SetInputMode_GameAndUIEx` _returnvalue _questwidget_2))))

(fn `HideQuestMarker`
  (params (`Quest Marker` :type "Actor Object Reference"))
  (`Actor.SetActorHiddenInGame` `Quest Marker` true))

(fn `QuestInteraction`
  (returns (ObjectiveID :type String))
  (locals (HasQuest :type Boolean))
  (bind (_questtogive_datatable _questtogive_rowname) (break `DataTableRowHandle` (`self.QuestToGive`)))
  (bind _returnvalue (`KismetSystemLibrary.GetDisplayName` (`self.GetOwner`)))
  (bind _asbp_player_char (cast `/Game/Characters/BP_PlayerChar` (`GameplayStatics.GetPlayerCharacter` 0)))
  (if (not (`/Game/Components/ActorComponents/AC_Questlog.QueryActiveQuest` (`/Game/Characters/BP_PlayerChar.AC_QuestTurnIn` _asbp_player_char) _questtogive_rowname))
    (`self.DisplayQuest`)
    (return _returnvalue)
    (else
      (`KismetSystemLibrary.PrintString` "AlreadyOnQuest")
      (return _returnvalue))))