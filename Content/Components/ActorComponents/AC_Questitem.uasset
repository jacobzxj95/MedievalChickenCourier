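; Actor component that links its owning actor to quests through a list of quest IDs.
; After a short delay on BeginPlay, it tags the owner as the current quest item if flagged as needed.
; It sends a chosen ID to every BP_QuestManager and shows or hides a waypoint when an objective ID matches, tracking the enabled state.
; It also creates an objective icon widget bound to the owner.
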(event `self.ReceiveBeginPlay`
  (`KismetSystemLibrary.Delay` 3.0)
  (if (`self.NeededForQuest?`)
    (`KismetArrayLibrary.Array_AddUnique` (`Actor.Tags` (`self.GetOwner`)) "CurrentQuestItem")))

(fn `Check To Turn On Waypoints`
  (params (WaypointActor :type "WidgetComponent Object Reference") (`On/Off` :type Boolean) (ObjectiveID :type String))
  (for _array_element (`self.ActorQuestIDS`)
    (if (`KismetStringLibrary.EqualEqual_StrStr` _array_element ObjectiveID)
      (if `On/Off`
        (`self.On Off Waypoint` WaypointActor true)
        (else
          (`self.On Off Waypoint` WaypointActor))))))

(fn `CreateWidget`
  (returns (Output_Get :type "/Game/UI/Icons/W_MainObjectiveIcon Object Reference"))
  (bind _returnvalue (`|CreateWidget` "/Game/UI/Icons/W_MainObjectiveIcon.W_MainObjectiveIcon_C"))
  (bind _output_get (set `self.TurninIcon` _returnvalue))
  (set `/Game/UI/Icons/W_MainObjectiveIcon.OwningActor` (`self.GetOwner`) _output_get)
  (return _output_get))

(fn `On Off Waypoint`
  (params (Widget :type "SceneComponent Object Reference") (`On/Off` :type Boolean))
  (if `On/Off`
    (`SceneComponent.SetHiddenInGame` Widget false false)
    (set `self.IsQuestEnabled` true)
    (else
      (`SceneComponent.SetHiddenInGame` Widget true false)
      (set `self.IsQuestEnabled` false))))

(fn `Send ID`
  (params (Index :type Integer))
  (bind _outactors (`GameplayStatics.GetAllActorsOfClass` "/Game/RodgerL/BP_QuestManager.BP_QuestManager_C"))
  (for _array_element _outactors
    (message `/Game/Utility/Interfaces/BPI_Quest.QuestUpdate` _array_element (`|GetArrayItem` (`self.ActorQuestIDS`) Index))))