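; Actor component that lets its owner pick up, carry, drop and hand over interactable items, intended mainly for chickens.
; GrabItem checks the Interactable tag, notifies the item, attaches it to a skeletal mesh socket (separate one for eggs) and shrinks non-chickens.
; DropItem notifies and detaches the held item, while GiveItem transfers items through the receiver's copy of this component.
; A temporary reference feeds the held-object variable and clears on a short timer.
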(event `GrabItem`
  (params (HitItem :type "Actor Object Reference"))
  ;[1 0.1309 0.001194] check if overlapping actors have tag "interactable" if they do, attach to player charecter, set as currently held item. This is specifically made for chickens, and is sperate to any other item pick/throw code
  (if (and (`Actor.ActorHasTag` HitItem "Interactable") (not (`self.Is Holding?`)))
    (set `self.CurrentHeldObject` HitItem)
    (set `self.RegularScale` (`Actor.GetActorScale3D` (`self.CurrentHeldObject`)))
    (message `/Game/Utility/Interfaces/BPI_EPS.ItemPickedUp` (`self.CurrentHeldObject`) null false false)
    (`self.AttachActor` (`self.GetOwner`) (`self.CurrentHeldObject`))
    (if (not (== (`GameplayStatics.GetObjectClass` (`self.CurrentHeldObjectTemp`)) "/Game/AI/AICharacters/BP_AI_Chicken.BP_AI_Chicken_C"))
      (`Actor.SetActorScale3D` (`self.CurrentHeldObjectTemp`) (0.5 0.5 0.5)))))

(event `Drop Item`
  ;[1 0.1309 0.001194] Drop Chicken Actor
  (if (`self.Is Holding?`)
    (message `/Game/Utility/Interfaces/BPI_EPS.ItemDropped` (`self.CurrentHeldObject`) (0.0 0.0 0.0))
    (`self.Detach Actor`)
    (set `self.CurrentHeldObject` null)))

(event `Detach Actor`
  (bind _currentheldobject (`self.CurrentHeldObject`))
  ;[1 0.1309 0.001194] Drop Chicken Actor
  (`/Engine/EditorBlueprintResources/StandardMacros.IsValid` _currentheldobject
    (:`Is Valid`
      (`Actor.K2_DetachFromActor` _currentheldobject "KeepWorld" "KeepWorld" "KeepWorld")
      (set `self.Is Holding?` false))))

(event `AttachActor`
  (params (ActorToGiveTo :type "Actor Object Reference") (ItemToGive :type "Actor Object Reference"))
  ;[1 0.1309 0.001194] Attach Object
  (set `self.CurrentHeldObjectTemp` ItemToGive)
  (if (== (`self.CurrentHeldObjectTemp`) "/Game/LevelObjects/EnviormentalPickups/BP_Egg.BP_Egg_C")
    (`Actor.K2_AttachToComponent` (`self.CurrentHeldObjectTemp`) (`Actor.GetComponentByClass` ActorToGiveTo "/Script/Engine.SkeletalMeshComponent") "eggSocket" "SnapToTarget" "SnapToTarget" "KeepWorld" true)
    (else
      (`Actor.K2_AttachToComponent` (`self.CurrentHeldObjectTemp`) (`Actor.GetComponentByClass` ActorToGiveTo "/Script/Engine.SkeletalMeshComponent") "ActorLoc" "SnapToTarget" "SnapToTarget" "KeepWorld" true)))
  (set `self.Is Holding?` true)
  (`self.Update References`)
  (`KismetSystemLibrary.K2_SetTimer` null "ClearReferences" 0.5))

(event `ClearReferences`
  ;[1 1 1] Clear References
  (set `self.CurrentHeldObjectTemp` null))

(event `GiveItem`
  (params (ActorToGiveTo :type "Actor Object Reference") (ItemToGive :type "Actor Object Reference"))
  (bind _returnvalue (`Actor.GetComponentByClass` ActorToGiveTo "AC_PickupChicken_C"))
  ;[1 1 1] Comment
  (if (`self.Is Holding?`)
    (`self.Detach Actor`)
    (else
      (`self.Detach Actor` _returnvalue)))
  (`self.AttachActor` _returnvalue ActorToGiveTo ItemToGive))

(event `Update References`
  ;[1 1 1] Update References
  (set `self.CurrentHeldObject` (`self.CurrentHeldObjectTemp`)))

(fn `HasGoldenChicken`
  (return))

(fn `PickupChicken`
  (returns (`Currently being held` :type Boolean))
  (return false))