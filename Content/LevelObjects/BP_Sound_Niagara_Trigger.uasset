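; BP_Sound_Niagara_Trigger is a level trigger volume that starts a Niagara effect and two sounds when the player pawn enters.
; A DoOnce gates the start: it activates the effect and plays the first sound, then the second after a short delay, skipping any already playing.
; Any end overlap, not filtered to the player, fades both sounds out, deactivates the effect and re-arms the gate after a cooldown.
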(event `self.Volume.OnComponentBeginOverlap`
  (params (OverlappedComponent :type "PrimitiveComponent Object Reference") (OtherActor :type "Actor Object Reference") (OtherComp :type "PrimitiveComponent Object Reference") (OtherBodyIndex :type Integer) (bFromSweep :type Boolean) (SweepResult :type "HitResult Structure (by ref)"))
  (bind _sound1 (`self.Sound1`))
  (bind _sound2 (`self.Sound2`))
  (if (== OtherActor (`GameplayStatics.GetPlayerPawn` 0))
    (`/Engine/EditorBlueprintResources/StandardMacros.DoOnce` false :!label _label
      (:`Completed`
        (`ActorComponent.Activate` (`self.NiagaraSystem`) true)
        (if (not (`AudioComponent.IsPlaying` _sound1))
          (`AudioComponent.Play` _sound1 (`self.Start Time_1`))
          (`KismetSystemLibrary.Delay` 0.2)
          (if (not (`AudioComponent.IsPlaying` _sound2))
            (`AudioComponent.Play` _sound2 (`self.Start Time_2`))))))))

(event `AllowReset`
  (goto _label :!via `Reset`))

(event `self.Volume.OnComponentEndOverlap`
  (params (OverlappedComponent :type "PrimitiveComponent Object Reference") (OtherActor :type "Actor Object Reference") (OtherComp :type "PrimitiveComponent Object Reference") (OtherBodyIndex :type Integer))
  (`AudioComponent.FadeOut` (`self.Sound1`) 2.0 0.0 "Linear")
  (`AudioComponent.FadeOut` (`self.Sound2`) 2.0 0.0 "Linear")
  (`ActorComponent.Deactivate` (`self.NiagaraSystem`))
  (`KismetSystemLibrary.Delay` 10.0)
  (`self.AllowReset`))

(fn `UserConstructionScript`)