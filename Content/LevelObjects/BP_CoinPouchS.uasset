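; BP_CoinPouchS is a one-time currency pickup that bobs on a timeline and is scaled by its currency value within clamped limits.
; Overlap by the player pawn or Golden Chicken boomerang adds currency through the game mode and plays a Niagara burst and sound.
; After a short delay it saves its display name to the game instance and destroys itself.
; When GM_MVP broadcasts Loaded, it self-destructs if that name is among the map's keys.
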(event `self.ReceiveBeginPlay`
  (bind (_returnvalue_x _returnvalue_y _returnvalue_z) (`KismetMathLibrary.BreakVector` (`SceneComponent.K2_GetComponentLocation` (`self.CoinPurse`))))
  (bind _asgm_mvp (cast `/Game/Maps/GameModes/GM_MVP` (`GameplayStatics.GetGameMode`)))
  (add `/Game/Maps/GameModes/GM_MVP.Loaded` _asgm_mvp (delegate `Loaded`))
  (bind (_direction _float_track) (`Timeline|FloatTL`)
    (:`Update`
      (`self.K2_SetActorRelativeLocation` (`KismetMathLibrary.MakeVector` _returnvalue_x _returnvalue_y (`KismetMathLibrary.Lerp` (- _returnvalue_z 1.0) (+ _returnvalue_z 1.0) _float_track))))))

(event `Loaded`
  (params (`Actor Map` :type "Map of String to Boolean"))
  (bind _keys (`BlueprintMapLibrary.Map_Keys` `Actor Map`))
  (for _array_element _keys
    (if (`KismetStringLibrary.EqualEqual_StrStr` _array_element (`KismetSystemLibrary.GetDisplayName` self))
      (`self.K2_DestroyActor`))))

(event `self.ReceiveTick`
  (params (DeltaSeconds :type "Float (single-precision)")))

(event `self.Box.OnComponentBeginOverlap`
  (params (OverlappedComponent :type "PrimitiveComponent Object Reference") (OtherActor :type "Actor Object Reference") (OtherComp :type "PrimitiveComponent Object Reference") (OtherBodyIndex :type Integer) (bFromSweep :type Boolean) (SweepResult :type "HitResult Structure (by ref)"))
  (bind _niagaracoinburst (`self.NiagaraCoinBurst`))
  (if (or (== (`GameplayStatics.GetPlayerPawn` 0) OtherActor) (== (`GameplayStatics.GetObjectClass` OtherActor) "/Game/AI/AICharacters/BP_GoldenChicken_Boomerang.BP_GoldenChicken_Boomerang_C"))
    (`/Engine/EditorBlueprintResources/StandardMacros.DoOnce` false
      (:`Completed`
        (`SceneComponent.SetHiddenInGame` (`self.CoinPurse`) true false)
        (message `/Game/Utility/Interfaces/BPI_UI.UpdateCurrency` (`GameplayStatics.GetGameMode`) (`self.CurrencyToAdd`))
        (`ActorComponent.Activate` _niagaracoinburst false)
        (`GameplayStatics.PlaySound2D` "/Game/SFX/Collectibles/ES_Lighter_Flick_-_SFX_Producer.ES_Lighter_Flick_-_SFX_Producer" 1.0 1.0 0.0 null null)
        (`KismetSystemLibrary.Delay` 0.5)
        (`ActorComponent.Deactivate` _niagaracoinburst)
        (`SceneComponent.SetHiddenInGame` (`self.DefaultSceneRoot`) true false)
        (bind _asbp_game_instance (cast `/Game/Utility/GameModes/BP_GameInstance` (`GameplayStatics.GetGameInstance`)))
        (`/Game/Utility/GameModes/BP_GameInstance.SaveObjectData` _asbp_game_instance (`KismetStringLibrary.Conv_StringToName` (`KismetSystemLibrary.GetDisplayName` self)) true)
        (`self.K2_DestroyActor`)))))

(fn `UserConstructionScript`
  (`SceneComponent.SetWorldScale3D` (`self.CoinPurse`) (* (`self.DefaultScale`) (`KismetMathLibrary.FClamp` (/ (`KismetMathLibrary.Conv_IntToDouble` (`self.CurrencyToAdd`)) 2.0) 1.0 2.0))))