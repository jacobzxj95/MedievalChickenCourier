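; BP_LevelTransition is a level exit that asks the player for confirmation on entering its volume.
; Once a started quest completes, it reveals an objective icon widget labelled as the exit.
; A separate volume toggles warning text, while overlapping the transition volume opens a confirmation widget holding a reference to this actor.
; ExitLevellll copies actor tags into the game instance's player start tag, stops music and opens the target level.
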(event `QuestStarted`
  (params (ActiveQuest :type "/Game/RodgerL/BP_QuestManager Object Reference"))
  (add `/Game/RodgerL/BP_QuestManager.QuestCompleted` ActiveQuest (delegate `ShowIcon`)))

(event `ShowIcon`
  (params (Manager :type "/Game/RodgerL/BP_QuestManager Object Reference"))
  (bind _objectiveicon (`self.ObjectiveIcon`))
  (`SceneComponent.SetHiddenInGame` (`self.Widget`) false false)
  (`/Game/UI/Icons/W_MainObjectiveIcon.TurnOnObjectiveIcon` _objectiveicon 2)
  (`/Game/UI/Icons/W_MainObjectiveIcon.TurnOnLevelName` _objectiveicon (`self.Exit`)))

(event `self.ReceiveBeginPlay`
  (bind _asbp_game_instance (cast `/Game/Utility/GameModes/BP_GameInstance` (`GameplayStatics.GetGameInstance`)))
  (set `self.GameInstance_Ref` _asbp_game_instance)
  (bind _returnvalue (`|CreateWidget` "/Game/UI/Icons/W_MainObjectiveIcon.W_MainObjectiveIcon_C"))
  (bind _output_get (set `self.ObjectiveIcon` _returnvalue))
  (set `/Game/UI/Icons/W_MainObjectiveIcon.OwningActor` self _returnvalue)
  (`WidgetComponent.SetWidget` (`self.Widget`) _output_get)
  (bind _asbp_player_char (cast `/Game/Characters/BP_PlayerChar` (`GameplayStatics.GetPlayerCharacter` 0)))
  (add `/Game/Components/ActorComponents/AC_Questlog.Quest Started` (`/Game/Characters/BP_PlayerChar.AC_QuestTurnIn` _asbp_player_char) (delegate `QuestStarted`)))

(event `self.LevelTransitionVolume.OnComponentBeginOverlap`
  (params (OverlappedComponent :type "PrimitiveComponent Object Reference") (OtherActor :type "Actor Object Reference") (OtherComp :type "PrimitiveComponent Object Reference") (OtherBodyIndex :type Integer) (bFromSweep :type Boolean) (SweepResult :type "HitResult Structure (by ref)"))
  ;[1 0 0.8195] Open Next Level
  (if (== OtherActor (`GameplayStatics.GetPlayerPawn` 0))
    (bind _returnvalue (`|CreateWidget` "/Game/UI/W_LevelExitConfirmation.W_LevelExitConfirmation_C" (`GameplayStatics.GetPlayerController` 0)))
    (bind _output_get (set `self.Conf Widget` _returnvalue))
    (`UserWidget.AddToViewport` _output_get 0)
    (set `/Game/UI/W_LevelExitConfirmation.Level transition` self _output_get)))

(event `self.MessageVolume.OnComponentBeginOverlap`
  (params (OverlappedComponent :type "PrimitiveComponent Object Reference") (OtherActor :type "Actor Object Reference") (OtherComp :type "PrimitiveComponent Object Reference") (OtherBodyIndex :type Integer) (bFromSweep :type Boolean) (SweepResult :type "HitResult Structure (by ref)"))
  ;[1 0.7916 0.1382] Reveal and hide warning message on overlap
  (if (== OtherActor (`GameplayStatics.GetPlayerPawn` 0))
    (`SceneComponent.SetHiddenInGame` (`self.PlaceHolderText`) false false)))

(event `self.MessageVolume.OnComponentEndOverlap`
  (params (OverlappedComponent :type "PrimitiveComponent Object Reference") (OtherActor :type "Actor Object Reference") (OtherComp :type "PrimitiveComponent Object Reference") (OtherBodyIndex :type Integer))
  ;[1 0.7916 0.1382] Reveal and hide warning message on overlap
  (if (== OtherActor (`GameplayStatics.GetPlayerPawn` 0))
    (`SceneComponent.SetHiddenInGame` (`self.PlaceHolderText`) true false)))

(fn `ExitLevellll`
  (bind _tags (`self.Tags`))
  (for (_array_element _array_index) _tags
    (if (`KismetArrayLibrary.Array_IsValidIndex` _tags _array_index)
      (bind _gameinstance_ref (`self.GameInstance_Ref`)
        (:`then`
          (set `/Game/Utility/GameModes/BP_GameInstance.PlayerStartTag` _array_element _gameinstance_ref)
          (`/Game/Utility/GameModes/BP_GameInstance.UpdatePlayerStartTag` _gameinstance_ref))
        (:`else`
          (`KismetSystemLibrary.PrintString` "Level Transition BP: INVALID GAME INSTANCE REF" true true (struct :`R` 1.0 :`G` 0.064346 :`A` 1.0) 7.0)))))
  (`/Game/Utility/GameModes/BP_GameInstance.Stop Music` (`self.GameInstance_Ref`))
  (`GameplayStatics.OpenLevelBySoftObjectPtr` (`self.Level`)))

(fn `UserConstructionScript`
  (`TextRenderComponent.K2_SetText` (`self.PlaceHolderText`) (`self.WarningText`)))