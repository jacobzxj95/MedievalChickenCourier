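; Environmental prop the player can pick up, drop and throw as a projectile, with its MeshEnum variant setting mesh, materials and effects at construction.
; Box overlap shows the interact prompt, and a look-at dot product on Tick drives the highlight.
; Thrown hits stun or goop BPI_Hit targets, or reduce durability until it breaks, optionally spawning coins.
; A velocity-polling timer ends physics, Fall cascades to props above, and ACQuestitem handles quest reporting and waypoints.
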(event `self.ReceiveTick`
  (params (DeltaSeconds :type "Float (single-precision)"))
  ;[1 1 1] Tick
  (bind _inversedotproduct (`self.IsPlayerLookingAtMe`))
  (if (and (`self.InRange?`) (> _inversedotproduct 0.9))
    (bind _returnvalue (`PrimitiveComponent.CreateDynamicMaterialInstance` (`self.StaticMesh`) (`self.HighlightMaterialIndex`) "/Game/Art/Materials/M_HighlightColor.M_HighlightColor" "None"))
    (`PrimitiveComponent.SetMaterial` (`self.StaticMesh`) (`self.HighlightMaterialIndex`) _returnvalue)
    (else
      (`PrimitiveComponent.SetMaterial` (`self.StaticMesh`) (`self.HighlightMaterialIndex`) (`self.RegularMaterial`)))))

(event `self.Box.OnComponentBeginOverlap`
  (params (OverlappedComponent :type "PrimitiveComponent Object Reference") (OtherActor :type "Actor Object Reference") (OtherComp :type "PrimitiveComponent Object Reference") (OtherBodyIndex :type Integer) (bFromSweep :type Boolean) (SweepResult :type "HitResult Structure (by ref)"))
  ;[1 1 1] EPS Collision Overlap
  (if (== OtherActor (`GameplayStatics.GetPlayerPawn` 0))
    (set `self.InRange?` true)
    (bind _asgm_mvp (cast `/Game/Maps/GameModes/GM_MVP` (`GameplayStatics.GetGameMode`)))
    (`Widget.SetVisibility` (`/Game/UI/W_HUD.EtoInteract` (`/Game/Maps/GameModes/GM_MVP.PlayerHUD` _asgm_mvp)) "Visible")))

(event `self.Box.OnComponentEndOverlap`
  (params (OverlappedComponent :type "PrimitiveComponent Object Reference") (OtherActor :type "Actor Object Reference") (OtherComp :type "PrimitiveComponent Object Reference") (OtherBodyIndex :type Integer))
  ;[1 1 1] EPS Collision Overlap
  (if (== OtherActor (`GameplayStatics.GetPlayerPawn` 0))
    (set `self.InRange?` false)
    (bind _asgm_mvp (cast `/Game/Maps/GameModes/GM_MVP` (`GameplayStatics.GetGameMode`)))
    (`Widget.SetVisibility` (`/Game/UI/W_HUD.EtoInteract` (`/Game/Maps/GameModes/GM_MVP.PlayerHUD` _asgm_mvp)) "Hidden")))

(event `/Game/Utility/Interfaces/BPI_EPS.ItemPickedUp`
  (params (CurrentChicken :type "Actor Object Reference") (`CapturingChicken?` :type Boolean) (`HasChicken?` :type Boolean))
  (bind _ac_questitem (`self.AC_Questitem`))
  ;[1 0.2304 0.1407] Pickup Interface
  (`PrimitiveComponent.SetSimulatePhysics` (`self.StaticMesh`) false)
  (`KismetSystemLibrary.K2_ClearAndInvalidateTimerHandle` (`self.SimulationTimer`))
  (`self.ResetHitEvent`)
  (`self.Renable/DisableCollision` false)
  (`SceneComponent.SetHiddenInGame` (`self.Billboard`) true true)
  (`/Game/Components/ActorComponents/AC_Questitem.Send ID` (`self.AC_Questitem`) 0)
  (set `self.IsBeingHeld` true)
  (if (`/Game/Components/ActorComponents/AC_Questitem.IsQuestEnabled` _ac_questitem)
    (`SceneComponent.SetHiddenInGame` (`self.Widget`) true false)
    (set `/Game/Components/ActorComponents/AC_Questitem.IsQuestEnabled` false _ac_questitem)))

(event `self.ReceiveBeginPlay`
  ;[1 1 1] Begin play
  (`KismetSystemLibrary.DelayUntilNextTick` :!label _label)
  (bind _asbp_player_char (cast `/Game/Characters/BP_PlayerChar` (`GameplayStatics.GetPlayerCharacter` 0))
    (:`then`
      (set `self.PlayerChar` _asbp_player_char))
    (:`CastFailed`
      (goto _label))))

(event `/Game/Utility/Interfaces/BPI_EPS.ItemDropped`
  (params (DropLocation :type "Vector Structure"))
  (bind _ac_questitem (`self.AC_Questitem`))
  (bind (_returnvalue_roll _returnvalue_pitch _returnvalue_yaw) (`KismetMathLibrary.BreakRotator` (`KismetMathLibrary.FindLookAtRotation` (`self.K2_GetActorLocation` (`GameplayStatics.GetPlayerCharacter` 0)) DropLocation)))
  ;[1 0.2304 0.1407] Dropped Interface
  (`self.Renable/DisableCollision` true)
  (`self.K2_SetActorLocation` DropLocation)
  (`self.K2_SetActorRotation` (`KismetMathLibrary.MakeRotator` _returnvalue_roll 0.0 _returnvalue_yaw))
  (`GameplayStatics.PlaySoundAtLocation` "/Game/SFX/Mechanics/Throw_Hit_Drop/SC_FunnyHit.SC_FunnyHit" DropLocation (struct) 1.0 1.0 0.0 null null null null)
  (if (`/Game/Components/ActorComponents/AC_Questitem.IsQuestEnabled` _ac_questitem)
    (`SceneComponent.SetHiddenInGame` (`self.Widget`) false false)
    (set `/Game/Components/ActorComponents/AC_Questitem.IsQuestEnabled` true _ac_questitem)))

(event `self.StaticMesh.OnComponentHit`
  (params (HitComponent :type "PrimitiveComponent Object Reference") (OtherActor :type "Actor Object Reference") (OtherComp :type "PrimitiveComponent Object Reference") (NormalImpulse :type "Vector Structure") (Hit :type "HitResult Structure (by ref)"))
  (bind _ac_questitem (`self.AC_Questitem`))
  ;[1 1 1] Static mesh hit event
  (if (and (not (== OtherActor (`GameplayStatics.GetPlayerPawn` 0))) (`self.IsBeingThrown`))
    (`/Engine/EditorBlueprintResources/StandardMacros.DoOnce` false :!label _label_2
      (:`Completed`
        (set `self.HitLocation` (`.Location` (`GameplayStatics.BreakHitResult` Hit)))
        (if (`/Game/Components/ActorComponents/AC_Questitem.IsQuestEnabled` _ac_questitem)
          (`SceneComponent.SetHiddenInGame` (`self.Widget`) true false)
          (set `/Game/Components/ActorComponents/AC_Questitem.IsQuestEnabled` false _ac_questitem))
        (bind _returnvalue (`KismetSystemLibrary.K2_SetTimerDelegate` (delegate `ResetSimulate`) 0.1 true))
        (set `self.SimulationTimer` _returnvalue)
        (if (`KismetSystemLibrary.DoesImplementInterface` OtherActor "/Game/Utility/Interfaces/BPI_Hit.BPI_Hit_C")
          (switch `/Game/Utility/Enums/E_LevelObjects` (`self.MeshEnum`)
            (:`NewEnumerator0`
              (message `/Game/Utility/Interfaces/BPI_Hit.HitByProjectile` OtherActor (`self.Stun Duration`) :!label _label_3))
            (:`NewEnumerator1`
              (goto _label_3))
            (:`NewEnumerator2`
              (goto _label_3))
            (:`NewEnumerator3`
              (goto _label_3))
            (:`NewEnumerator4`
              (message `/Game/Utility/Interfaces/BPI_Hit.HitByGoop` OtherActor)))
          (`GameplayStatics.PlaySoundAtLocation` (`self.ImpactSound`) (`self.HitLocation`) (struct) 1.0 1.0 0.0 null null null null)
          (`self.HideActor`)
          (else
            (bind _isbroken_ (`self.DurabilityCalc`))
            (if _isbroken_
              (`self.HideActor`)
              (`KismetSystemLibrary.PrintString` (`KismetStringLibrary.Conv_VectorToString` (`self.HitLocation`))))))))))

(event `ResetHitEvent`
  ;[1 1 1] Static mesh hit event
  (goto _label_2 :!via `Reset`))

(event `/Game/Utility/Interfaces/BPI_EPS.ItemThrown`
  (params (ThrowingForce :type "Float (double-precision)") (ThrowingDirection :type "Vector Structure") (StartingTransform :type "Transform Structure") (`CatapultLaunched?` :type Boolean) (StunDuration :type "Float (double-precision)"))
  (bind _staticmesh (`self.StaticMesh`))
  ;[1 0.2304 0.1407] Setup the EPS object to be thrown
  (set `self.Stun Duration` StunDuration)
  (`self.K2_DetachFromActor` "KeepWorld" "KeepWorld" "KeepWorld")
  (`self.K2_SetActorLocationAndRotation` (.location StartingTransform) (.rotation StartingTransform))
  (`PrimitiveComponent.SetSimulatePhysics` _staticmesh true)
  (`self.SetActorScale3D` (.scale StartingTransform))
  (`PrimitiveComponent.SetCollisionEnabled` _staticmesh "QueryAndPhysics")
  (`PrimitiveComponent.SetCollisionEnabled` (`self.Box`) "QueryAndPhysics")
  (`PrimitiveComponent.AddImpulse` (`self.StaticMesh`) (* ThrowingForce ThrowingDirection) "None" true)
  (set `self.IsBeingThrown` true))

(event `ResetSimulate`
  ;[0 0.2912 1] Set simulate physics to off and let the projectile know it's no longer being thrown
  (if (< (`KismetMathLibrary.VSize` (`self.GetVelocity`)) 4.0)
    (`PrimitiveComponent.SetSimulatePhysics` (`self.StaticMesh`) false)
    (set `self.IsBeingThrown` false)
    (`self.Renable/DisableCollision` true)
    (`self.ResetHitEvent`)
    (`KismetSystemLibrary.K2_ClearAndInvalidateTimerHandle` (`self.SimulationTimer`))))

(event `HideActor`
  ;[0 0.2912 1] Hide Actor
  (`PrimitiveComponent.SetCollisionEnabled` (`self.Box`) "NoCollision")
  (`self.SetActorHiddenInGame` true)
  (`NiagaraFunctionLibrary.SpawnSystemAtLocation` (`self.DestructionVFX`) (`self.HitLocation`))
  (`GameplayStatics.PlaySoundAtLocation` (`self.ImpactSound`) (`self.HitLocation`) (struct) 1.0 1.0 0.0 null null null null)
  (`/Game/Components/ActorComponents/AC_Questitem.Send ID` (`self.AC_Questitem`) 1)
  (if (`self.ShouldSpawnCoinPouch`)
    (`|SpawnActorFromClass` "/Game/LevelObjects/BP_CoinPouchL.BP_CoinPouchL_C" (`KismetMathLibrary.MakeTransform` (`self.HitLocation`)) "Undefined" "OverrideRootScale" null null))
  (`KismetSystemLibrary.Delay` 1.2)
  (`self.K2_DestroyActor`))

(event `/Game/Utility/Interfaces/BPI_Quest.TurnOnWaypoints`
  (params (ObjectiveID :type String) (`On/Off` :type Boolean))
  ;[1 0.2304 0.1407] Turn on waypoints
  (`/Game/Components/ActorComponents/AC_Questitem.Check To Turn On Waypoints` (`self.AC_Questitem`) (`self.Widget`) `On/Off` ObjectiveID))

(event `/Game/Utility/Interfaces/BPI_EPS.Fall`
  (params (IsBeingPickedup :type Boolean))
  (bind (_returnvalue_x _returnvalue_y _returnvalue_z) (`KismetMathLibrary.BreakVector` (`self.K2_GetActorLocation`)))
  (bind _staticmesh (`self.StaticMesh`))
  (bind _returnvalue (+ (+ (`KismetMathLibrary.MakeVector` _returnvalue_x _returnvalue_y _returnvalue_z) (* (`KismetMathLibrary.LessLess_VectorRotator` (`SceneComponent.GetUpVector` _staticmesh) (`SceneComponent.K2_GetComponentRotation` _staticmesh)) 100.0)) (0.0 0.0 50.0)))
  ;[1 0.03125 0.03125] Event fall
  (bind (_outhits _returnvalue_2) (`KismetSystemLibrary.SphereTraceMultiForObjects` :`Start` _returnvalue :`End` _returnvalue :`Radius` 20.0 :`ObjectTypes` (`|MakeArray` "ObjectTypeQuery2" :!type "EObjectTypeQuery Enum") :`DrawDebugType` "Persistent"))
  (if _returnvalue_2
    (for _array_element _outhits
      (message `/Game/Utility/Interfaces/BPI_EPS.Fall` (`.HitActor` (`GameplayStatics.BreakHitResult` _array_element)) false)))
  (if (not IsBeingPickedup)
    (`PrimitiveComponent.SetSimulatePhysics` (`self.StaticMesh`) true)
    (bind _returnvalue_3 (`KismetSystemLibrary.K2_SetTimer` null "ResetSimulate" 0.1 true))
    (set `self.SimulationTimer` _returnvalue_3)))

(event `Hit Something`
  ;[0 0.2912 1] Hit Event
  (`self.HideActor`)
  (set `self.IsBeingThrown` false))

(fn `DurabilityCalc`
  (returns (`IsBroken?` :type Boolean))
  (bind _output_get (set `self.CurDurability` (`KismetMathLibrary.Clamp` (- (`self.CurDurability`) 1) 0 (`self.MaxDurability`))))
  (`KismetSystemLibrary.PrintString` (`KismetStringLibrary.Conv_IntToString` _output_get))
  (return (== _output_get 0)))

(fn `EvaluateObjectsBelow`
  (params (ActorToIgnore :type "Actor Object Reference"))
  (bind (_returnvalue_x _returnvalue_y _returnvalue_z) (`KismetMathLibrary.BreakVector` (`self.K2_GetActorLocation`)))
  (bind _returnvalue (`KismetMathLibrary.MakeVector` _returnvalue_x _returnvalue_y (+ _returnvalue_z 50.0)))
  (bind _outhit (`KismetSystemLibrary.SphereTraceSingleForObjects` :`Start` _returnvalue :`End` _returnvalue :`Radius` 40.0 :`ObjectTypes` (`|MakeArray` "ObjectTypeQuery1" :!type "EObjectTypeQuery Enum") :`DrawDebugType` "Persistent"))
  (if (`GameplayStatics.BreakHitResult` _outhit)
    _))

(fn `IsPlayerLookingAtMe`
  (returns (InverseDotProduct :type "Float (double-precision)"))
  (bind _playerchar (`self.PlayerChar`)
    (:`then`
      (bind _camera (`/Game/Characters/BP_PlayerChar.Camera` _playerchar))
      (return (* (`KismetMathLibrary.Dot_VectorVector` (`KismetMathLibrary.GetForwardVector` (`KismetMathLibrary.FindLookAtRotation` (`self.K2_GetActorLocation`) (`SceneComponent.K2_GetComponentLocation` _camera))) (`SceneComponent.GetForwardVector` _camera)) -1.0)))
    (:`else`)))

(fn `Renable/DisableCollision`
  (params (`Enable?` :type Boolean))
  ;[1 1 1] Enable/Disable collision of static mesh and box collision
  (if `Enable?`
    (`PrimitiveComponent.SetCollisionEnabled` (`self.StaticMesh`) "QueryAndPhysics")
    (`PrimitiveComponent.SetCollisionEnabled` (`self.Box`) "QueryAndPhysics")
    (set `self.IsBeingHeld` false)
    (else
      (`PrimitiveComponent.SetCollisionEnabled` (`self.StaticMesh`) "NoCollision")
      (`PrimitiveComponent.SetCollisionEnabled` (`self.Box`) "NoCollision")
      (set `self.IsBeingHeld` true)))
  (return))

(fn `UserConstructionScript`
  (switch `/Game/Utility/Enums/E_LevelObjects` (`self.MeshEnum`)
    (:`NewEnumerator0`
      ;[1 1 1] Set the static mesh and where the highlight material should be placed
      (`StaticMeshComponent.SetStaticMesh` (`self.StaticMesh`) "/Game/Meshes/Crates_Barrels/SM_WoodenBox.SM_WoodenBox")
      (set `self.RegularMaterial` "/Game/Art/Materials/MI_WoodCrateLight.MI_WoodCrateLight")
      (set `self.HighlightMaterialIndex` 12)
      ;;[1 1 1] SFX and VFX setup
      (set `self.ImpactSound` "/Game/SFX/Mechanics/Throw_Hit_Drop/SC_BarrelHit.SC_BarrelHit")
      (set `self.DestructionVFX` "/Game/Art/VFX/VFX_BarrelBreak.VFX_BarrelBreak"))
    (:`NewEnumerator1`
      (`StaticMeshComponent.SetStaticMesh` (`self.StaticMesh`) "/Game/Meshes/Crates_Barrels/SM_Barrel.SM_Barrel")
      (set `self.RegularMaterial` "/Game/Art/Materials/MI_WoodBarrelLight.MI_WoodBarrelLight")
      (set `self.HighlightMaterialIndex` 5)
      (set `self.ImpactSound` "/Game/SFX/Mechanics/Throw_Hit_Drop/SC_BarrelHit.SC_BarrelHit")
      (set `self.DestructionVFX` "/Game/Art/VFX/VFX_BarrelBreak.VFX_BarrelBreak"))
    (:`NewEnumerator2`
      (`StaticMeshComponent.SetStaticMesh` (`self.StaticMesh`) "/Game/Meshes/SM_Egg.SM_Egg")
      (set `self.RegularMaterial` "/Game/Art/Materials/M_White.M_White")
      (set `self.HighlightMaterialIndex` 0)
      (set `self.ImpactSound` "/Game/SFX/Mechanics/Throw_Hit_Drop/SC_EggHit.SC_EggHit")
      (set `self.DestructionVFX` "/Game/Art/VFX/VFX_Confetti.VFX_Confetti"))
    (:`NewEnumerator3`
      (`StaticMeshComponent.SetStaticMesh` (`self.StaticMesh`) "/Game/Meshes/Construction/SM_Plank.SM_Plank")
      (set `self.RegularMaterial` "/Game/Art/Materials/M_WheatBrown.M_WheatBrown")
      (set `self.HighlightMaterialIndex` 0))
    (:`NewEnumerator4`
      (`StaticMeshComponent.SetStaticMesh` (`self.StaticMesh`) "/Game/Meshes/Crates_Barrels/SM_Barrel.SM_Barrel")
      (set `self.RegularMaterial` "/Game/Art/Materials/M_Green.M_Green")
      (set `self.HighlightMaterialIndex` 5)
      (set `self.ImpactSound` "/Game/SFX/ChickenSounds/preacher13__bwack_shortened.preacher13__bwack_shortened")
      (set `self.DestructionVFX` "/Game/Art/VFX/VFX_BarrelBreak.VFX_BarrelBreak"))
    (:`NewEnumerator5`
      (`StaticMeshComponent.SetStaticMesh` (`self.StaticMesh`) "/Game/Meshes/Chests/SM_Chest.SM_Chest")
      (set `self.RegularMaterial` "/Game/Art/Materials/M_DarkBrown_Wood.M_DarkBrown_Wood")
      (set `self.HighlightMaterialIndex` 4)
      (set `self.ImpactSound` "/Game/SFX/Collectibles/Bag_of_Coin_Sound_Effect_001.Bag_of_Coin_Sound_Effect_001")
      (set `self.DestructionVFX` "/Game/Art/VFX/VFX_BarrelBreak.VFX_BarrelBreak"))
    (:`NewEnumerator6`
      (`StaticMeshComponent.SetStaticMesh` (`self.StaticMesh`) "/Game/Meshes/SM_WaterBucket.SM_WaterBucket")
      (set `self.RegularMaterial` "/Game/Art/Materials/M_DarkBrown_Wood.M_DarkBrown_Wood")
      (set `self.HighlightMaterialIndex` 1))))