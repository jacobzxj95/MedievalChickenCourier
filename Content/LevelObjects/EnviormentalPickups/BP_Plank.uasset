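; BP_Plank is a plank level object, filed under environmental pickups, that turns a BP_MudPuddle's hidden cube solid on contact.
; When its static mesh hits a puddle, it disables the puddle's box collision and reveals the cube with query and physics collision.
; The plank then destroys itself after a brief delay, apparently leaving the cube as its placed stand-in.
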(event `self.ReceiveBeginPlay`
  (`parent.ReceiveBeginPlay`))

(event `self.ReceiveActorBeginOverlap`
  (params (OtherActor :type "Actor Object Reference")))

(event `self.ReceiveTick`
  (params (DeltaSeconds :type "Float (single-precision)")))

(event `self.StaticMesh.OnComponentHit`
  (params (HitComponent :type "PrimitiveComponent Object Reference") (OtherActor :type "Actor Object Reference") (OtherComp :type "PrimitiveComponent Object Reference") (NormalImpulse :type "Vector Structure") (Hit :type "HitResult Structure (by ref)"))
  (bind _asbp_mud_puddle (cast `/Game/LevelObjects/LevelMechanics/BP_MudPuddle` OtherActor))
  (`PrimitiveComponent.SetCollisionEnabled` (`/Game/LevelObjects/LevelMechanics/BP_MudPuddle.Box` _asbp_mud_puddle) "NoCollision")
  (bind _cube (`/Game/LevelObjects/LevelMechanics/BP_MudPuddle.Cube` _asbp_mud_puddle))
  (`SceneComponent.SetHiddenInGame` _cube false false)
  (`PrimitiveComponent.SetCollisionEnabled` _cube "QueryAndPhysics")
  (`KismetSystemLibrary.Delay` 0.1)
  (`self.K2_DestroyActor`))

(fn `UserConstructionScript`
  (`parent.UserConstructionScript`))