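; BP_WaterBucket is an environmental pickup that activates magic sand on a BP_Quicksand actor it hits.
; When its static mesh hits quicksand, it sets MagicSandUsed, enables query-only collision on the quicksand's overlap volume and reveals that actor's activation VFX.
; The bucket then appears used up, with its mesh hidden and box collision disabled, though the actor is not destroyed.
; A branch that would show the quicksand's widget is left unconnected.
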(event `self.StaticMesh.OnComponentHit`
  (params (HitComponent :type "PrimitiveComponent Object Reference") (OtherActor :type "Actor Object Reference") (OtherComp :type "PrimitiveComponent Object Reference") (NormalImpulse :type "Vector Structure") (Hit :type "HitResult Structure (by ref)"))
  (bind _asbp_quicksand (cast `/Game/LevelObjects/LevelMechanics/BP_Quicksand` OtherActor))
  (set `self.magicSandUsed?` true)
  (`PrimitiveComponent.SetCollisionEnabled` (`/Game/LevelObjects/LevelMechanics/BP_Quicksand.OverlapVolume` _asbp_quicksand) "QueryOnly")
  (`SceneComponent.SetHiddenInGame` (`self.StaticMesh`) true false)
  (`PrimitiveComponent.SetCollisionEnabled` (`self.Box`) "NoCollision")
  (`SceneComponent.SetHiddenInGame` (`/Game/LevelObjects/LevelMechanics/BP_Quicksand.VFX_MagicSandActivation` _asbp_quicksand) false false))

(fn `UserConstructionScript`
  (`parent.UserConstructionScript`))