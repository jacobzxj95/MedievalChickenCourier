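; BP_Egg is an environmental pickup egg that inherits drop and pickup behavior from its parent, passing chicken flags as false on pickup.
; On BeginPlay a looping timer checks its distance to the player and destroys the egg once it is far enough away.
; When it hits something, it plays an egg-hit sound at its location.
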(event `/Game/Utility/Interfaces/BPI_EPS.ItemDropped`
  (params (DropLocation :type "Vector Structure"))
  (`parent.ItemDropped` DropLocation))

(event `/Game/Utility/Interfaces/BPI_EPS.ItemPickedUp`
  (params (CurrentChicken :type "Actor Object Reference") (`CapturingChicken?` :type Boolean) (`HasChicken?` :type Boolean))
  (`parent.ItemPickedUp` null false false))

(event `self.ReceiveBeginPlay`
  (`KismetSystemLibrary.K2_SetTimerDelegate` (delegate `Destroy egg relative to player distance`) 2.0 true))

(event `Destroy egg relative to player distance`
  (if (>= (`self.GetDistanceTo` (`GameplayStatics.GetPlayerCharacter` 0)) 1000.0)
    (`self.K2_DestroyActor`)))

(event `self.Hit Something`
  (`GameplayStatics.PlaySoundAtLocation` "/Game/SFX/Mechanics/Throw_Hit_Drop/SC_EggHit.SC_EggHit" (`self.K2_GetActorLocation`) (struct) 1.0 1.0 0.0 null null null null))

(fn `UserConstructionScript`
  (`parent.UserConstructionScript`))