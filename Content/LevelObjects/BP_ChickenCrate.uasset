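; Carriable, throwable crate that holds up to two captured chickens.
; Capturing sends the chicken to a storage actor, shows a stand-in mesh and copies its tags and quest IDs onto the crate for waypoints.
; Tick uses overlap and a camera dot product to highlight the crate and start polling R to release chickens.
; Thrown hits on non-soft surfaces reduce durability; breaking drops the chickens and returns their quest IDs.
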(event `PlayHeldChickenSounds`
  (bind _returnvalue (`self.K2_GetActorLocation`))
  (bind _returnvalue_2 (`KismetMathLibrary.RandomFloatInRange` 5.0 20.0))
  ;[0.05966 0.3229 0.2777] BEGIN PLAY: Gather references and set inital variables
  (if (`self.HasChicken?`) :!label _label
    ;[1 0.9988 0.7106] Play Chicken Sounds on occasion
    (if (`self.Held?`)
      (`GameplayStatics.PlaySoundAtLocation` "/Game/SFX/ChickenSounds/SC_ChickenCluck.SC_ChickenCluck" _returnvalue (struct) 1.0 1.0 0.0 null null null null)
      (`KismetSystemLibrary.Delay` _returnvalue_2)
      (`self.PlayHeldChickenSounds`)
      (else
        (`GameplayStatics.PlaySoundAtLocation` "/Game/SFX/ChickenSounds/SC_RandomChickenSounds.SC_RandomChickenSounds" _returnvalue (struct) 1.0 1.0 0.0 null null null null)
        (`KismetSystemLibrary.Delay` _returnvalue_2)
        (`self.PlayRandomChickenSounds`)))))

(event `self.ReceiveBeginPlay`
  ;[0.05966 0.3229 0.2777] BEGIN PLAY: Gather references and set inital variables
  (`|ExecutionSequence`
    (:`then_0`
      (bind _returnvalue (`GameplayStatics.GetActorOfClass` "/Game/LevelObjects/BP_ActorStorageLocation.BP_ActorStorageLocation_C"))
      (set `self.StorageActor_Ref` _returnvalue)
      (bind _outactors (`GameplayStatics.GetAllActorsOfClass` "/Game/AI/AICharacters/BP_AI_Chicken.BP_AI_Chicken_C"))
      (set `self.ChickenPool` _outactors)
      (set `self.DefaultScale` (`self.GetActorScale3D`))
      (bind _asgm_mvp (cast `/Game/Maps/GameModes/GM_MVP` (`GameplayStatics.GetGameMode`))
        (:`then`
          (set `self.As GM MVP` _asgm_mvp)
          (goto _label))
        (:`CastFailed`
          (goto _label))))
    (:`then_1`
      (set `self.CurrentDurabilityLvl` (`self.MaxDurabilityLvl`))
      (`KismetSystemLibrary.Delay` 2.0)
      (bind _playercharacterref (message `/Game/Utility/Interfaces/BPI_UI.Pass Out Playercharacter ref` (`GameplayStatics.GetGameMode`)))
      (bind _output_get (set `self.PlayerChar` _playercharacterref))
      (add `/Game/Components/ActorComponents/AC_Questlog.Quest Started` (`/Game/Characters/BP_PlayerChar.AC_QuestTurnIn` _output_get) (delegate `QuestInitiated`))
      ;[0 0.05955 1] Check to see if the crate is burried
      (`KismetSystemLibrary.K2_SetTimerDelegate` (delegate `CheckForBurriedCrate`) 7.0 true)
      ;[0.375 0 0.2858] Check Crate durability level
      (`KismetSystemLibrary.K2_SetTimerDelegate` (delegate `CheckCrateDurability`) 0.1 true)
      ;[1 0.7318 0] Check if the crate has a chicken
      (bind _returnvalue_2 (`KismetSystemLibrary.K2_SetTimerDelegate` (delegate `CheckForChicken`) 0.1 true))
      (set `self.ChickenIcon_TagTimerHandle` _returnvalue_2))
    (:`then_2`
      (set `self.CratedChickens` (`|MakeArray` (`self.Slot1`) (`self.Slot2`) :!type "Actor Object Reference")))))

(event `PlayRandomChickenSounds`
  ;[0.05966 0.3229 0.2777] BEGIN PLAY: Gather references and set inital variables
  (goto _label))

(event `QuestInitiated`
  (params (ActiveQuest :type "/Game/RodgerL/BP_QuestManager Object Reference"))
  ;[0.05966 0.3229 0.2777] BEGIN PLAY: Gather references and set inital variables
  (set `self.QuestStarted?` true))

(event `CheckForBurriedCrate`
  (bind _snowparticle (`self.SnowParticle`))
  ;[0 0.05955 1] Check to see if the crate is burried
  (for _array_element (`self.GetOverlappingActors` "/Game/LevelObjects/LevelMechanics/BP_SoftSurface.BP_SoftSurface_C")
    (`SceneComponent.K2_SetWorldRotation` _snowparticle (`KismetMathLibrary.MakeRotFromZ` (`self.GetActorUpVector` _array_element)) false false)
    (`ActorComponent.Activate` _snowparticle false))
  (`KismetSystemLibrary.Delay` 10.0)
  (`ActorComponent.Deactivate` _snowparticle))

(event `CheckCrateDurability`
  ;[0.375 0 0.2858] Check Crate durability level
  (if (>= (`self.CurrentDurabilityLvl`) (`self.MinDurabilityLvl`))
    (set `self.CrateDurabilityGood?` true)
    (else
      (set `self.CrateDurabilityGood?` false))))

(event `CheckForChicken`
  (bind _tags (`self.Tags`))
  ;[1 0.7318 0] Check if the crate has a chicken
  (if (and (`self.HasChicken?`) (`self.CrateDurabilityGood?`))
    (`|ExecutionSequence`
      (:`then_0`
        (`/Engine/EditorBlueprintResources/StandardMacros.DoOnce` false :!label _label_2
          (:`Completed`
            (bind _playerchar (`self.PlayerChar`)
              (:`then`
                (message `/Game/Utility/Interfaces/BPI_EPS.ItemPickedUp` _playerchar null false true)
                (`KismetArrayLibrary.Array_Add` (`self.Tags`) (`self.HasChickenTag`)))
              (:`else`)))))
      (:`then_1`
        (goto _label_3 :!via `Reset`)))
    (else
      (`|ExecutionSequence`
        (:`then_0`
          (goto _label_2 :!via `Reset`))
        (:`then_1`
          (`/Engine/EditorBlueprintResources/StandardMacros.DoOnce` false :!label _label_3
            (:`Completed`
              (bind _playerchar_2 (`self.PlayerChar`)
                (:`then`
                  (message `/Game/Utility/Interfaces/BPI_EPS.ItemPickedUp` _playerchar_2 null false false)
                  (for _array_element _tags
                    (if (== _array_element (`self.HasChickenTag`))
                      (`KismetArrayLibrary.Array_RemoveItem` _tags _array_element)
                      (break))))
                (:`else`)))))))))

(event `self.ReceiveTick`
  (params (DeltaSeconds :type "Float (single-precision)"))
  (bind _sm_crate (`self.SM_Crate`))
  (bind _etointeract (`/Game/UI/W_HUD.EtoInteract` (`/Game/Maps/GameModes/GM_MVP.PlayerHUD` (`self.As GM MVP`))))
  ;[1 0.07331 0] EVENT TICK: Display interact info if the player is in range and looking at the object
  (bind _dotproductinverse (`self.IsPlayerLookingHere`))
  (if (and (`self.InRange?`) (> _dotproductinverse 0.7))
    (`Widget.SetVisibility` _etointeract "Visible")
    (`PrimitiveComponent.CreateDynamicMaterialInstance` _sm_crate 0 "/Game/Art/Materials/M_HighlightColor.M_HighlightColor" "None")
    (`/Engine/EditorBlueprintResources/StandardMacros.DoOnce` false :!label _label_4
      (:`Completed`
        (bind _returnvalue (`KismetSystemLibrary.K2_SetTimer` null "CheckForChickenRelease" 0.1 true))
        (set `self.CheckForChickenReleaseHandle` _returnvalue)))
    (else
      (`Widget.SetVisibility` _etointeract "Hidden")
      (`PrimitiveComponent.CreateDynamicMaterialInstance` _sm_crate 0 "/Game/Art/Materials/M_DarkBrown_Wood.M_DarkBrown_Wood" "None")
      (`KismetSystemLibrary.K2_ClearAndInvalidateTimerHandle` (`self.CheckForChickenReleaseHandle`))
      (goto _label_4 :!via `Reset`))))

(event `/Game/Utility/Interfaces/BPI_Quest.TurnOnWaypoints`
  (params (ObjectiveID :type String) (`On/Off` :type Boolean))
  ;[1 1 1] Turn on and off Waypoints when Quest starts
  (`/Game/Components/ActorComponents/AC_Questitem.Check To Turn On Waypoints` (`self.AC_Questitem`) (`self.Widget`) `On/Off` ObjectiveID))

(event `/Game/Utility/Interfaces/BPI_EPS.ItemPickedUp`
  (params (CurrentChicken :type "Actor Object Reference") (`CapturingChicken?` :type Boolean) (`HasChicken?` :type Boolean))
  (bind _output (`|GetArrayItem` (`self.CratedChickens`) (`self.CurrentIndex`)))
  ;[1 0 0.8949] Item Picked Up
  (set `self.Current Chicken` CurrentChicken)
  (if (not `CapturingChicken?`)
    (set `self.Held?` true)
    (`self.HandleCollision` false)
    (`Widget.SetVisibility` (`/Game/UI/W_HUD.EtoInteract` (`/Game/Maps/GameModes/GM_MVP.PlayerHUD` (`self.As GM MVP`))) "Hidden")
    (else
      (if (== (`GameplayStatics.GetObjectClass` (`/Game/Characters/BP_ActiveChar.Current Item` (`self.PlayerChar`))) "BP_ChickenCrate_C")
        (`self.HandleCollision` true)
        (else
          (set `self.HoldingChicken?` true)))
      (`|ExecutionSequence`
        (:`then_0`
          (for _array_element (`self.ChickenPool`) :!label _label_5
            (bind _current_chicken (`self.Current Chicken`)
              (:`then`
                (if (== _current_chicken _array_element)
                  (if (== (`self.Slot1`) null)
                    (set `self.CurrentIndex` 0)
                    (bind _output_get (set `self.Slot1` _array_element))
                    (`KismetArrayLibrary.Array_Set` (`self.CratedChickens`) 0 _output_get)
                    (set `self.HasChicken?` true)
                    (`SceneComponent.SetHiddenInGame` (`self.ChickenMesh1`) false false)
                    (bind _storageactor_ref (`self.StorageActor_Ref` :!label _label_6)
                      (:`then`
                        (message `/Game/Utility/Interfaces/BPI_StoreActor.StorageLocation` _storageactor_ref _array_element))
                      (:`else`))
                    (elif (== (`self.Slot2`) null)
                      (set `self.CurrentIndex` 1)
                      (bind _output_get_2 (set `self.Slot2` _array_element))
                      (`KismetArrayLibrary.Array_Set` (`self.CratedChickens`) 1 _output_get_2)
                      (set `self.CrateFull` true)
                      (`SceneComponent.SetHiddenInGame` (`self.ChickenMesh2`) false false)
                      (goto _label_6)
                      (else
                        (set `self.CrateFull` true))))
                  (`self.BreakChickenCheckLoop`)
                  (`GameplayStatics.PlaySoundAtLocation` "/Game/SFX/Mechanics/Throw_Hit_Drop/SC_PlaceDownObject.SC_PlaceDownObject" (`self.K2_GetActorLocation`) (struct) 1.0 1.0 0.0 null null null null)))
              (:`else`
                (`KismetSystemLibrary.PrintString` "CHICKEN CRATE: CURRENT CHICKEN INVALID" true true (struct :`R` 1.0 :`B` 0.059606 :`A` 1.0) 4.0))))
          (if (and (`self.Held?`) (not (`self.HoldingChicken?`)))
            (`self.HandleCollision` false)))
        (:`then_1`
          (if (`KismetSystemLibrary.IsValid` _output)
            (for _array_element_2 (`Actor.Tags` _output)
              (`KismetArrayLibrary.Array_AddUnique` (`self.Tags`) _array_element_2))
            (`SceneComponent.SetHiddenInGame` (`self.Widget`) false false)
            (`/Game/Components/ActorComponents/AC_Questitem.Send ID` (`self.AC_Questitem`) 1)
            (bind _slot1 (`self.Slot1`)
              (:`then`
                (for _array_element_3 (`/Game/Components/ActorComponents/AC_Questitem.ActorQuestIDS` (`/Game/AI/AICharacters/BP_AI_Chicken.AC_Questitem` _slot1))
                  (`KismetArrayLibrary.Array_AddUnique` (`/Game/Components/ActorComponents/AC_Questitem.ActorQuestIDS` (`self.AC_Questitem`)) _array_element_3)))
              (:`else`
                _))
            (`KismetArrayLibrary.Array_Clear` (`/Game/Components/ActorComponents/AC_Questitem.ActorQuestIDS` (`/Game/AI/AICharacters/BP_AI_Chicken.AC_Questitem` (`self.Slot1`))))))))))

(event `BreakChickenCheckLoop`
  ;[1 0 0.8949] Item Picked Up
  (goto _label_5 :!via `Break`))

(event `/Game/Utility/Interfaces/BPI_EPS.ItemDropped`
  (params (DropLocation :type "Vector Structure"))
  (bind _ac_questitem (`self.AC_Questitem`))
  ;[0.04688 0 0.03545] Item Dropped
  (`self.K2_SetActorTransform` (`KismetMathLibrary.MakeTransform` DropLocation (`self.K2_GetActorRotation` (`GameplayStatics.GetPlayerPawn` 0))))
  (`GameplayStatics.PlaySoundAtLocation` "/Game/SFX/Mechanics/Throw_Hit_Drop/SC_ChickenCrateDrop.SC_ChickenCrateDrop" DropLocation (struct) 1.0 1.0 0.0 null null null null)
  (`KismetSystemLibrary.Delay` 0.2)
  (`self.HandleCollision` true)
  (set `self.Held?` false)
  (if (`/Game/Components/ActorComponents/AC_Questitem.IsQuestEnabled` _ac_questitem)
    (`/Game/Components/ActorComponents/AC_Questitem.On Off Waypoint` _ac_questitem (`self.Widget`) true)
    (else
      (`KismetSystemLibrary.PrintString` "dropped-quest not enabled??"))))

(event `/Game/Utility/Interfaces/BPI_EPS.ItemThrown`
  (params (ThrowingForce :type "Float (double-precision)") (ThrowingDirection :type "Vector Structure") (StartingTransform :type "Transform Structure") (`CatapultLaunched?` :type Boolean) (StunDuration :type "Float (double-precision)"))
  (bind _sm_crate (`self.SM_Crate`))
  (bind _ac_questitem (`self.AC_Questitem`))
  ;[0.2932 0 1] Item Thrown
  (set `self.IsBeingThrown?` true)
  (`self.HandleCollision` true)
  (`PrimitiveComponent.SetSimulatePhysics` _sm_crate true)
  (`PrimitiveComponent.AddImpulse` _sm_crate (* ThrowingForce ThrowingDirection) "None" true)
  (`self.K2_SetActorLocation` (.location StartingTransform))
  (`self.SetActorScale3D` (`self.DefaultScale`))
  (set `self.Held?` false)
  (if (`/Game/Components/ActorComponents/AC_Questitem.IsQuestEnabled` _ac_questitem)
    (`/Game/Components/ActorComponents/AC_Questitem.On Off Waypoint` _ac_questitem (`self.Widget`) true)))

(event `self.OverlapVolume.OnComponentBeginOverlap`
  (params (OverlappedComponent :type "PrimitiveComponent Object Reference") (OtherActor :type "Actor Object Reference") (OtherComp :type "PrimitiveComponent Object Reference") (OtherBodyIndex :type Integer) (bFromSweep :type Boolean) (SweepResult :type "HitResult Structure (by ref)"))
  ;[0.9525 1 0] Player Overlap (In Range) and Soft Surface Check
  (if (== OtherActor (`GameplayStatics.GetPlayerPawn` 0))
    (if (not (and (`/Game/Components/ActorComponents/AC_Questitem.NeededForQuest?` (`self.AC_Questitem`)) (not (`self.QuestStarted?`))))
      (set `self.InRange?` true)
      (else
        (if (`self.ActorHasTag` OtherActor "Soft") :!label _label_7
          (set `self.PrepSoftImpact?` true)
          (else
            (set `self.PrepSoftImpact?` false)))))
    (else
      (goto _label_7))))

(event `CheckForChickenRelease`
  ;[0.1158 0.1046 1] Pull Chicken From Crate
  (if (`PlayerController.WasInputKeyJustPressed` (`GameplayStatics.GetPlayerController` 0) "R")
    (`KismetSystemLibrary.K2_ClearAndInvalidateTimerHandle` (`self.CheckForChickenReleaseHandle`))
    (bind _dotproductinverse (`self.IsPlayerLookingHere`))
    (if (and (`self.InRange?`) (> _dotproductinverse 0.7) (not (`/Game/Characters/BP_ActiveChar.Is Holding?` (`self.PlayerChar`))))
      (if (`self.CrateFull`)
        (`/Game/Characters/BP_PlayerChar.Pickup (NonInput)` (`self.PlayerChar`) (`self.Slot2`))
        (set `self.CrateFull` false)
        (`SceneComponent.SetHiddenInGame` (`self.ChickenMesh2`) true false)
        (set `self.Slot2` null)
        (`/Game/Components/ActorComponents/AC_Questitem.Send ID` (`self.AC_Questitem`) 1)
        (elif (`self.HasChicken?`)
          (`/Game/Characters/BP_PlayerChar.Pickup (NonInput)` (`self.PlayerChar`) (`self.Slot1`))
          (set `self.HasChicken?` false)
          (`SceneComponent.SetHiddenInGame` (`self.ChickenMesh1`) true false)
          (for _array_element (`/Game/Components/ActorComponents/AC_Questitem.ActorQuestIDS` (`self.AC_Questitem`))
            (bind _cratedchickenref (`self.CheckCratedChickensAgainstPool`)
              (:`LoopOutput`
                (bind _ac_questitem (`/Game/AI/AICharacters/BP_AI_Chicken.AC_Questitem` _cratedchickenref))
                (`KismetArrayLibrary.Array_AddUnique` (`/Game/Components/ActorComponents/AC_Questitem.ActorQuestIDS` _ac_questitem) _array_element)
                ;[1 1 1] Turns on chickens' icons
                (message `/Game/Utility/Interfaces/BPI_Quest.TurnOnWaypoints` (`self.Slot1`) _array_element true)
                (message `/Game/Utility/Interfaces/BPI_Quest.TurnOnWaypoints` (`self.Slot2`) _array_element true))))
          (set `self.QuestItem?` false)
          (`/Game/Components/ActorComponents/AC_Questitem.Send ID` _ac_questitem 1)
          (`KismetArrayLibrary.Array_Clear` (`/Game/Components/ActorComponents/AC_Questitem.ActorQuestIDS` (`self.AC_Questitem`)))
          (set `self.Slot1` null)
          (`SceneComponent.SetHiddenInGame` (`self.Widget`) true false)
          (`/Game/Components/ActorComponents/AC_Questitem.Send ID` (`self.AC_Questitem`) 1))))))

(event `self.OverlapVolume.OnComponentEndOverlap`
  (params (OverlappedComponent :type "PrimitiveComponent Object Reference") (OtherActor :type "Actor Object Reference") (OtherComp :type "PrimitiveComponent Object Reference") (OtherBodyIndex :type Integer))
  ;[0.9525 1 0] Player Overlap (In Range) and Soft Surface Check
  (if (== (`GameplayStatics.GetPlayerPawn` 0) OtherActor)
    (set `self.InRange?` false)
    (`KismetSystemLibrary.K2_ClearAndInvalidateTimerHandle` (`self.CheckForChickenReleaseHandle`))
    (else
      (set `self.PrepSoftImpact?` false))))

(event `AllowImpactSoundAgain`
  ;[0.4137 0.09 0.5417] Crate Impact after being thrown
  (`/Engine/EditorBlueprintResources/StandardMacros.DoOnce` false :!label _label_8
    (:`Completed`
      (`GameplayStatics.PlaySoundAtLocation` "/Game/SFX/Mechanics/Throw_Hit_Drop/SC_ThrownCrateImpact.SC_ThrownCrateImpact" (`.Location` (`GameplayStatics.BreakHitResult` (stale `self.SM_Crate.OnComponentHit` Hit))) (struct) 1.0 1.0 0.1 null null null null)
      (set `self.ImpactSoundOverlap?` true)
      (if (`self.JustThrown?`)
        (`KismetSystemLibrary.RetriggerableDelay` 0.2)
        (set `self.ImpactSoundOverlap?` false)
        (else
          (`KismetSystemLibrary.Delay` 0.5)))
      (`self.AllowImpactSoundAgain`))))

(event `self.SM_Crate.OnComponentHit`
  (params (HitComponent :type "PrimitiveComponent Object Reference") (OtherActor :type "Actor Object Reference") (OtherComp :type "PrimitiveComponent Object Reference") (NormalImpulse :type "Vector Structure") (Hit :type "HitResult Structure (by ref)"))
  (bind _returnvalue (`self.K2_GetActorLocation`))
  (bind _woodsplinters (`self.WoodSplinters`))
  (bind _slot1 (`self.Slot1`))
  (bind _slot2 (`self.Slot2`))
  (bind _ac_questitem (`self.AC_Questitem`))
  ;[0.4137 0.09 0.5417] Crate Impact after being thrown
  (set `ProjectileMovementComponent.bSimulationEnabled` false (`self.ProjectileMovement`))
  (`|ExecutionSequence`
    (:`then_0`
      (if (and (`self.JustThrown?`) (not (`self.PrepSoftImpact?`)) (not (`self.ImpactSoundOverlap?`)))
        (goto _label_8)))
    (:`then_1`
      (if (and (!= OtherActor (`GameplayStatics.GetPlayerPawn` 0)) (`self.IsBeingThrown?`))
        (`/Engine/EditorBlueprintResources/StandardMacros.DoOnce` false :!label _label_9
          (:`Completed`
            (message `/Game/Utility/Interfaces/BPI_Hit.HitByProjectile` OtherActor 0.0)
            (set `self.IsBeingThrown?` false)
            (set `self.ImpactLocation` (`.Location` (`GameplayStatics.BreakHitResult` Hit)))
            (if (`self.PrepSoftImpact?`)
              (`self.ResetHitByProjectile`)
              (else
                (`self.CrateDurability`
                  (:`CrateBroken`
                    (`|ExecutionSequence`
                      (:`then_0`
                        (for (_array_element _array_index) (`/Game/Components/ActorComponents/AC_Questitem.ActorQuestIDS` _ac_questitem)
                          (`KismetArrayLibrary.Array_AddUnique` (`/Game/Components/ActorComponents/AC_Questitem.ActorQuestIDS` (`/Game/AI/AICharacters/BP_AI_Chicken.AC_Questitem` (`self.Slot1`))) _array_element)
                          (`KismetArrayLibrary.Array_AddUnique` (`/Game/Components/ActorComponents/AC_Questitem.ActorQuestIDS` (`/Game/AI/AICharacters/BP_AI_Chicken.AC_Questitem` (`self.Slot2`))) _array_element)
                          (`/Game/Components/ActorComponents/AC_Questitem.Send ID` _ac_questitem _array_index))
                        (`KismetArrayLibrary.Array_Clear` (`/Game/Components/ActorComponents/AC_Questitem.ActorQuestIDS` (`self.AC_Questitem`)))
                        (if (and (`self.QuestStarted?`) (`self.QuestItem?`))
                          (message `/Game/Utility/Interfaces/BPI_Quest.TurnOnWaypoints` _slot1 _array_element true)
                          (message `/Game/Utility/Interfaces/BPI_Quest.TurnOnWaypoints` _slot2 _array_element true)
                          (else
                            (message `/Game/Utility/Interfaces/BPI_Quest.TurnOnWaypoints` _slot1 _array_element false)
                            (message `/Game/Utility/Interfaces/BPI_Quest.TurnOnWaypoints` _slot2 _array_element false))))
                      (:`then_1`
                        (if (`self.CrateFull`)
                          (message `/Game/Utility/Interfaces/BPI_EPS.ItemDropped` (`self.Slot2`) (+ _returnvalue (0.0 5.0 0.0)))
                          (message `/Game/Utility/Interfaces/BPI_EPS.ItemDropped` (`self.Slot1`) _returnvalue :!label _label_10)
                          (elif (`self.HasChicken?`)
                            (goto _label_10)
                            (else
                              _)))
                        ;;[0.3592 0 1] Breaking functionality
                        (`GameplayStatics.PlaySoundAtLocation` "/Game/SFX/Mechanics/Throw_Hit_Drop/SC_ChickenCrateBreak.SC_ChickenCrateBreak" (`self.ImpactLocation`) (struct) 1.0 1.0 0.0 null null null null)
                        (`ActorComponent.Activate` _woodsplinters true)
                        (`SceneComponent.SetHiddenInGame` (`self.SM_Crate`) true false)
                        (`SceneComponent.SetHiddenInGame` (`self.ChickenMesh2`) true false)
                        (`SceneComponent.SetHiddenInGame` (`self.ChickenMesh1`) true false)
                        (`self.HandleCollision` false)
                        (`KismetSystemLibrary.Delay` 0.5)
                        (`SceneComponent.SetHiddenInGame` (`self.SM_Crate`) true true)
                        (`ActorComponent.Deactivate` _woodsplinters)
                        (`self.ResetHitByProjectile` :!label _label_11)
                        (set `self.PrepSoftImpact?` false)
                        (set `self.JustThrown?` true)
                        (`KismetSystemLibrary.Delay` 0.3) ; This prevents the additional impact sounds from triggering at the same time as the intial impact sound.
                        (set `self.ImpactSoundOverlap?` false)
                        (`KismetSystemLibrary.Delay` 1.0)
                        (set `self.JustThrown?` false))))
                  (:`CrateDamaged`
                    (`GameplayStatics.PlaySoundAtLocation` "/Game/SFX/Mechanics/Throw_Hit_Drop/SC_ThrownCrateImpact.SC_ThrownCrateImpact" (`self.ImpactLocation`) (struct) 1.0 1.0 0.0 null null null null)
                    (set `self.ImpactSoundOverlap?` true)
                    (goto _label_11)))))))))))

(event `ResetHitByProjectile`
  ;[0.4137 0.09 0.5417] Crate Impact after being thrown
  (goto _label_9 :!via `Reset`))

(fn `HandleCollision`
  (params (`CollisionEnabled?` :type Boolean))
  (bind _sm_crate (`self.SM_Crate`))
  (if `CollisionEnabled?`
    (`PrimitiveComponent.SetCollisionEnabled` _sm_crate "QueryAndPhysics")
    (`PrimitiveComponent.SetCollisionEnabled` (`self.OverlapVolume`) "QueryAndPhysics")
    (else
      (`PrimitiveComponent.SetCollisionEnabled` _sm_crate "NoCollision")
      (`PrimitiveComponent.SetCollisionEnabled` (`self.OverlapVolume`) "NoCollision"))))

(fn `IsPlayerLookingHere`
  (returns (DotProductInverse :type "Float (double-precision)"))
  (bind _playerchar (`self.PlayerChar`)
    (:`then`
      (bind _camera (`/Game/Characters/BP_PlayerChar.Camera` _playerchar))
      (return (* (`KismetMathLibrary.Dot_VectorVector` (`KismetMathLibrary.Normal` (`KismetMathLibrary.GetForwardVector` (`KismetMathLibrary.FindLookAtRotation` (`self.K2_GetActorLocation`) (`SceneComponent.K2_GetComponentLocation` _camera)))) (`KismetMathLibrary.Normal` (`SceneComponent.GetForwardVector` _camera))) -1.0)))
    (:`else`)))

(fn `QuestInteraction`
  (returns (ObjectiveID :type String))
  (return ""))

(fn `UserConstructionScript`
  (bind _chickenmesh1 (`self.ChickenMesh1`))
  (bind _chickenmesh2 (`self.ChickenMesh2`))
  (if (`self.HasChicken?`)
    (`SceneComponent.SetHiddenInGame` _chickenmesh1 false false)
    (if (`self.CrateFull`)
      (`SceneComponent.SetHiddenInGame` _chickenmesh2 false false)
      (else
        (`SceneComponent.SetHiddenInGame` _chickenmesh2 true false)))
    (else
      (`SceneComponent.SetHiddenInGame` _chickenmesh1 true false))))