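; Level drop point that plays a short cutscene of a given Honing Chicken falling into place.
; On BeginPlay it caches a start point above its root and an end point at its own location.
; AnimateHoningChicken disables player input, fades out, switches the view target to itself and fades in while a timeline lerps the chicken down with a spin.
; When the timeline finishes, it restores input and view, then asks the game mode to show a UI message.
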(event `self.ReceiveBeginPlay`
  (bind (_returnvalue_x _returnvalue_y _returnvalue_z) (`KismetMathLibrary.BreakVector` (`SceneComponent.K2_GetComponentLocation` (`self.DefaultSceneRoot`))))
  (set `self.startingLocation` (`KismetMathLibrary.MakeVector` _returnvalue_x _returnvalue_y (+ _returnvalue_z 500.0)))
  (set `self.endingLocation` (`self.K2_GetActorLocation`)))

(event `AnimateHoningChicken`
  (params (GivenChicken :type "Actor Object Reference"))
  (`self.DisableInput` (`GameplayStatics.GetPlayerCharacter` 0) (`GameplayStatics.GetPlayerController` 0))
  (set `self.HoiningChicken` GivenChicken)
  (`PlayerCameraManager.StartCameraFade` :`self` (`GameplayStatics.GetPlayerCameraManager` 0) :`ToAlpha` 1.0 :`Duration` 0.4 :`bShouldFadeAudio` true :`bHoldWhenFinished` true)
  (`KismetSystemLibrary.Delay` 0.6)
  (`PlayerController.SetViewTargetWithBlend` (`GameplayStatics.GetPlayerController` 0) self 0.0 "VTBlend_Linear" 0.0 false)
  (`PlayerCameraManager.StartCameraFade` :`self` (`GameplayStatics.GetPlayerCameraManager` 0) :`FromAlpha` 1.0 :`Duration` 4.0 :`bShouldFadeAudio` true)
  (`KismetSystemLibrary.Delay` 0.6)
  (bind (_direction _newtrack_0) (`Timeline|AnimateChickenFalling` :!via `PlayFromStart`)
    (:`Update`
      (`self.K2_SetActorLocation` (`self.HoiningChicken`) (`KismetMathLibrary.VLerp` (`self.startingLocation`) (`self.endingLocation`) _newtrack_0) false false)
      (`self.K2_SetActorRotation` (`self.HoiningChicken`) (`KismetMathLibrary.RLerp` (struct) (struct :`Pitch` 360.0) _newtrack_0) false))
    (:`Finished`
      (`self.EnableInput` (`GameplayStatics.GetPlayerCharacter` 0) (`GameplayStatics.GetPlayerController` 0))
      (`PlayerController.SetViewTargetWithBlend` (`GameplayStatics.GetPlayerController` 0) (`GameplayStatics.GetPlayerCharacter` 0) 0.0 "VTBlend_Linear" 0.0 false)
      (message `/Game/Utility/Interfaces/BPI_UI.TurnOnUI` (`GameplayStatics.GetGameMode`) "NewEnumerator0"))))

(fn `UserConstructionScript`)