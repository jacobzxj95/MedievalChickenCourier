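; Destructible shutters level object that acts as a quest turn-in target for catapult-launched chickens.
; On overlap, a launched chicken is checked by the ACQuestTurnin component; an accepted one triggers confetti, shows the chicken icon, sets Hit and is destroyed shortly after.
; The component's turn-in finished event hides the waypoint icon and stops further hits.
; TurnonWaypoints toggles that icon when the objective ID matches one of the component's objectives.
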(event `self.ReceiveBeginPlay`
  (add `/Game/Components/ActorComponents/AC_QuestTurnin.TurninFinished` (`self.AC_QuestTurnin`) (delegate `TurnInDone`)))

(event `TurnInDone`
  (`SceneComponent.SetHiddenInGame` (`self.TurnInIcon`) true false)
  (set `self.TurninFinished` true))

(event `self.OverlapVolume.OnComponentBeginOverlap`
  (params (OverlappedComponent :type "PrimitiveComponent Object Reference") (OtherActor :type "Actor Object Reference") (OtherComp :type "PrimitiveComponent Object Reference") (OtherBodyIndex :type Integer) (bFromSweep :type Boolean) (SweepResult :type "HitResult Structure (by ref)"))
  (bind _asbp_ai_chicken (cast `/Game/AI/AICharacters/BP_AI_Chicken` OtherActor))
  (bind _output_get (set `self.As BP AI Chicken` _asbp_ai_chicken))
  (if (and (`/Game/AI/AICharacters/BP_AI_Chicken.Catapult Launched?` _output_get) (not (`self.TurninFinished`)))
    (bind _isquestitem (`/Game/Components/ActorComponents/AC_QuestTurnin.Actor to Check` (`self.AC_QuestTurnin`) OtherActor))
    (if _isquestitem
      (`KismetSystemLibrary.PrintString` "actorID has been sent")
      (`NiagaraFunctionLibrary.SpawnSystemAttached` "/Game/Art/VFX/VFX_Confetti.VFX_Confetti" (`self.OverlapVolume`) "None" (0.0 0.0 0.0) (struct) "KeepRelativeOffset")
      (`SceneComponent.SetVisibility` (`self.ChickenIcon`) true false)
      (set `self.Hit` true)
      (bind _as_bp_ai_chicken (`self.As BP AI Chicken`)
        (:`then`
          (`KismetSystemLibrary.Delay` 0.05)
          (`self.K2_DestroyActor` _as_bp_ai_chicken))
        (:`else`)))))

(event `/Game/Utility/Interfaces/BPI_Quest.TurnOnWaypoints`
  (params (ObjectiveID :type String) (`On/Off` :type Boolean))
  (bind _turninicon (`self.TurnInIcon`))
  (for _array_element (`/Game/Components/ActorComponents/AC_QuestTurnin.ObjectiveName` (`self.AC_QuestTurnin`))
    (if (`KismetStringLibrary.EqualEqual_StrStr` ObjectiveID _array_element)
      (if `On/Off`
        (`SceneComponent.SetHiddenInGame` _turninicon false false)
        (else
          (`SceneComponent.SetHiddenInGame` _turninicon true false))))))

(fn `UserConstructionScript`)