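; BP_SoftSurface is a level object that acts as a soft surface, either a hay pile or deep snow.
; Its construction script sets the mesh from MeshType and, for snow, optionally enables a visible, collidable physical surface.
; Overlapping actors receive SoftSurfaceMessage and trigger matching sound and splash effects, with the message cleared only when the player leaves.
; In the non-snow case, an overlapping BP_ChickenCrate snaps to AttachmentPoint, keeping its rotation.
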(event `self.OverlapVolume.OnComponentBeginOverlap`
  (params (OverlappedComponent :type "PrimitiveComponent Object Reference") (OtherActor :type "Actor Object Reference") (OtherComp :type "PrimitiveComponent Object Reference") (OtherBodyIndex :type Integer) (bFromSweep :type Boolean) (SweepResult :type "HitResult Structure (by ref)"))
  (bind _returnvalue (`self.K2_GetActorLocation` OtherActor))
  (bind _returnvalue_2 (`self.K2_GetActorLocation` OtherActor))
  (message `/Game/Utility/Interfaces/BPI_LevelMechanics.SoftSurface` OtherActor true)
  (if (`|EnumEquality` (`self.MeshType`) "NewEnumerator1")
    (`GameplayStatics.PlaySoundAtLocation` "/Game/SFX/CharacterSounds/Footsteps/Snow/DeepSnow/SC_DeepSnow.SC_DeepSnow" _returnvalue_2 (struct) 1.0 1.0 0.0 null null null null)
    (`NiagaraFunctionLibrary.SpawnSystemAtLocation` "/Game/Art/VFX/VFX_SnowSplash.VFX_SnowSplash" _returnvalue_2 (`KismetMathLibrary.MakeRotFromZ` SweepResult_ImpactPoint) (5.0 5.0 5.0))
    (else
      (`GameplayStatics.PlaySoundAtLocation` "/Game/SFX/CharacterSounds/Footsteps/Leaves_Branches_Hay/SC_Footsteps_Leaves_Hay_Branches.SC_Footsteps_Leaves_Hay_Branches" _returnvalue (struct) 1.0 1.0 0.0 null null null null)
      (`NiagaraFunctionLibrary.SpawnSystemAtLocation` "/Game/Art/VFX/VFX_HaySplash.VFX_HaySplash" _returnvalue (`KismetMathLibrary.MakeRotFromZ` SweepResult_ImpactPoint))
      (if (== (`GameplayStatics.GetObjectClass` OtherActor) "/Game/LevelObjects/BP_ChickenCrate.BP_ChickenCrate_C")
        (`self.K2_AttachToComponent` OtherActor (`self.AttachmentPoint`) "None" "SnapToTarget" "KeepWorld" "KeepWorld" true)))))

(event `self.OverlapVolume.OnComponentEndOverlap`
  (params (OverlappedComponent :type "PrimitiveComponent Object Reference") (OtherActor :type "Actor Object Reference") (OtherComp :type "PrimitiveComponent Object Reference") (OtherBodyIndex :type Integer))
  (if (== OtherActor (`GameplayStatics.GetPlayerPawn` 0))
    (message `/Game/Utility/Interfaces/BPI_LevelMechanics.SoftSurface` OtherActor false)))

(fn `QuestInteraction`
  (returns (ObjectiveID :type String))
  (return ""))

(fn `UserConstructionScript`
  (bind _physicalsurface (`self.PhysicalSurface`))
  (bind _mesh (`self.Mesh`))
  (bind _physicalsurface_2 (`self.PhysicalSurface`))
  (switch `/Game/Utility/Enums/E_SoftSurfaces` (`self.MeshType`)
    (:`NewEnumerator0`
      (`StaticMeshComponent.SetStaticMesh` _mesh "/Game/Aaron/Meshes/SM_HayPile.SM_HayPile")
      (`PrimitiveComponent.SetMaterial` _mesh 0 "/Game/Aaron/Materials/MI_HayStack.MI_HayStack"))
    (:`NewEnumerator1`
      (`StaticMeshComponent.SetStaticMesh` _mesh "/Engine/BasicShapes/Cube.Cube")
      (if (`self.PhysicalSurfaceActive?`)
        (`|ExecutionSequence`
          (:`then_0`
            (if (`|EnumEquality` (`self.MeshType`) "NewEnumerator1")
              (`PrimitiveComponent.SetMaterial` _physicalsurface_2 0 "/Game/Art/Materials/MI_DeepSnowBlue.MI_DeepSnowBlue")
              (else
                (`PrimitiveComponent.SetMaterial` _physicalsurface_2 0 "/Game/Aaron/Materials/MI_HayStack.MI_HayStack"))))
          (:`then_1`
            (`PrimitiveComponent.SetCollisionEnabled` _physicalsurface "QueryAndPhysics")
            (`SceneComponent.SetVisibility` _physicalsurface true false)))
        (else
          (`PrimitiveComponent.SetCollisionEnabled` _physicalsurface "NoCollision")
          (`SceneComponent.SetVisibility` _physicalsurface false false))))))