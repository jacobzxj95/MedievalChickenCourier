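; Water reset volume that teleports the player and other overlapping actors, except the pirate ship, back to a water well.
; The player moves behind a water-coloured camera fade, then a radial force impulse fires.
; Chickens are thrown mostly upward through an item-thrown message, while other actors get the impulse after a short delay.
; Separate well and surface volumes play splash sounds and spawn splash VFX on enter and exit.
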(event `self.ResetVolume.OnComponentBeginOverlap`
  (params (OverlappedComponent :type "PrimitiveComponent Object Reference") (OtherActor :type "Actor Object Reference") (OtherComp :type "PrimitiveComponent Object Reference") (OtherBodyIndex :type Integer) (bFromSweep :type Boolean) (SweepResult :type "HitResult Structure (by ref)"))
  (bind _returnvalue (`SceneComponent.K2_GetComponentLocation` (`self.SM_WaterWell`)))
  (if (== OtherActor (`GameplayStatics.GetPlayerPawn` 0))
    (`PlayerCameraManager.StartCameraFade` (`GameplayStatics.GetPlayerCameraManager` 0) 0.0 1.0 0.5 (struct :`G` 0.689592 :`B` 0.776042 :`A` 1.0) false true)
    (`KismetSystemLibrary.Delay` 0.5)
    (`self.K2_SetActorLocation` OtherActor _returnvalue false false)
    (`PlayerCameraManager.StartCameraFade` (`GameplayStatics.GetPlayerCameraManager` 0) 1.0 0.0 0.5 (struct :`G` 0.690196 :`B` 0.776471 :`A` 1.0) false true)
    (`RadialForceComponent.FireImpulse` (`self.RadialForce`) :!label _label)
    (elif (`self.ActorHasTag` OtherActor "Chicken")
      (set `self.IsChicken?` true)
      (`self.K2_SetActorLocation` OtherActor _returnvalue false false :!label _label_2)
      (if (not (`self.IsChicken?`))
        (`KismetSystemLibrary.Delay` 0.05)
        (goto _label)
        (else
          (message `/Game/Utility/Interfaces/BPI_EPS.ItemThrown` OtherActor 100.0 (+ (`self.GetActorForwardVector` OtherActor) (0.0 0.0 10.0)) (`self.GetTransform` OtherActor) false 0.0)))
      (elif (!= (`GameplayStatics.GetObjectClass` OtherActor) "/Game/LevelObjects/BP_PirateShip.BP_PirateShip_C")
        (goto _label_2)))))

(event `self.WellWaterVolume.OnComponentBeginOverlap`
  (params (OverlappedComponent :type "PrimitiveComponent Object Reference") (OtherActor :type "Actor Object Reference") (OtherComp :type "PrimitiveComponent Object Reference") (OtherBodyIndex :type Integer) (bFromSweep :type Boolean) (SweepResult :type "HitResult Structure (by ref)"))
  (`GameplayStatics.PlaySoundAtLocation` "/Game/SFX/Environment/SC_EnterWaterSplash.SC_EnterWaterSplash" (`SceneComponent.K2_GetComponentLocation` (`self.WellWaterVolume`)) (struct) 1.0 1.0 0.0 null null null null))

(event `self.WellWaterVolume.OnComponentEndOverlap`
  (params (OverlappedComponent :type "PrimitiveComponent Object Reference") (OtherActor :type "Actor Object Reference") (OtherComp :type "PrimitiveComponent Object Reference") (OtherBodyIndex :type Integer))
  (`GameplayStatics.PlaySoundAtLocation` "/Game/SFX/Environment/SC_ExitWaterSplash.SC_ExitWaterSplash" (`SceneComponent.K2_GetComponentLocation` (`self.WellWaterVolume`)) (struct) 0.5 1.0 0.5 null null null null)
  (set `self.IsChicken?` false))

(event `self.WaterSurfaceVolume.OnComponentBeginOverlap`
  (params (OverlappedComponent :type "PrimitiveComponent Object Reference") (OtherActor :type "Actor Object Reference") (OtherComp :type "PrimitiveComponent Object Reference") (OtherBodyIndex :type Integer) (bFromSweep :type Boolean) (SweepResult :type "HitResult Structure (by ref)"))
  (`NiagaraFunctionLibrary.SpawnSystemAtLocation` "/Game/Art/VFX/VFX_WaterSplash.VFX_WaterSplash" (`self.K2_GetActorLocation` OtherActor) (`KismetMathLibrary.MakeRotFromZ` SweepResult_ImpactPoint)))

(event `self.WaterSurfaceVolume.OnComponentEndOverlap`
  (params (OverlappedComponent :type "PrimitiveComponent Object Reference") (OtherActor :type "Actor Object Reference") (OtherComp :type "PrimitiveComponent Object Reference") (OtherBodyIndex :type Integer))
  (`NiagaraFunctionLibrary.SpawnSystemAtLocation` "/Game/Art/VFX/VFX_WaterSplash.VFX_WaterSplash" (+ (`SceneComponent.K2_GetComponentLocation` (`self.WaterSurfaceVolume`)) (0.0 0.0 30.0)) (`KismetMathLibrary.MakeRotFromZ` (`self.GetActorUpVector` OtherActor))))

(fn `UserConstructionScript`)