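; BP_MudPuddle is a level hazard that slows the player and weakens their jump while inside it.
; Box overlap casts to BP_PlayerChar, caches it, sets its player-effect enum and lowers walk speed and jump velocity.
; End overlap switches the effect and restores hardcoded default movement values rather than saved ones, for that cached player only.
; The construction script toggles the Cylinder and its children's visibility through MudCirclesVisible.
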(event `self.ReceiveBeginPlay`)

(event `self.ReceiveActorBeginOverlap`
  (params (OtherActor :type "Actor Object Reference")))

(event `self.Box.OnComponentBeginOverlap`
  (params (OverlappedComponent :type "PrimitiveComponent Object Reference") (OtherActor :type "Actor Object Reference") (OtherComp :type "PrimitiveComponent Object Reference") (OtherBodyIndex :type Integer) (bFromSweep :type Boolean) (SweepResult :type "HitResult Structure (by ref)"))
  (bind _asbp_player_char (cast `/Game/Characters/BP_PlayerChar` OtherActor))
  (set `self.As BP Player Char` _asbp_player_char)
  (set `/Game/Characters/BP_PlayerChar.E_PlayerEffects` "NewEnumerator2" _asbp_player_char)
  (bind _charactermovement (`Character.CharacterMovement` _asbp_player_char))
  (set `CharacterMovementComponent.MaxWalkSpeed` 200.0 _charactermovement)
  (set `CharacterMovementComponent.JumpZVelocity` 100.0 _charactermovement))

(event `self.Box.OnComponentEndOverlap`
  (params (OverlappedComponent :type "PrimitiveComponent Object Reference") (OtherActor :type "Actor Object Reference") (OtherComp :type "PrimitiveComponent Object Reference") (OtherBodyIndex :type Integer))
  ;[0.349 0.349 0.349] When the player leaves the mud, return their jump and movement to their default values
  (bind _as_bp_player_char (`self.As BP Player Char`)
    (:`then`
      (if (== _as_bp_player_char OtherActor)
        (set `/Game/Characters/BP_PlayerChar.E_PlayerEffects` "NewEnumerator3" _as_bp_player_char)
        (bind _charactermovement (`Character.CharacterMovement` _as_bp_player_char))
        (set `CharacterMovementComponent.MaxWalkSpeed` 660.0 _charactermovement)
        (set `CharacterMovementComponent.JumpZVelocity` 550.0 _charactermovement)))
    (:`else`)))

(event `/Game/Utility/Interfaces/BPI_Hit.HitByProjectile`)

(fn `UserConstructionScript`
  (`SceneComponent.SetVisibility` (`self.Cylinder`) (`self.MudCirclesVisible?`) true))