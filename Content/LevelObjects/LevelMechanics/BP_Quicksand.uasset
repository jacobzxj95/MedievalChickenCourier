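; Quicksand hazard that sinks the player and teleports them to a destination point.
; The overlap volume flags quicksand on the player, starts a sand-coloured camera fade and pauses held-chicken timers.
; Two near-identical teleport volume handlers move the player, fire a radial impulse, resume those timers and clear the state.
; Their chicken-tag branch throws the chicken but calls SetActorLocation on the quicksand itself; index-paired teleport code is unused.
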(event `self.ReceiveBeginPlay`
  (`GameplayStatics.PlaySoundAtLocation` "/Game/SFX/Mechanics/Quicksand/SC_QuicksandMovement.SC_QuicksandMovement" (`self.K2_GetActorLocation`) (struct) 1.0 1.0 0.0 null null null null)
  (`MovementComponent.SetUpdatedComponent` (`self.RotatingMovement`) (`self.LightColor_1`))
  (`KismetSystemLibrary.Delay` 3.0)
  (bind _playercharacterref (message `/Game/Utility/Interfaces/BPI_UI.Pass Out Playercharacter ref` (`GameplayStatics.GetGameMode`)))
  (set `self.Player Character Ref` _playercharacterref)
  (bind _asgm_mvp (cast `/Game/Maps/GameModes/GM_MVP` (`GameplayStatics.GetGameMode`)))
  (set `self.As GM MVP` _asgm_mvp))

(event `self.OverlapVolume.OnComponentBeginOverlap`
  (params (OverlappedComponent :type "PrimitiveComponent Object Reference") (OtherActor :type "Actor Object Reference") (OtherComp :type "PrimitiveComponent Object Reference") (OtherBodyIndex :type Integer) (bFromSweep :type Boolean) (SweepResult :type "HitResult Structure (by ref)"))
  (bind _chickentempermeter (`/Game/Maps/GameModes/GM_MVP.ChickenTemperMeter` (`self.As GM MVP`)))
  (`self.IsPlayer?` OtherActor
    (:`True`
      (bind _player_character_ref (`self.PlayerHasChicken?`)
        (:`PlayerHasChicken`
          (`KismetSystemLibrary.K2_PauseTimerHandle` (`/Game/Characters/BP_PlayerChar.ChickenTimerHandle` _player_character_ref))
          (`KismetSystemLibrary.K2_PauseTimerHandle` (`/Game/UI/W_TemperMeter.TemperDrainHandle` _chickentempermeter))
          ;[0.4896 0.418 0.2583] Check if the overlapping actor is the player and then see if the sinking timer is paused
          (`KismetSystemLibrary.K2_PauseTimerHandle` (`/Game/UI/W_TemperMeter.PlayerGripDurationHandle` _chickentempermeter)))
        (:`NotHoldingAChicken`
          _))
      (`/Engine/EditorBlueprintResources/StandardMacros.DoOnce` false :!label _label
        (:`Completed`
          (bind _output_get (set `self.InQuickSand?` true))
          (message `/Game/Utility/Interfaces/BPI_LevelMechanics.QuickSand` OtherActor _output_get)
          (`PlayerCameraManager.StartCameraFade` (`GameplayStatics.GetPlayerCameraManager` 0) 0.0 0.5 2.0 (struct :`R` 0.717647 :`G` 0.482353 :`B` 0.082353 :`A` 1.0) false true))))))

(event `ResetDoOnce`
  ;[0.4896 0.418 0.2583] Check if the overlapping actor is the player and then see if the sinking timer is paused
  (goto _label :!via `Reset`))

(event `self.TeleportVolume1.OnComponentBeginOverlap`
  (params (OverlappedComponent :type "PrimitiveComponent Object Reference") (OtherActor :type "Actor Object Reference") (OtherComp :type "PrimitiveComponent Object Reference") (OtherBodyIndex :type Integer) (bFromSweep :type Boolean) (SweepResult :type "HitResult Structure (by ref)"))
  (bind _returnvalue (`SceneComponent.K2_GetComponentLocation` (`self.TeleportDestination`)))
  (bind _chickentempermeter (`/Game/Maps/GameModes/GM_MVP.ChickenTemperMeter` (`self.As GM MVP`)))
  (`self.IsPlayer?` OtherActor
    (:`True`
      (`PlayerCameraManager.StartCameraFade` (`GameplayStatics.GetPlayerCameraManager` 0) 0.5 1.0 1.0 (struct :`R` 0.717647 :`G` 0.482353 :`B` 0.082353 :`A` 1.0) false true)
      (`|ExecutionSequence`
        (:`then_0`
          (`KismetSystemLibrary.Delay` 0.5)
          (`PlayerCameraManager.StartCameraFade` (`GameplayStatics.GetPlayerCameraManager` 0) 1.0 0.0 0.2 (struct :`R` 0.717647 :`G` 0.482353 :`B` 0.082353 :`A` 1.0) false true))
        (:`then_1`
          (bind _player_character_ref (`self.Player Character Ref`)
            (:`then`
              (`self.K2_SetActorLocation` _player_character_ref _returnvalue false true)
              (`self.ResetDoOnce`)
              (set `self.InQuickSand?` false)
              (bind _player_character_ref_2 (`self.PlayerHasChicken?`)
                (:`PlayerHasChicken`
                  (`KismetSystemLibrary.K2_UnPauseTimerHandle` (`/Game/Characters/BP_PlayerChar.ChickenTimerHandle` _player_character_ref_2))
                  (`KismetSystemLibrary.K2_UnPauseTimerHandle` (`/Game/UI/W_TemperMeter.PlayerGripDurationHandle` _chickentempermeter))
                  (`KismetSystemLibrary.K2_UnPauseTimerHandle` (`/Game/UI/W_TemperMeter.TemperDrainHandle` _chickentempermeter)))
                (:`NotHoldingAChicken`
                  _))
              (`RadialForceComponent.FireImpulse` (`self.RadialForce`))
              (bind _output_get (set `self.InQuickSand?` false))
              (message `/Game/Utility/Interfaces/BPI_LevelMechanics.QuickSand` (`self.Player Character Ref`) _output_get))
            (:`else`)))))
    (:`False`
      (if (`self.ActorHasTag` OtherActor "Chicken")
        (set `self.IsChicken?` true)
        (`self.K2_SetActorLocation` _returnvalue false true)
        (message `/Game/Utility/Interfaces/BPI_EPS.ItemThrown` OtherActor 100.0 (+ (`self.GetActorForwardVector` OtherActor) (0.0 0.0 10.0)) (`self.GetTransform` OtherActor) false 0.0)))))

(event `self.TeleportVolume2.OnComponentBeginOverlap`
  (params (OverlappedComponent :type "PrimitiveComponent Object Reference") (OtherActor :type "Actor Object Reference") (OtherComp :type "PrimitiveComponent Object Reference") (OtherBodyIndex :type Integer) (bFromSweep :type Boolean) (SweepResult :type "HitResult Structure (by ref)"))
  (bind _returnvalue (`SceneComponent.K2_GetComponentLocation` (`self.TeleportDestination`)))
  (bind _chickentempermeter (`/Game/Maps/GameModes/GM_MVP.ChickenTemperMeter` (`self.As GM MVP`)))
  (`self.IsPlayer?` OtherActor
    (:`True`
      (`PlayerCameraManager.StartCameraFade` (`GameplayStatics.GetPlayerCameraManager` 0) 0.5 1.0 1.0 (struct :`R` 0.717647 :`G` 0.482353 :`B` 0.082353 :`A` 1.0) false true)
      (`|ExecutionSequence`
        (:`then_0`
          (`KismetSystemLibrary.Delay` 0.5)
          (`PlayerCameraManager.StartCameraFade` (`GameplayStatics.GetPlayerCameraManager` 0) 1.0 0.0 0.2 (struct :`R` 0.717647 :`G` 0.482353 :`B` 0.082353 :`A` 1.0) false true))
        (:`then_1`
          (bind _player_character_ref (`self.Player Character Ref`)
            (:`then`
              (`self.K2_SetActorLocation` _player_character_ref _returnvalue false true)
              (`self.ResetDoOnce`)
              (set `self.InQuickSand?` false)
              (bind _player_character_ref_2 (`self.PlayerHasChicken?`)
                (:`PlayerHasChicken`
                  (`KismetSystemLibrary.K2_UnPauseTimerHandle` (`/Game/Characters/BP_PlayerChar.ChickenTimerHandle` _player_character_ref_2))
                  (`KismetSystemLibrary.K2_UnPauseTimerHandle` (`/Game/UI/W_TemperMeter.PlayerGripDurationHandle` _chickentempermeter))
                  (`KismetSystemLibrary.K2_UnPauseTimerHandle` (`/Game/UI/W_TemperMeter.TemperDrainHandle` _chickentempermeter)))
                (:`NotHoldingAChicken`
                  _))
              (`RadialForceComponent.FireImpulse` (`self.RadialForce`))
              (bind _output_get (set `self.InQuickSand?` false))
              (message `/Game/Utility/Interfaces/BPI_LevelMechanics.QuickSand` (`self.Player Character Ref`) _output_get))
            (:`else`)))))
    (:`False`
      (if (`self.ActorHasTag` OtherActor "Chicken")
        (set `self.IsChicken?` true)
        (`self.K2_SetActorLocation` _returnvalue false true)
        (message `/Game/Utility/Interfaces/BPI_EPS.ItemThrown` OtherActor 100.0 (+ (`self.GetActorForwardVector` OtherActor) (0.0 0.0 10.0)) (`self.GetTransform` OtherActor) false 0.0)
        (else
          (`KismetSystemLibrary.PrintString` "SOMETHING AINT RIGHT WITH THIS QUICK SAND"))))))

(event `Teleport`
  ;[1 1 1] Not used: Gregs old code
  (if (`self.isEntrance?`)
    (bind _outactors (`GameplayStatics.GetAllActorsOfClass` "BP_Quicksand_C"))
    (for _array_element _outactors
      (if (and (== (`/Game/LevelObjects/LevelMechanics/BP_Quicksand.QuicksandIndex` _array_element) (`self.QuicksandIndex`)) (not (`/Game/LevelObjects/LevelMechanics/BP_Quicksand.isEntrance?` _array_element)))
        (break)))
    (`self.Call Move Actor` _array_element)
    (else
      (bind _outactors_2 (`GameplayStatics.GetAllActorsOfClass` "BP_Quicksand_C"))
      (for _array_element_2 _outactors_2
        (if (and (== (`/Game/LevelObjects/LevelMechanics/BP_Quicksand.QuicksandIndex` _array_element_2) (`self.QuicksandIndex`)) (and (not (`self.isEntrance?`)) (`/Game/LevelObjects/LevelMechanics/BP_Quicksand.isEntrance?` _array_element_2)))
          (break)))
      (`self.Call Move Actor` _array_element_2))))

(event `Call Move Actor`
  (params (Target :type "/Game/LevelObjects/LevelMechanics/BP_Quicksand Object Reference"))
  ;[1 1 1] Not used: Gregs old code
)

(event `SetCollision`
  ;[1 1 1] Not used: Gregs old code
  (`PrimitiveComponent.SetCollisionEnabled` (`self.OverlapVolume`) "QueryAndPhysics"))

(fn `QuestInteraction`
  (returns (ObjectiveID :type String))
  (return ""))

(fn `UserConstructionScript`)