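; BP_SlipperyIce is a level mechanic volume that marks an area as slippery ice.
; Its Box overlap events send SlipperyIceMessage true on enter and false on exit to actors implementing BPI_LevelMechanics, leaving the slip response to them.
; The construction script scales the Box and Plane in X and Y by Size, toggles Plane visibility with ShowPlane and tints its material.
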(event `self.ReceiveBeginPlay`)

(event `self.Box.OnComponentBeginOverlap`
  (params (OverlappedComponent :type "PrimitiveComponent Object Reference") (OtherActor :type "Actor Object Reference") (OtherComp :type "PrimitiveComponent Object Reference") (OtherBodyIndex :type Integer) (bFromSweep :type Boolean) (SweepResult :type "HitResult Structure (by ref)"))
  ;[1 1 1] On Ice
  (if (`KismetSystemLibrary.DoesImplementInterface` OtherActor "/Game/Utility/Interfaces/BPI_LevelMechanics.BPI_LevelMechanics_C")
    (message `/Game/Utility/Interfaces/BPI_LevelMechanics.SlipperyIce` OtherActor true)))

(event `self.Box.OnComponentEndOverlap`
  (params (OverlappedComponent :type "PrimitiveComponent Object Reference") (OtherActor :type "Actor Object Reference") (OtherComp :type "PrimitiveComponent Object Reference") (OtherBodyIndex :type Integer))
  ;[0.1406 0.1406 0.1406] Off Ice
  (if (`KismetSystemLibrary.DoesImplementInterface` OtherActor "/Game/Utility/Interfaces/BPI_LevelMechanics.BPI_LevelMechanics_C")
    (message `/Game/Utility/Interfaces/BPI_LevelMechanics.SlipperyIce` OtherActor false)))

(fn `UserConstructionScript`
  (bind _size (`self.Size`))
  (`SceneComponent.SetVisibility` (`self.Plane`) (`self.ShowPlane?`) false)
  (`SceneComponent.SetRelativeScale3D` (`self.Box`) (`KismetMathLibrary.MakeVector` _size _size 1.0))
  (`SceneComponent.SetRelativeScale3D` (`self.Plane`) (`KismetMathLibrary.MakeVector` _size _size 1.0))
  (`MeshComponent.SetVectorParameterValueOnMaterials` (`self.Plane`) "Color" (1.0 0.0 0.5)))