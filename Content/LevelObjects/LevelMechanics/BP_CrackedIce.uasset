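; Cracked ice hazard that collapses under the player and drops them into water, then teleports them to an exit point.
; Standing on the surface runs a durability timer that pauses on step-off and resumes on return; expiry removes collision, sinks the ice and switches camera.
; Water and portal volumes handle splash effects, screen fades, relocation and view restoration.
; The player receives ice state through CrackedIceMessage calls.
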(event `self.ReceiveBeginPlay`)

(event `self.SurfaceTriggerVolume.OnComponentBeginOverlap`
  (params (OverlappedComponent :type "PrimitiveComponent Object Reference") (OtherActor :type "Actor Object Reference") (OtherComp :type "PrimitiveComponent Object Reference") (OtherBodyIndex :type Integer) (bFromSweep :type Boolean) (SweepResult :type "HitResult Structure (by ref)"))
  (bind _durabilitydurationhandle (`self.DurabilityDurationHandle`))
  ;[0.7887 0 1] On overlap, start or unpause the timer for the duration of the ice's durability
  (`self.IsThePlayer?` OtherActor
    (:`True`
      (`/Engine/EditorBlueprintResources/StandardMacros.DoOnce` false :!label _label
        (:`Completed`
          (if (not (`self.IceIsGone?`))
            (set `self.OnCrackedIce?` true)
            (if (`KismetSystemLibrary.K2_IsTimerPausedHandle` _durabilitydurationhandle)
              (`KismetSystemLibrary.K2_UnPauseTimerHandle` _durabilitydurationhandle)
              (`GameplayStatics.PlaySoundAtLocation` "/Game/SFX/Mechanics/CrackedIce/SC_CrackingIce.SC_CrackingIce" (`self.K2_GetActorLocation`) (struct) 1.0 1.0 0.0 null null null null)
              (else
                (`GameplayStatics.PlaySoundAtLocation` "/Game/SFX/Mechanics/CrackedIce/SC_CrackingIce.SC_CrackingIce" (`self.K2_GetActorLocation`) (struct) 1.0 1.0 0.0 null null null null)
                (bind _returnvalue (`KismetSystemLibrary.K2_SetTimerDelegate` (delegate `MoveIce`) 3.0))
                (set `self.DurabilityDurationHandle` _returnvalue)))))))))

(event `ResetDoOnce`
  ;[0.7887 0 1] On overlap, start or unpause the timer for the duration of the ice's durability
  (goto _label :!via `Reset`))

(event `MoveIce`
  (bind _ice (`self.Ice`))
  (bind _oncrackedice_ (`self.OnCrackedIce?`))
  (bind _relativelocation (`SceneComponent.RelativeLocation` _ice))
  ;[0.7887 0 1] On overlap, start or unpause the timer for the duration of the ice's durability
  (`PrimitiveComponent.SetCollisionEnabled` (`self.Ice`) "NoCollision")
  (`GameplayStatics.PlaySoundAtLocation` "/Game/SFX/Mechanics/CrackedIce/ES_Impact_Ice_Sheet_2_-_SFX_Producer.ES_Impact_Ice_Sheet_2_-_SFX_Producer" (`self.K2_GetActorLocation`) (struct) 1.0 1.0 0.0 null null null null)
  (bind _output_get (set `self.IceIsGone?` true))
  (message `/Game/Utility/Interfaces/BPI_LevelMechanics.CrackedIce` (stale `self.SurfaceTriggerVolume.OnComponentBeginOverlap` OtherActor) _oncrackedice_ self _output_get (and _oncrackedice_ (`self.IceIsGone?`)))
  (`PlayerController.SetViewTargetWithBlend` (`GameplayStatics.GetPlayerController` 0) (`ActorComponent.GetOwner` (`self.Camera`)) 0.0 "VTBlend_Linear" 0.0 false)
  (bind (_direction _alpha) (`Timeline|IceMoveAlpha`)
    (:`Update`
      (`SceneComponent.K2_SetRelativeLocation` _ice (`KismetMathLibrary.VLerp` _relativelocation (- _relativelocation (0.0 0.0 50.0)) _alpha) false false))))

(event `self.SurfaceTriggerVolume.OnComponentEndOverlap`
  (params (OverlappedComponent :type "PrimitiveComponent Object Reference") (OtherActor :type "Actor Object Reference") (OtherComp :type "PrimitiveComponent Object Reference") (OtherBodyIndex :type Integer))
  (bind _durabilitydurationhandle (`self.DurabilityDurationHandle`))
  ;[0.02078 1 0.9901] On end overlap, stop the durability duration timer if the player got off of the ice in time.
  (`self.IsThePlayer?` OtherActor
    (:`True`
      (set `self.OnCrackedIce?` false)
      (`KismetSystemLibrary.K2_PauseTimerHandle` _durabilitydurationhandle)
      (if (> (`KismetSystemLibrary.K2_GetTimerElapsedTimeHandle` _durabilitydurationhandle) 3.0)
        (`PrimitiveComponent.SetCollisionEnabled` (`self.Ice`) "QueryAndPhysics"))
      (`self.ResetDoOnce`)
      (`PlayerController.SetViewTargetWithBlend` (`GameplayStatics.GetPlayerController` 0) OtherActor 0.0 "VTBlend_Linear" 0.0 false))))

(event `self.WaterLevelVolume.OnComponentBeginOverlap`
  (params (OverlappedComponent :type "PrimitiveComponent Object Reference") (OtherActor :type "Actor Object Reference") (OtherComp :type "PrimitiveComponent Object Reference") (OtherBodyIndex :type Integer) (bFromSweep :type Boolean) (SweepResult :type "HitResult Structure (by ref)"))
  ;[0.03332 0.148 1] Play the watersplash sound on impact.
  (`self.IsThePlayer?` OtherActor
    (:`True`
      (message `/Game/Utility/Interfaces/BPI_LevelMechanics.CrackedIce` OtherActor (`self.OnCrackedIce?`) self (`self.IceIsGone?`) false)
      (`PlayerCameraManager.StartCameraFade` (`GameplayStatics.GetPlayerCameraManager` 0) 0.0 1.0 2.0 (struct :`G` 0.082353 :`B` 0.623529 :`A` 1.0) false true))
    (:`False`
      _))
  (`/Engine/EditorBlueprintResources/StandardMacros.DoOnce` false :!label _label_2
    (:`Completed`
      (`GameplayStatics.PlaySoundAtLocation` "/Game/SFX/Mechanics/CrackedIce/ES_Impact_Water_Ice_1_-_SFX_Producer.ES_Impact_Water_Ice_1_-_SFX_Producer" (`self.K2_GetActorLocation`) (struct) 1.0 1.0 0.0 null null null null)
      (`NiagaraFunctionLibrary.SpawnSystemAtLocation` "/Game/Art/VFX/VFX_WaterSplash.VFX_WaterSplash" (`self.K2_GetActorLocation` OtherActor) (`KismetMathLibrary.MakeRotFromZ` SweepResult_ImpactNormal))
      (`KismetSystemLibrary.Delay` 0.2)
      (`self.ResetWaterSplashDoOnce`))))

(event `ResetWaterSplashDoOnce`
  ;[0.03332 0.148 1] Play the watersplash sound on impact.
  (goto _label_2 :!via `Reset`))

(event `self.PortalVolume.OnComponentBeginOverlap`
  (params (OverlappedComponent :type "PrimitiveComponent Object Reference") (OtherActor :type "Actor Object Reference") (OtherComp :type "PrimitiveComponent Object Reference") (OtherBodyIndex :type Integer) (bFromSweep :type Boolean) (SweepResult :type "HitResult Structure (by ref)"))
  ;[0 1 0.001622] Ideally this would be done elsewhere, where we could call the teleportation effects/script for other level mechanics like the mud and quicksand (unless the quicksand becomes something completely different)
  (`self.K2_SetActorLocation` OtherActor (`self.PortalExitLocation`) false false)
  (`self.IsThePlayer?` OtherActor
    (:`True`
      ;[0.08121 1 0.9403] Ensure the player is considered to be on cracked ice (disables their movement) for the duration of the collapsed ice and for them to be submerged in water.
      (message `/Game/Utility/Interfaces/BPI_LevelMechanics.CrackedIce` OtherActor (`self.OnCrackedIce?`) self (`self.IceIsGone?`) false)
      (`PlayerController.SetViewTargetWithBlend` (`GameplayStatics.GetPlayerController` 0) OtherActor 0.0 "VTBlend_Linear" 0.0 false)
      (`PlayerCameraManager.StartCameraFade` :`self` (`GameplayStatics.GetPlayerCameraManager` 0) :`FromAlpha` 1.0 :`Duration` 1.0 :`bHoldWhenFinished` true)
      (`KismetSystemLibrary.Delay` 2.0)
      (message `/Game/Utility/Interfaces/BPI_LevelMechanics.CrackedIce` OtherActor (`self.OnCrackedIce?`) self (`self.IceIsGone?`) false))))

(event `self.WaterLevelVolume.OnComponentEndOverlap`
  (params (OverlappedComponent :type "PrimitiveComponent Object Reference") (OtherActor :type "Actor Object Reference") (OtherComp :type "PrimitiveComponent Object Reference") (OtherBodyIndex :type Integer))
  (`self.IsThePlayer?` OtherActor
    (:`True`
      (`PlayerCameraManager.StartCameraFade` (`GameplayStatics.GetPlayerCameraManager` 0) 1.0 0.0 2.0 (struct :`G` 0.082353 :`B` 0.623529 :`A` 1.0) false true))))

(fn `UserConstructionScript`)