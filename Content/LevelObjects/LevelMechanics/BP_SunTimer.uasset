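; BP_SunTimer runs each level's day/night cycle and the nightfall deadline for time-sensitive quests.
; Tick rotates the sun, waiting for quest start in Deserton and Winterton, with pitch thresholds driving torches, lanterns, post-process, fog and sky.
; Per-level DoOnce gates reset each other to fire transitions once, with timelines fading lighting.
; Day/night quests show a HUD clock, cue villagers to the chapel and can fail at night; failures play a fade-and-relight sequence.
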(event `Stop Timer`
  (params (Manager :type "/Game/RodgerL/BP_QuestManager Object Reference"))
  (`KismetSystemLibrary.K2_ClearAndInvalidateTimerHandle` (`self.60secTimer`))
  (`KismetSystemLibrary.K2_ClearAndInvalidateTimerHandle` (`self.90SecTimer`)))

(event `self.ReceiveBeginPlay`
  (bind _returnvalue_roll (`KismetMathLibrary.BreakRotator` (`self.K2_GetActorRotation` (`self.SunRef`))))
  (`self.TimeSensitiveLevelCheck`)
  (`self.SetCurrentLevel`)
  (bind _outactors (`GameplayStatics.GetAllActorsOfClass` "/Game/LevelObjects/BP_WallTorch.BP_WallTorch_C"))
  (set `self.Torches` _outactors)
  (bind _outactors_2 (`GameplayStatics.GetAllActorsOfClass` "/Game/LevelObjects/BP_Lantern.BP_Lantern_C"))
  (set `self.Lanterns` _outactors_2)
  (bind _asbp_game_instance (cast `/Game/Utility/GameModes/BP_GameInstance` (`GameplayStatics.GetGameInstance`)))
  (set `self.As BP Game Instance` _asbp_game_instance)
  (bind _asgm_mvp (cast `/Game/Maps/GameModes/GM_MVP` (`GameplayStatics.GetGameMode`)))
  (bind _playerhud (`/Game/Maps/GameModes/GM_MVP.PlayerHUD` _asgm_mvp))
  (`/Engine/EditorBlueprintResources/StandardMacros.IsValid` _playerhud :!label _label
    (:`Is Valid`
      (set `self.HUD` _playerhud)
      (bind _playerchar (`/Game/Maps/GameModes/GM_MVP.PlayerChar` _asgm_mvp))
      (`/Engine/EditorBlueprintResources/StandardMacros.IsValid` _playerchar :!label _label_2
        (:`Is Valid`
          (bind _output_get (set `self.PlayerCharRef` _playerchar))
          (add `/Game/Components/ActorComponents/AC_Questlog.Quest Started` (`/Game/Characters/BP_PlayerChar.AC_QuestTurnIn` _output_get) (delegate `Started Main Quest`))
          (set `self.StartingRotation` _returnvalue_roll)
          (set `self.FinishedRotation` (+ _returnvalue_roll 180.0)))
        (:`Is Not Valid`
          (`KismetSystemLibrary.DelayUntilNextTick`)
          (goto _label_2))))
    (:`Is Not Valid`
      (`KismetSystemLibrary.DelayUntilNextTick`)
      (goto _label))))

(event `Started Main Quest`
  (params (ActiveQuest :type "/Game/RodgerL/BP_QuestManager Object Reference"))
  (bind _hud (`self.HUD`))
  (bind _output_get (set `self.MainQuestRef` ActiveQuest))
  (set `self.QuestStarted` true)
  (`/Engine/EditorBlueprintResources/StandardMacros.IsValid` _output_get
    (:`Is Valid`
      (if (`.DayNightLossCondition_28_525E3B524BCCFBB40506DC96BB5017F7` (break `/Game/Utility/Struct/STR_QuestDetails` (`/Game/RodgerL/BP_QuestManager.QuestDetails` _output_get)))
        (`Widget.SetVisibility` (`/Game/UI/W_HUD.ClockFrame` _hud) "Visible")
        (`Widget.SetVisibility` (`/Game/UI/W_HUD.ClockBackground` _hud) "Visible")
        (`UserWidget.PlayAnimation` _hud (`/Game/UI/W_HUD.ClockRotate` _hud) 0.0 1 "Forward" (* (`self.SunSpeed`) 0.25) true)
        (set `self.QuestHasDayNightLossCondition` true))
      (add `/Game/RodgerL/BP_QuestManager.Quest Failed` _output_get (delegate `QuestFailed`))
      (add `/Game/RodgerL/BP_QuestManager.QuestCompleted` _output_get (delegate `Stop Timer`)))))

(event `QuestFailed`
  (params (Loss :type String))
  (bind _as_bp_game_instance (`self.As BP Game Instance`)
    (:`then`
      (set `self.TriggeredLossCondition` Loss)
      (`/Game/Utility/GameModes/BP_GameInstance.Stop Music` _as_bp_game_instance)
      (`GameplayStatics.PlaySound2D` "/Game/SFX/QuestRelated/STGR_Fail_3.STGR_Fail_3" 1.0 1.0 0.0 null null)
      (bind _returnvalue (`|CreateWidget` "/Game/UI/WBP_QuestFailed.WBP_QuestFailed_C"))
      (`UserWidget.AddToViewport` _returnvalue 0)
      (`PlayerCameraManager.StartCameraFade` :`self` (`GameplayStatics.GetPlayerCameraManager` 0) :`ToAlpha` 1.0 :`Duration` 1.0 :`bHoldWhenFinished` true)
      (`KismetSystemLibrary.Delay` 1.5)
      (`PlayerController.SetViewTargetWithBlend` (`GameplayStatics.GetPlayerController` 0) self 0.0 "VTBlend_Linear" 0.0 false)
      (`KismetSystemLibrary.Delay` 1.0)
      (`PlayerCameraManager.StartCameraFade` :`self` (`GameplayStatics.GetPlayerCameraManager` 0) :`FromAlpha` 1.0 :`Duration` 1.0)
      (`self.Quest Failed`))
    (:`else`)))

(event `Quest Failed`
  (bind _sunref (`self.SunRef`))
  (bind (_returnvalue_roll _returnvalue_pitch) (`KismetMathLibrary.BreakRotator` (`self.K2_GetActorRotation` (`self.SunRef`))))
  ;[1 1 1] Quest Failed Lerp
  (bind (_direction _lerp_slowly) (`Timeline|Quickly Lerp` :!via `PlayFromStart`)
    (:`Update`
      (`|ExecutionSequence`
        (:`then_0`
          (`/Engine/EditorBlueprintResources/StandardMacros.DoOnce` false
            (:`Completed`
              (`KismetSystemLibrary.Delay` 4.0)
              (`SceneComponent.SetHiddenInGame` (`self.SkySphereMesh`) true false))))
        (:`then_1`
          (`self.K2_AddActorLocalRotation` _sunref (`KismetMathLibrary.MakeRotator` 0.0 (`KismetMathLibrary.Lerp` _returnvalue_pitch 1.5 _lerp_slowly)) false false)
          (`LightComponent.SetIntensity` (`Light.LightComponent` _sunref) (`KismetMathLibrary.Lerp` (`LightComponentBase.Intensity` (`Light.LightComponent` (`self.SunRef`))) 6.0 _lerp_slowly))
          (`MeshComponent.SetScalarParameterValueOnMaterials` (`self.SkySphereMesh`) "Opacity" (`KismetMathLibrary.Lerp` 1.0 0.0 _lerp_slowly))
          (`SkyLightComponent.SetIntensity` (`SkyLight.LightComponent` (`self.SkylightRef`)) (`KismetMathLibrary.Lerp` 0.3 0.8 _lerp_slowly)))))
    (:`Finished`
      (`PrimitiveComponent.SetMaterial` (`self.SkySphereMesh`) 0 "/Engine/EngineSky/M_Sky_Panning_Clouds2.M_Sky_Panning_Clouds2")
      (bind _as_bp_game_instance (`self.As BP Game Instance`)
        (:`then`
          (`/Game/Utility/GameModes/BP_GameInstance.Quest Failed` _as_bp_game_instance (`self.TriggeredLossCondition`)))
        (:`else`)))))

(event `1/4  Done`
  (bind _outactors (`GameplayStatics.GetAllActorsOfClass` "/Game/Characters/BP_Villager.BP_Villager_C"))
  (for _array_element _outactors
    (`BlackboardComponent.SetValueAsBool` (`AIBlueprintHelperLibrary.GetBlackboard` (`AIBlueprintHelperLibrary.GetAIController` _array_element)) "Call_SO_Claim_Chapel" true)))

(event `ResetCastletonNotAlmostNight`
  ;[0 1 0.06875] Castleton Custom Day/Night Cycle
  (goto _label_4 :!via `Reset`))

(event `ResetCastletonNight`
  (bind _skyspheremesh (`self.SkySphereMesh`))
  ;[0 1 0.06875] Castleton Custom Day/Night Cycle
  ;;[0.125 0.125 0.125] Day/Night Transition
  (goto _label_6 :!via `Reset`))

(event `ResetCastletonDay`
  (bind _skyspheremesh (`self.SkySphereMesh`))
  ;[0 1 0.06875] Castleton Custom Day/Night Cycle
  ;;[0.125 0.125 0.125] Day/Night Transition
  (goto _label_8 :!via `Reset`))

(event `ResetCastletonAlmostNight`
  ;[0 1 0.06875] Castleton Custom Day/Night Cycle
  (goto _label_9 :!via `Reset`))

(event `ResetRufftonNotAlmostNight`
  ;[0.01649 0 1] Ruffton Custom Day/Night Cycle
  (goto _label_11 :!via `Reset`))

(event `self.ReceiveTick`
  (params (DeltaSeconds :type "Float (single-precision)"))
  (bind _skyspheremesh (`self.SkySphereMesh`))
  (bind _sunref (`self.SunRef`))
  (bind _sunref_2 (`self.SunRef`))
  (bind _sunref_3 (`self.SunRef`))
  (bind _skyspheremesh_2 (`self.SkySphereMesh`))
  (bind _skyspheremesh_3 (`self.SkySphereMesh`))
  (bind _sunref_4 (`self.SunRef`))
  (bind _skyspheremesh_4 (`self.SkySphereMesh`))
  (bind (_returnvalue_roll _returnvalue_pitch) (`KismetMathLibrary.BreakRotator` (`self.K2_GetActorRotation` _sunref_4)))
  (bind (_returnvalue_roll_2 _returnvalue_pitch_2) (`KismetMathLibrary.BreakRotator` (`self.K2_GetActorRotation` _sunref_2)))
  (bind (_returnvalue_roll_3 _returnvalue_pitch_3) (`KismetMathLibrary.BreakRotator` (`self.K2_GetActorRotation` _sunref)))
  (bind (_returnvalue_roll_4 _returnvalue_pitch_4) (`KismetMathLibrary.BreakRotator` (`self.K2_GetActorRotation` _sunref_3)))
  (bind _component (`ExponentialHeightFog.Component` (`self.ExponentialHeightFog`)))
  (bind _component_2 (`ExponentialHeightFog.Component` (`self.ExponentialHeightFog`)))
  (bind _component_3 (`ExponentialHeightFog.Component` (`self.ExponentialHeightFog`)))
  (bind _component_4 (`ExponentialHeightFog.Component` (`self.ExponentialHeightFog`)))
  (bind _returnvalue (`KismetMathLibrary.MakeRotator` 0.0 (* DeltaSeconds (`self.SunSpeed`))))
  (`|ExecutionSequence`
    (:`then_0`
      (if (`self.QuestHasDayNightLossCondition`)
        (`/Engine/EditorBlueprintResources/StandardMacros.DoOnce` false
          (:`Completed`
            (bind _returnvalue_2 (`KismetSystemLibrary.K2_SetTimerDelegate` (delegate `1/4  Done`) 30.0))
            (set `self.30sec Timer` _returnvalue_2)))))
    (:`then_1`
      (if (not (`self.LvlHasTimeSensitiveQuest`))
        ;[0.01649 0 1] Ruffton Custom Day/Night Cycle
        ;;[1 0.7789 0] Move the Sun
        (switch `/Game/Utility/Enums/E_Levels` (`self.CurrentLevel`) :!label _label_3
          (:`NewEnumerator0`
            ;[0 1 0.06875] Castleton Custom Day/Night Cycle
            ;;[1 0.7789 0] Move the Sun
            (bind _as_bp_game_instance (`self.As BP Game Instance`)
              (:`then`
                (if (`/Game/Utility/GameModes/BP_GameInstance.GameStartSequenceFinished?` _as_bp_game_instance)
                  (`self.K2_AddActorLocalRotation` _sunref _returnvalue false false)
                  (if (> _returnvalue_pitch_3 -4.0)
                    (set `self.AlmostNight?` true)
                    (`|ExecutionSequence`
                      (:`then_0`
                        (`/Engine/EditorBlueprintResources/StandardMacros.DoOnce` false :!label _label_4
                          (:`Completed`
                            (`self.ToggleLights`)
                            (`self.CastletonPostProcessVolumeSetting`)
                            (`self.ResetCastletonAlmostNight`))))
                      (:`then_1`
                        ;;[0.125 0.125 0.125] Day/Night Transition
                        (if (> _returnvalue_pitch_3 2.0) :!label _label_5
                          (`/Engine/EditorBlueprintResources/StandardMacros.DoOnce` false :!label _label_6
                            (:`Completed`
                              (set `self.NightTIme` true)
                              (`SceneComponent.SetHiddenInGame` _skyspheremesh false false)
                              (`PrimitiveComponent.SetMaterial` _skyspheremesh 0 "/Game/Art/Materials/Sky_Materials/M_StaryNight.M_StaryNight")
                              (`ExponentialHeightFogComponent.SetFogDensity` _component 0.05)
                              ;;[0.1896 0.3782 1] Update the suns intensity (currently set up to deacrease the intesnity to 0.01 after 10 min)
                              (bind (_direction _alpha) (`Timeline|Timeline_0` :!label _label_7)
                                (:`Update`
                                  (`MeshComponent.SetScalarParameterValueOnMaterials` _skyspheremesh "Opacity" (`KismetMathLibrary.Lerp` 0.0 0.5 _alpha))
                                  (`SkyLightComponent.SetIntensity` (`SkyLight.LightComponent` (`self.SkylightRef`)) (`KismetMathLibrary.Lerp` 0.6 0.1 _alpha))
                                  (`LightComponent.SetIntensity` (`Light.LightComponent` (`self.SunRef`)) (`KismetMathLibrary.Lerp` 7.0 0.01 _alpha)))
                                (:`Finished`
                                  (`self.ResetCastletonNight`)))))
                          (else
                            (`/Engine/EditorBlueprintResources/StandardMacros.DoOnce` false :!label _label_8
                              (:`Completed`
                                (set `self.NightTIme` false)
                                (`SceneComponent.SetHiddenInGame` _skyspheremesh true false)
                                (`self.ResetCastletonDay`)
                                (`ExponentialHeightFogComponent.SetFogDensity` _component 0.01)
                                (goto _label_7 :!via `Reverse`)))))))
                    (else
                      (set `self.AlmostNight?` false)
                      (`|ExecutionSequence`
                        (:`then_0`
                          (goto _label_5))
                        (:`then_1`
                          (`/Engine/EditorBlueprintResources/StandardMacros.DoOnce` false :!label _label_9
                            (:`Completed`
                              (`self.ToggleLights`)
                              (`self.CastletonPostProcessVolumeSetting`)
                              (`self.ResetCastletonNotAlmostNight`)))))))))
              (:`else`
                (`KismetSystemLibrary.PrintString` "Sun Timer: INVALID GAME INSTANCE VAR" true true (struct :`R` 1.0 :`G` 0.027941 :`A` 1.0) 7.0))))
          (:`NewEnumerator1`
            (`self.K2_AddActorLocalRotation` _sunref_4 _returnvalue false false :!label _label_10)
            (if (> _returnvalue_pitch -4.0)
              (set `self.AlmostNight?` true)
              (`|ExecutionSequence`
                (:`then_0`
                  (`/Engine/EditorBlueprintResources/StandardMacros.DoOnce` false :!label _label_11
                    (:`Completed`
                      (`self.ToggleLights`)
                      (`self.RufftonPostProcessVolumeSetting`)
                      (`self.ResetRufftonAlmostNight`))))
                (:`then_1`
                  ;;[0.125 0.125 0.125] Day/Night Transition
                  (if (> _returnvalue_pitch 2.0) :!label _label_12
                    (`/Engine/EditorBlueprintResources/StandardMacros.DoOnce` false :!label _label_13
                      (:`Completed`
                        (set `self.NightTIme` true)
                        (`SceneComponent.SetHiddenInGame` _skyspheremesh_3 false false)
                        (`PrimitiveComponent.SetMaterial` _skyspheremesh_3 0 "/Game/Art/Materials/Sky_Materials/M_StaryNight.M_StaryNight")
                        (`ExponentialHeightFogComponent.SetFogDensity` _component_2 0.1)
                        (`|ExecutionSequence`
                          (:`then_0`
                            ;[1 1 1] wait for timeline below
                            (`KismetSystemLibrary.Delay` 3.0 :!label _label_14)
                            (if (and (not (`self.Quest Has Been Completed`)) (`self.QuestHasDayNightLossCondition`))
                              ;[1 0 0] Mission Failure
                              (`/Game/RodgerL/BP_QuestManager.Quest Failed` (`self.MainQuestRef`) "DayNight")
                              (set `self.QuestHasDayNightLossCondition` false)))
                          (:`then_1`
                            ;;[0.1896 0.3782 1] Update the suns intensity (currently set up to deacrease the intesnity to 0.01 after 10 min)
                            (bind (_direction_2 _alpha_2) (`Timeline|Timeline` :!label _label_15)
                              (:`Update`
                                (`MeshComponent.SetScalarParameterValueOnMaterials` _skyspheremesh_3 "Opacity" (`KismetMathLibrary.Lerp` 0.0 1.0 _alpha_2))
                                (`SkyLightComponent.SetIntensity` (`SkyLight.LightComponent` (`self.SkylightRef`)) (`KismetMathLibrary.Lerp` 0.8 0.3 _alpha_2))
                                (`LightComponent.SetIntensity` (`Light.LightComponent` (`self.SunRef`)) (`KismetMathLibrary.Lerp` 6.0 0.03 _alpha_2)))
                              (:`Finished`
                                (`self.ResetDayDoOnce`)))))))
                    (else
                      (`/Engine/EditorBlueprintResources/StandardMacros.DoOnce` false :!label _label_16
                        (:`Completed`
                          (set `self.NightTIme` false)
                          (`SceneComponent.SetHiddenInGame` _skyspheremesh_3 true false)
                          (`self.ResetNightDoOnce`)
                          (`ExponentialHeightFogComponent.SetFogDensity` _component_2 0.3)
                          (goto _label_15 :!via `Reverse`)))))))
              (else
                (set `self.AlmostNight?` false)
                (`|ExecutionSequence`
                  (:`then_0`
                    (goto _label_12))
                  (:`then_1`
                    (`/Engine/EditorBlueprintResources/StandardMacros.DoOnce` false :!label _label_17
                      (:`Completed`
                        (`self.ToggleLights`)
                        (`self.RufftonPostProcessVolumeSetting`)
                        (`self.ResetRufftonNotAlmostNight`))))))))
          (:`NewEnumerator2`
            (`self.K2_AddActorLocalRotation` _sunref_3 _returnvalue false false)
            (if (> _returnvalue_pitch_4 -4.0)
              (set `self.AlmostNight?` true)
              (`|ExecutionSequence`
                (:`then_0`
                  (`/Engine/EditorBlueprintResources/StandardMacros.DoOnce` false :!label _label_18
                    (:`Completed`
                      (`self.ToggleLights`)
                      (`self.CoastaltonPostProcessVolumeSetting`)
                      (`self.CoastaltonAlmostNight`))))
                (:`then_1`
                  (if (> _returnvalue_pitch_4 2.0) :!label _label_19
                    (`/Engine/EditorBlueprintResources/StandardMacros.DoOnce` false :!label _label_20
                      (:`Completed`
                        (set `self.NightTIme` true)
                        (`SceneComponent.SetHiddenInGame` _skyspheremesh_2 false false)
                        (`PrimitiveComponent.SetMaterial` _skyspheremesh_2 0 "/Game/Art/Materials/Sky_Materials/MI_StaryNight.MI_StaryNight")
                        (`ExponentialHeightFogComponent.SetFogDensity` _component_3 0.1)
                        ;[0.1896 0.3782 1] Update the suns intensity (currently set up to deacrease the intesnity to 0.01 after 10 min)
                        (bind (_direction_3 _alpha_3) (`Timeline|Timeline_2` :!label _label_21)
                          (:`Update`
                            (`MeshComponent.SetScalarParameterValueOnMaterials` (`self.SkySphereMesh`) "Opacity" (`KismetMathLibrary.Lerp` 0.0 0.5 _alpha_3))
                            (`SkyLightComponent.SetIntensity` (`SkyLight.LightComponent` (`self.SkylightRef`)) (`KismetMathLibrary.Lerp` 1.0 0.1 _alpha_3))
                            (`LightComponent.SetIntensity` (`Light.LightComponent` (`self.SunRef`)) (`KismetMathLibrary.Lerp` 10.0 0.01 _alpha_3)))
                          (:`Finished`
                            (`self.ResetCoastaltonDay`)))))
                    (else
                      (`/Engine/EditorBlueprintResources/StandardMacros.DoOnce` false :!label _label_22
                        (:`Completed`
                          (set `self.NightTIme` false)
                          (`SceneComponent.SetHiddenInGame` _skyspheremesh_2 true false)
                          (`self.ResetCoastaltonNight`)
                          (`ExponentialHeightFogComponent.SetFogDensity` _component_3 0.3) ; .3 is default
                          (goto _label_21 :!via `Reverse`)))))))
              (else
                (set `self.AlmostNight?` false)
                (`|ExecutionSequence`
                  (:`then_0`
                    (goto _label_19))
                  (:`then_1`
                    (`/Engine/EditorBlueprintResources/StandardMacros.DoOnce` false :!label _label_23
                      (:`Completed`
                        (`self.ToggleLights`)
                        (`self.CoastaltonPostProcessVolumeSetting`)
                        (`self.CoastaltonAlmostDay`))))))))
          (:`NewEnumerator3`
            ;[0.5021 0.69 1] Winterton Custon Day/Night Cycle
            (`self.K2_AddActorLocalRotation` _sunref_2 _returnvalue false false)
            (if (> _returnvalue_pitch_2 -4.0)
              (set `self.AlmostNight?` true)
              (`|ExecutionSequence`
                (:`then_0`
                  (`/Engine/EditorBlueprintResources/StandardMacros.DoOnce` false :!label _label_24
                    (:`Completed`
                      (`self.ToggleLights`)
                      (`self.WintertonPostProcessVolumeSetting`)
                      (`self.WintertonAlmostNight`))))
                (:`then_1`
                  (if (> _returnvalue_pitch_2 2.0) :!label _label_25
                    (`/Engine/EditorBlueprintResources/StandardMacros.DoOnce` false :!label _label_26
                      (:`Completed`
                        (set `self.NightTIme` true)
                        (`SceneComponent.SetHiddenInGame` _skyspheremesh_4 false false)
                        (`PrimitiveComponent.SetMaterial` _skyspheremesh_4 0 "/Game/Art/Materials/Sky_Materials/MI_StaryNight.MI_StaryNight")
                        (`|ExecutionSequence`
                          (:`then_0`
                            (goto _label_14))
                          (:`then_1`
                            (`ExponentialHeightFogComponent.SetFogDensity` _component_4 0.1)
                            ;;[0.1896 0.3782 1] Update the suns intensity (currently set up to deacrease the intesnity to 0.01 after 10 min)
                            (bind (_direction_4 _alpha_4) (`Timeline|Timeline_1` :!label _label_27)
                              (:`Update`
                                (`MeshComponent.SetScalarParameterValueOnMaterials` (`self.SkySphereMesh`) "Opacity" (`KismetMathLibrary.Lerp` 0.0 0.5 _alpha_4))
                                (`SkyLightComponent.SetIntensity` (`SkyLight.LightComponent` (`self.SkylightRef`)) (`KismetMathLibrary.Lerp` 0.8 0.1 _alpha_4))
                                (`LightComponent.SetIntensity` (`Light.LightComponent` (`self.SunRef`)) (`KismetMathLibrary.Lerp` 10.0 0.01 _alpha_4)))
                              (:`Finished`
                                (`self.ResetWintertonDay`)))))))
                    (else
                      (`/Engine/EditorBlueprintResources/StandardMacros.DoOnce` false :!label _label_28
                        (:`Completed`
                          (set `self.NightTIme` false)
                          (`SceneComponent.SetHiddenInGame` _skyspheremesh_4 true false)
                          (`self.ResetWintertonNight`)
                          (`ExponentialHeightFogComponent.SetFogDensity` _component_4 0.3) ; .3 is default
                          (goto _label_27 :!via `Reverse`)))))))
              (else
                (set `self.AlmostNight?` false)
                (`|ExecutionSequence`
                  (:`then_0`
                    (goto _label_25))
                  (:`then_1`
                    (`/Engine/EditorBlueprintResources/StandardMacros.DoOnce` false :!label _label_29
                      (:`Completed`
                        (`self.ToggleLights`)
                        (`self.WintertonPostProcessVolumeSetting`)
                        (`self.WintertonAlmostDay`))))))))
          (:`NewEnumerator4`
            (goto _label_10)))
        (elif (`self.QuestStarted`)
          (goto _label_3))))))

(event `ResetNightDoOnce`
  ;[0.01649 0 1] Ruffton Custom Day/Night Cycle
  ;;[0.125 0.125 0.125] Day/Night Transition
  (goto _label_13 :!via `Reset`))

(event `ResetDayDoOnce`
  ;[0.01649 0 1] Ruffton Custom Day/Night Cycle
  ;;[0.125 0.125 0.125] Day/Night Transition
  (goto _label_16 :!via `Reset`))

(event `ResetRufftonAlmostNight`
  ;[0.01649 0 1] Ruffton Custom Day/Night Cycle
  (goto _label_17 :!via `Reset`))

(event `WintertonAlmostNight`
  ;[0.5021 0.69 1] Winterton Custon Day/Night Cycle
  (goto _label_24 :!via `Reset`))

(event `ResetWintertonNight`
  ;[0.5021 0.69 1] Winterton Custon Day/Night Cycle
  (goto _label_26 :!via `Reset`))

(event `ResetWintertonDay`
  ;[0.5021 0.69 1] Winterton Custon Day/Night Cycle
  (goto _label_28 :!via `Reset`))

(event `WintertonAlmostDay`
  ;[0.5021 0.69 1] Winterton Custon Day/Night Cycle
  (goto _label_29 :!via `Reset`))

(event `CoastaltonAlmostNight`
  (goto _label_18 :!via `Reset`))

(event `ResetCoastaltonNight`
  (goto _label_20 :!via `Reset`))

(event `ResetCoastaltonDay`
  (goto _label_22 :!via `Reset`))

(event `CoastaltonAlmostDay`
  (goto _label_23 :!via `Reset`))

(fn `CastletonPostProcessVolumeSetting`
  (if (`self.AlmostNight?`)
    (bind _postprocessvolume (`self.PostProcessVolume`) ; Night Setting
      (:`then`
        (set `PostProcessVolume.Settings` (`self.CastletonNightSetting`) _postprocessvolume))
      (:`else`))
    (else
      (bind _postprocessvolume_2 (`self.PostProcessVolume`) ; Day Setting
        (:`then`
          (set `PostProcessVolume.Settings` (`self.CastletonDaySetting`) _postprocessvolume_2))
        (:`else`)))))

(fn `CoastaltonPostProcessVolumeSetting`
  (if (`self.AlmostNight?`)
    (bind _postprocessvolume (`self.PostProcessVolume`) ; Night Setting
      (:`then`
        (set `PostProcessVolume.Settings` (`self.CoastaltonNightSetting`) _postprocessvolume))
      (:`else`))
    (else
      (bind _postprocessvolume_2 (`self.PostProcessVolume`) ; Day Setting
        (:`then`
          (set `PostProcessVolume.Settings` (`self.CoastaltonDaySetting`) _postprocessvolume_2))
        (:`else`)))))

(fn `RefreshMaterial`
  (`parent.RefreshMaterial`))

(fn `RufftonPostProcessVolumeSetting`
  (if (`self.AlmostNight?`)
    (bind _postprocessvolume (`self.PostProcessVolume`) ; Night Setting
      (:`then`
        (set `PostProcessVolume.Settings` (`self.RufftonNightSetting`) _postprocessvolume))
      (:`else`))
    (else
      (bind _postprocessvolume_2 (`self.PostProcessVolume`) ; Day Setting
        (:`then`
          (set `PostProcessVolume.Settings` (`self.RufftonDaySetting`) _postprocessvolume_2))
        (:`else`)))))

(fn `SetCurrentLevel`
  ;[1 0.5573 0.937] What is the current level?
  (bind _returnvalue (`GameplayStatics.GetCurrentLevelName` true))
  (`|ExecutionSequence`
    (:`then_0`
      (bind _returnvalue_2 (`KismetStringLibrary.Conv_StringToName` _returnvalue))
      (if (== _returnvalue_2 "LVL_YeOleCastleton")
        (set `self.CurrentLevel` "NewEnumerator0")))
    (:`then_1`
      (if (== _returnvalue_2 "LVL_YeOleRuffton")
        (set `self.CurrentLevel` "NewEnumerator1")))
    (:`then_2`
      (if (== _returnvalue_2 "LVL_YeOleCoastalton")
        (set `self.CurrentLevel` "NewEnumerator2")))
    (:`then_3`
      (if (== _returnvalue_2 "LVL_YeOleWinterton")
        (set `self.CurrentLevel` "NewEnumerator3")))
    (:`then_4`
      (if (== _returnvalue_2 "LVL_YeOleDeserton")
        (set `self.CurrentLevel` "NewEnumerator4")))))

(fn `TimeSensitiveLevelCheck`
  (bind _returnvalue (`GameplayStatics.GetCurrentLevelName` true))
  (if (or (== (`KismetStringLibrary.Conv_StringToName` _returnvalue) "LVL_YeOleDeserton") (== (`KismetStringLibrary.Conv_StringToName` _returnvalue) "LVL_YeOleWinterton"))
    (set `self.LvlHasTimeSensitiveQuest` true)
    (else
      (set `self.LvlHasTimeSensitiveQuest` false))))

(fn `ToggleLights`
  (for _array_element (`self.Lanterns`)
    (if (not (`self.ActorHasTag` _array_element "StayLit"))
      (if (`self.AlmostNight?`)
        (bind _lit_ (`/Game/LevelObjects/BP_Lantern.Lit?` _array_element))
        (if (not _lit_)
          (`/Game/LevelObjects/BP_Lantern.ToggleLanterns` _array_element :!label _label))
        (elif _lit_
          (goto _label)))))
  (for _array_element_2 (`self.Torches`)
    (if (not (`self.ActorHasTag` _array_element_2 "StayLit"))
      (if (`self.AlmostNight?`)
        (bind _lit__2 (`/Game/LevelObjects/BP_WallTorch.Lit?` _array_element_2))
        (if (not _lit__2)
          (`/Game/LevelObjects/BP_WallTorch.ToggleTorches` _array_element_2 :!label _label_2))
        (elif _lit__2
          (goto _label_2))))))

(fn `UserConstructionScript`)

(fn `WintertonPostProcessVolumeSetting`
  (if (`self.AlmostNight?`)
    (bind _postprocessvolume (`self.PostProcessVolume`) ; Night Setting
      (:`then`
        (set `PostProcessVolume.Settings` (`self.WIntetonNightSetting`) _postprocessvolume))
      (:`else`))
    (else
      (bind _postprocessvolume_2 (`self.PostProcessVolume`) ; Day Setting
        (:`then`
          (set `PostProcessVolume.Settings` (`self.WintertonDaySetting`) _postprocessvolume_2))
        (:`else`)))))