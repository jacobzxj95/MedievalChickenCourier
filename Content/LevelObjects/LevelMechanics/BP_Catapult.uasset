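; Player-possessable catapult that launches carried chickens, usable once a quest starts.
; Successive interactions pull the arm back, load the chicken, then possess the catapult and enable delivery-volume collision, with a one-time tutorial popup.
; Move input rotates it within pitch limits, re-predicting the projectile path to respawn an aim marker.
; Firing swings the arm, throws the chicken and repossesses the player, while loading and launching also update thief AI.
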(event `self.ReceiveBeginPlay`
  (bind _returnvalue (`|CreateWidget` "/Game/UI/Dialogue/W_GoldenChickenSpawning.W_GoldenChickenSpawning_C"))
  (set `self.GoldenChickenSpawningWidget_ref` _returnvalue)
  (bind _returnvalue_2 (`|CreateWidget` "/Game/UI/W_TutorialBase.W_TutorialBase_C" (`GameplayStatics.GetPlayerController` 0)))
  (set `self.TutorialUI` _returnvalue_2)
  ;[0.194 0.1925 0.9479] Allow the player reference to become valid in the game mode then set it here.
  (`KismetSystemLibrary.Delay` 2.0)
  (bind _playercharacterref (message `/Game/Utility/Interfaces/BPI_UI.Pass Out Playercharacter ref` (`GameplayStatics.GetGameMode`)))
  (bind _output_get (set `self.GM_PlayerRef` _playercharacterref))
  (add `/Game/Components/ActorComponents/AC_Questlog.Quest Started` (`/Game/Characters/BP_PlayerChar.AC_QuestTurnIn` _output_get) (delegate `EnableUse`)))

(event `EnableUse`
  (params (ActiveQuest :type "/Game/RodgerL/BP_QuestManager Object Reference"))
  (set `self.QuestStarted?` true))

(event `EnhancedInput|/Game/ThirdPerson/Input/Actions/IA_Move`
  (params (ActionValue :type "Vector2D Structure") (ElapsedSeconds :type "Float (double-precision)") (TriggeredSeconds :type "Float (double-precision)") (InputAction :type "InputAction Object Reference" :default "/Game/ThirdPerson/Input/Actions/IA_Move.IA_Move"))
  (bind _returnvalue_roll (`KismetMathLibrary.BreakRotator` (`self.K2_GetActorRotation`)))
  (bind (_relativerotation_roll _relativerotation_pitch) (`KismetMathLibrary.BreakRotator` (`SceneComponent.RelativeRotation` (`self.DefaultSceneRoot`))))
  ;[0 1 0.1214] Inputs
  (:`Triggered`
    (`SceneComponent.K2_AddWorldRotation` (`self.DefaultSceneRoot`) (`KismetMathLibrary.MakeRotator` 0.0 0.0 ActionValue_X) false false)
    (if (<= _returnvalue_roll -40.0)
      (if (not (== ActionValue_Y 1.0))
        (`AudioComponent.Stop` (`self.CatapultMovementSound`))
        (else
          (`|ExecutionSequence` :!label _label
            (:`then_0`
              (if (<= _relativerotation_pitch -20.0)
                (if (< ActionValue_Y 0.0)
                  (`SceneComponent.K2_AddRelativeRotation` (`self.DefaultSceneRoot`) (`KismetMathLibrary.MakeRotator` 0.0 (* ActionValue_Y -1.0)) false false :!label _label_2)
                  (`self.PredictProjectilePath` false))
                (elif (>= _relativerotation_pitch 20.0)
                  (if (> ActionValue_Y 0.0)
                    (goto _label_2))
                  (else
                    (goto _label_2)))))
            (:`then_1`
              (`/Engine/EditorBlueprintResources/StandardMacros.DoOnce` false :!label _label_3
                (:`Completed`
                  (`AudioComponent.Play` (`self.CatapultMovementSound`) 0.0)))))))
      (elif (>= _returnvalue_roll 25.0)
        (if (== ActionValue_Y -1.0)
          (goto _label)
          (else
            (`AudioComponent.Stop` (`self.CatapultMovementSound`))))
        (else
          (goto _label)))))
  (:`Canceled`
    (`AudioComponent.Stop` (`self.CatapultMovementSound`) :!label _label_4)
    (`self.ResetMovementDoOnce`))
  (:`Completed`
    (`self.PredictProjectilePath` false)
    (goto _label_4)))

(event `ResetMovementDoOnce`
  ;[0 1 0.1214] Inputs
  (goto _label_3 :!via `Reset`))

(event `Key|E`
  (params (Key :type "Key Structure"))
  (bind _defaultsceneroot (`self.DefaultSceneRoot`))
  (bind (_returnvalue_roll _returnvalue_pitch _returnvalue_yaw) (`KismetMathLibrary.BreakRotator` (`SceneComponent.K2_GetComponentRotation` _defaultsceneroot)))
  ;[0 1 0.1214] Inputs
  (:`Pressed`
    (if (and (!= (`GameplayStatics.GetObjectClass` (`self.Held Object`)) null) (not (`self.InMotion?`)) (`self.ReadyToFire`))
      (`self.LaunchChicken`)
      (`KismetSystemLibrary.Delay` 2.0)
      (message `/Game/Utility/Interfaces/BPI_UI.TurnOffUI` (`GameplayStatics.GetGameMode`) "NewEnumerator20")
      (`self.RepossessPlayer`)
      (`SceneComponent.K2_SetRelativeRotation` _defaultsceneroot (`KismetMathLibrary.MakeRotator` _returnvalue_roll 0.0 _returnvalue_yaw) false false :!label _label_5))))

(event `Key|Q`
  (params (Key :type "Key Structure"))
  ;[0 1 0.1214] Inputs
  (:`Pressed`
    (message `/Game/Utility/Interfaces/BPI_UI.TurnOffUI` (`GameplayStatics.GetGameMode`) "NewEnumerator20")
    (`self.RepossessPlayer`)
    (goto _label_5)))

(event `Key|Escape`
  (params (Key :type "Key Structure"))
  ;[0 1 0.1214] Inputs
  (:`Pressed`
    (message `/Game/Utility/Interfaces/BPI_UI.TurnOffUI` (`GameplayStatics.GetGameMode`) "NewEnumerator20")
    (`self.RepossessPlayer`)))

(event `/Game/Utility/Interfaces/BPI_Interaction.InteractionStarted`
  (params (PlayerCharacter :type "/Game/Characters/BP_PlayerChar Object Reference") (HeldObject :type "Actor Object Reference"))
  (bind _returnvalue (`GameplayStatics.GetPlayerController` 0))
  (bind _arm (`self.Arm`))
  (bind _output_get (set `self.PlayerCharacter` PlayerCharacter))
  (if (and (not (`self.InMotion?`)) (`self.QuestStarted?`))
    (`self.CatapultTutorial`)
    (if (`self.PulledBack`)
      (if (`self.ReadyToFire`)
        (`self.SetActorHiddenInGame` _output_get true)
        (for _array_element (`self.DeliveryVolumes`)
          (`/Engine/EditorBlueprintResources/StandardMacros.IsValid` _array_element
            (:`Is Valid`
              (`/Game/Components/ActorComponents/AC_QuestTurnin.CheckTurninAllowance` (`/Game/LevelObjects/QuestRelated/BP_DeliveryVolume.AC_QuestTurnin` _array_element))
              (bind _box (`/Game/LevelObjects/QuestRelated/BP_DeliveryVolume.Box` _array_element))
              (`/Engine/EditorBlueprintResources/StandardMacros.IsValid` _box
                (:`Is Valid`
                  (`PrimitiveComponent.SetCollisionEnabled` _box "QueryOnly"))))))
        (`Controller.UnPossess` _returnvalue)
        (`Controller.Possess` _returnvalue self)
        (message `/Game/Utility/Interfaces/BPI_UI.TurnOnUI` (`GameplayStatics.GetGameMode`) "NewEnumerator20")
        (`self.PredictProjectilePath` true)
        (elif (== (`GameplayStatics.GetObjectClass` HeldObject) "/Game/AI/AICharacters/BP_AI_Chicken.BP_AI_Chicken_C")
          (`/Engine/EditorBlueprintResources/StandardMacros.IsValid` HeldObject
            (:`Is Valid`
              (bind _output_get_2 (set `self.Held Object` HeldObject))
              (`self.Player has chicken BB`
                (:`Is Valid?`
                  (`self.K2_AttachToComponent` _output_get_2 (`self.Arm`) "ChickenSlot" "KeepRelative" "KeepRelative" "KeepRelative" true)
                  (`GameplayStatics.PlaySoundAtLocation` "/Game/SFX/Mechanics/Throw_Hit_Drop/SC_PlaceDownObject.SC_PlaceDownObject" (`self.K2_GetActorLocation` (`self.Held Object`)) (struct) 1.0 1.0 0.0 null null null null)
                  (set `self.ReadyToFire` true)
                  (bind _gm_playerref (`self.GM_PlayerRef`)
                    (:`then`
                      (set `/Game/Characters/BP_ActiveChar.Is Holding?` false _gm_playerref)
                      (set `/Game/Characters/BP_ActiveChar.Current Item` null _gm_playerref))
                    (:`else`))))))))
      (else
        (`/Engine/EditorBlueprintResources/StandardMacros.DoOnce` false :!label _label_6
          (:`Completed`
            (set `self.InMotion?` true)
            (`GameplayStatics.PlaySoundAtLocation` "/Game/SFX/Mechanics/Catapult/SC_SettingCatyArm.SC_SettingCatyArm" (`self.K2_GetActorLocation`) (struct) 1.0 1.0 0.0 null null null null)
            (`KismetSystemLibrary.MoveComponentTo` _arm (`SceneComponent.RelativeLocation` _arm) (struct) true true 1.0)
            (`PhysicsConstraintComponent.SetAngularOrientationTarget` (`self.Spring`) (`KismetMathLibrary.MakeRotator` 0.0))
            (set `self.InMotion?` false)
            (set `self.PulledBack` true)))))))

(event `PredictProjectilePath`
  (params (`FirstTime?` :type Boolean))
  (bind _launchsite (`self.LaunchSite`))
  ;[1 1 1] Predict Projectile Path
  (if (not `FirstTime?`)
    (`self.K2_DestroyActor` (`self.AimActor`)))
  (bind _outhit (`GameplayStatics.Blueprint_PredictProjectilePath_ByTraceChannel` (`SceneComponent.K2_GetComponentLocation` _launchsite) (* (`SceneComponent.GetForwardVector` _launchsite) (`self.Throwing Force`)) true 5.0 "ECC_Visibility" false (`|MakeArray` self (`self.Held Object`) :!type "Actor Object Reference") "None" 5.0))
  (bind _returnvalue (`|SpawnActorFromClass` "/Game/LevelObjects/BP_AimTarget.BP_AimTarget_C" (`KismetMathLibrary.MakeTransform` (`.Location` (`GameplayStatics.BreakHitResult` _outhit)) (struct :`Pitch` 90.0) (1.5 1.5 1.5)) "Undefined" "OverrideRootScale" null null))
  (set `self.AimActor` _returnvalue))

(event `DoOnce_LoadCaty`
  (goto _label_6 :!via `Reset`))

(event `LaunchChicken`
  (bind _arm (`self.Arm`))
  (bind _arm_2 (`self.Arm`))
  ;[0.349 0 0.2657] Launch
  (`/Engine/EditorBlueprintResources/StandardMacros.DoOnce` false :!label _label_7
    (:`Completed`
      (set `self.ReadyToFire` false)
      (set `self.InMotion?` true)
      (`GameplayStatics.PlaySoundAtLocation` "/Game/SFX/Mechanics/Catapult/SC_CatapultLaunch.SC_CatapultLaunch" (`self.K2_GetActorLocation`) (struct) 1.0 1.0 0.0 null null null null)
      (`KismetSystemLibrary.MoveComponentTo` _arm (`SceneComponent.RelativeLocation` _arm) (struct :`Pitch` -90.0) false true (`self.ArmSwingDuration`))
      (set `self.CubeForwardVector` (`SceneComponent.GetForwardVector` (`self.Cube`)))
      (bind _held_object (`self.Held Object`)
        (:`then`
          (`self.K2_DetachFromActor` _held_object "KeepWorld" "KeepWorld" "KeepWorld")
          (message `/Game/Utility/Interfaces/BPI_EPS.ItemThrown` _held_object (`self.Throwing Force`) (`self.CubeForwardVector`) (`KismetMathLibrary.MakeTransform` (`SceneComponent.K2_GetComponentLocation` (`self.Cube`))) true 0.0)
          (bind _outactors (`GameplayStatics.GetAllActorsOfClass` "/Game/Characters/BP_Thief.BP_Thief_C"))
          (message `/Game/AI/BPI/BPI_Villager_Switch_States.Thief_Becomes_Villager` _outactors)
          (`/Game/Characters/BP_Thief.Reset return behavior` _outactors)
          (`KismetSystemLibrary.MoveComponentTo` _arm_2 (`SceneComponent.RelativeLocation` _arm_2) (`self.ArmStartingRotation`) false true (`self.ArmDownDuration`))
          (`KismetSystemLibrary.Delay` 0.2)
          (set `self.InMotion?` false)
          (set `self.PulledBack` false)
          (`self.DoOnce_LoadCaty`)
          (`self.ResetLaunchDoOnce`))
        (:`else`
          (`KismetSystemLibrary.PrintString` "Catapult: HELD OBJECT INVALID" true true (struct :`R` 1.0 :`B` 0.016322 :`A` 1.0) 7.0))))))

(event `ResetLaunchDoOnce`
  ;[0.349 0 0.2657] Launch
  (goto _label_7 :!via `Reset`))

(event `self.Base.OnComponentBeginOverlap`
  (params (OverlappedComponent :type "PrimitiveComponent Object Reference") (OtherActor :type "Actor Object Reference") (OtherComp :type "PrimitiveComponent Object Reference") (OtherBodyIndex :type Integer) (bFromSweep :type Boolean) (SweepResult :type "HitResult Structure (by ref)")))

(event `self. Box.OnComponentBeginOverlap`
  (params (OverlappedComponent :type "PrimitiveComponent Object Reference") (OtherActor :type "Actor Object Reference") (OtherComp :type "PrimitiveComponent Object Reference") (OtherBodyIndex :type Integer) (bFromSweep :type Boolean) (SweepResult :type "HitResult Structure (by ref)"))
  (bind _asbp_thief (cast `/Game/Characters/BP_Thief` OtherActor))
  (if (== (`self.Held Object`) "/Game/AI/AICharacters/BP_AI_Chicken.BP_AI_Chicken")
    (message `/Game/AI/BPI/BPI_Villager_Switch_States.Thief_Becomes_Villager` _asbp_thief)))

(fn `CatapultTutorial`
  (bind _game_instance (message `/Game/Utility/Interfaces/BPI_UI.Pass Out Game Instance Ref` (`GameplayStatics.GetGameMode`)))
  (if (not (`BlueprintMapLibrary.Map_Find` (`/Game/Utility/GameModes/BP_GameInstance.ShownTutorials` _game_instance) "NewEnumerator2"))
    (bind _tutorialui (`self.TutorialUI`)
      (:`then`
        (set `/Game/UI/W_TutorialBase.E_Mechanics` "NewEnumerator2" _tutorialui)
        (`UserWidget.AddToViewport` _tutorialui 0)
        (`/Game/Utility/GameModes/BP_GameInstance.SaveTutorialPopups` _game_instance (enumliteral `/Game/Utility/Enums/E_Mechanics` "NewEnumerator2") true))
      (:`else`)))
  (return))

(fn `QuestInteraction`
  (returns (ObjectiveID :type String))
  (return ""))

(fn `RepossessPlayer`
  (bind _returnvalue (`GameplayStatics.GetPlayerController` 0))
  (bind _goldenchickenspawningwidget_ref (`self.GoldenChickenSpawningWidget_ref`)
    (:`then`
      (if (`Widget.IsInViewport` _goldenchickenspawningwidget_ref)
        (bind _playercharacter (`self.PlayerCharacter`)
          (:`then`
            (`self.SetActorHiddenInGame` _playercharacter false)
            (bind _aimactor (`self.AimActor`)
              (:`then`
                (`self.K2_DestroyActor` _aimactor)
                (message `/Game/Utility/Interfaces/BPI_UI.TurnOffUI` (`GameplayStatics.GetGameMode`) "NewEnumerator20")
                (bind _outactors (`GameplayStatics.GetAllActorsOfClass` "/Game/Characters/BP_Thief.BP_Thief_C"))
                (message `/Game/AI/BPI/BPI_Villager_Switch_States.Thief_Becomes_Villager` _outactors)
                (`/Game/Characters/BP_Thief.Reset return behavior` _outactors))
              (:`else`)))
          (:`else`))
        (else
          (bind _playercharacter_2 (`self.PlayerCharacter`)
            (:`then`
              (`self.SetActorHiddenInGame` _playercharacter_2 false)
              (`Controller.UnPossess` _returnvalue)
              (`Controller.Possess` _returnvalue _playercharacter_2)
              (bind _aimactor_2 (`self.AimActor`)
                (:`then`
                  (`self.K2_DestroyActor` _aimactor_2)
                  (message `/Game/Utility/Interfaces/BPI_UI.TurnOffUI` (`GameplayStatics.GetGameMode`) "NewEnumerator20")
                  (bind _outactors_2 (`GameplayStatics.GetAllActorsOfClass` "/Game/Characters/BP_Thief.BP_Thief_C"))
                  (message `/Game/AI/BPI/BPI_Villager_Switch_States.Thief_Becomes_Villager` _outactors_2)
                  (`/Game/Characters/BP_Thief.Reset return behavior` _outactors_2))
                (:`else`)))
            (:`else`)))))
    (:`else`)))

(fn `UserConstructionScript`)