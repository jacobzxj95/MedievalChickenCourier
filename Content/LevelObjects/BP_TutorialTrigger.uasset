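; Tutorial trigger actor that shows in-world help text when the player walks into its volume.
; The construction script fills three text components from display-text variables.
; On the first overlap by player pawn 0, it unhides Text and its children, then hides them again after a fixed delay.
; A DoOnce limits this to one showing, as its reset event is left disconnected.
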(event `self.TriggerVolume.OnComponentBeginOverlap`
  (params (OverlappedComponent :type "PrimitiveComponent Object Reference") (OtherActor :type "Actor Object Reference") (OtherComp :type "PrimitiveComponent Object Reference") (OtherBodyIndex :type Integer) (bFromSweep :type Boolean) (SweepResult :type "HitResult Structure (by ref)"))
  ;[0.5506 0 1] Display the input text on overlap and remove it after a set delay (Repeatable if the reset Do Once pins are reconnected).
  (if (== OtherActor (`GameplayStatics.GetPlayerPawn` 0))
    (`/Engine/EditorBlueprintResources/StandardMacros.DoOnce` false
      (:`Completed`
        (`SceneComponent.SetHiddenInGame` (`self.Text`) false true)
        (`KismetSystemLibrary.Delay` 10.0)
        (`SceneComponent.SetHiddenInGame` (`self.Text`) true true)))))

(event `ResetDoOnce`
  ;[0.5506 0 1] Display the input text on overlap and remove it after a set delay (Repeatable if the reset Do Once pins are reconnected).
)

(fn `UserConstructionScript`
  (`TextRenderComponent.K2_SetText` (`self.Text`) (`self.DisplayText`))
  (`TextRenderComponent.K2_SetText` (`self.Text1`) (`self.DisplayText2`))
  (`TextRenderComponent.K2_SetText` (`self.Text2`) (`self.DisplayText3`)))