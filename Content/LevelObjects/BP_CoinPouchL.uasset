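; BP_CoinPouchL is a coin pouch level object that animates vertically and removes itself when found in loaded game data.
; On BeginPlay it binds to GM_MVP's Loaded event, destroying itself if its display name is a key in the received actor map.
; Tick plays a timeline that lerps actor Z around the CoinPurse component's current height.
; Both overlap events are empty, so no pickup logic exists here.
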(event `self.ReceiveBeginPlay`
  (bind _asgm_mvp (cast `/Game/Maps/GameModes/GM_MVP` (`GameplayStatics.GetGameMode`)))
  (add `/Game/Maps/GameModes/GM_MVP.Loaded` _asgm_mvp (delegate `Loaded`)))

(event `Loaded`
  (params (`Actor Map` :type "Map of String to Boolean"))
  (bind _keys (`BlueprintMapLibrary.Map_Keys` `Actor Map`))
  (for _array_element _keys
    (if (`KismetStringLibrary.EqualEqual_StrStr` _array_element (`KismetSystemLibrary.GetDisplayName` self))
      (`self.K2_DestroyActor`))))

(event `self.ReceiveTick`
  (params (DeltaSeconds :type "Float (single-precision)"))
  (bind (_returnvalue_x _returnvalue_y _returnvalue_z) (`KismetMathLibrary.BreakVector` (`SceneComponent.K2_GetComponentLocation` (`self.CoinPurse`))))
  (bind (_direction _float_track) (`Timeline|Timeline`)
    (:`Update`
      (`self.K2_SetActorRelativeLocation` (`KismetMathLibrary.MakeVector` _returnvalue_x _returnvalue_y (`KismetMathLibrary.Lerp` (- _returnvalue_z 1.0) (+ _returnvalue_z 1.0) _float_track))))))

(event `self.Box.OnComponentBeginOverlap`
  (params (OverlappedComponent :type "PrimitiveComponent Object Reference") (OtherActor :type "Actor Object Reference") (OtherComp :type "PrimitiveComponent Object Reference") (OtherBodyIndex :type Integer) (bFromSweep :type Boolean) (SweepResult :type "HitResult Structure (by ref)")))

(fn `UserConstructionScript`)