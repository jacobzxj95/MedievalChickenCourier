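; BP_CourierWagon is a level object that serves as a quest turn-in point for items the player carries.
; When the player enters its Box, the ACQuestTurnin component checks the held item, and an accepted item is taken and snapped to the ChickenSpot socket, clearing a UI message.
; TurnonWaypoints shows or hides the waypoint widget and spotlight for objective IDs listed in that component.
; QuestInteraction returns an empty string.
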(event `self.ReceiveBeginPlay`)

(event `self.Box.OnComponentBeginOverlap`
  (params (OverlappedComponent :type "PrimitiveComponent Object Reference") (OtherActor :type "Actor Object Reference") (OtherComp :type "PrimitiveComponent Object Reference") (OtherBodyIndex :type Integer) (bFromSweep :type Boolean) (SweepResult :type "HitResult Structure (by ref)"))
  (bind _asbp_player_char (cast `/Game/Characters/BP_PlayerChar` OtherActor))
  (bind _isquestitem (`/Game/Components/ActorComponents/AC_QuestTurnin.Actor to Check` (`self.AC_QuestTurnin`) (`/Game/Characters/BP_ActiveChar.Current Item` _asbp_player_char)))
  (if _isquestitem
    (bind _tempcurrentitem1 (`/Game/Characters/BP_PlayerChar.GiveItem` _asbp_player_char))
    (`/Engine/EditorBlueprintResources/StandardMacros.IsValid` _tempcurrentitem1
      (:`Is Valid`
        (`self.K2_AttachToComponent` _tempcurrentitem1 (`self.StaticMesh`) "ChickenSpot" "SnapToTarget" "SnapToTarget" "KeepWorld" true)
        (message `/Game/Utility/Interfaces/BPI_UI.TurnOffUI` (`GameplayStatics.GetGameMode`) "NewEnumerator12")))))

(event `/Game/Utility/Interfaces/BPI_Quest.TurnOnWaypoints`
  (params (ObjectiveID :type String) (`On/Off` :type Boolean))
  (for _array_element (`/Game/Components/ActorComponents/AC_QuestTurnin.ObjectiveName` (`self.AC_QuestTurnin`))
    (if (`KismetStringLibrary.EqualEqual_StrStr` ObjectiveID _array_element)
      (if `On/Off`
        (`SceneComponent.SetHiddenInGame` (`self.Widget`) false false)
        (`SceneComponent.SetHiddenInGame` (`self.SpotLight`) false false)
        (else
          (`SceneComponent.SetHiddenInGame` (`self.Widget`) true false)
          (`SceneComponent.SetHiddenInGame` (`self.SpotLight`) true false))))))

(fn `QuestInteraction`
  (returns (ObjectiveID :type String))
  (return ""))

(fn `UserConstructionScript`)