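; BP_Movementsurface is a level surface that toggles between ledge-grab enabled and disabled states.
; On BeginPlay, IsEnabled selects the state through EnabledDisableLedgegrab, which swaps a transparent green or yellow material and inverts Surface's Block/Ignore responses on two custom trace channels.
; The HitbyGoop event is an empty stub, so goop hits do not change the state here.
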(event `self.ReceiveBeginPlay`
  (if (`self.IsEnabled?`)
    (`self.EnabledDisableLedgegrab` true)
    (else
      (`self.EnabledDisableLedgegrab` false))))

(event `/Game/Utility/Interfaces/BPI_Hit.HitByGoop`)

(fn `EnabledDisableLedgegrab`
  (params (`Enable?` :type Boolean))
  (if `Enable?`
    (`PrimitiveComponent.SetMaterial` (`self.Surface`) 0 "/Game/Art/Materials/MI_TransparentGreen.MI_TransparentGreen")
    (`PrimitiveComponent.SetCollisionResponseToChannel` (`self.Surface`) "ECC_GameTraceChannel2" "ECR_Ignore")
    (`PrimitiveComponent.SetCollisionResponseToChannel` (`self.Surface`) "ECC_GameTraceChannel3" "ECR_Block")
    (else
      (`PrimitiveComponent.SetMaterial` (`self.Surface`) 0 "/Game/Art/Materials/MI_TransparentYellow.MI_TransparentYellow")
      (`PrimitiveComponent.SetCollisionResponseToChannel` (`self.Surface`) "ECC_GameTraceChannel2" "ECR_Block")
      (`PrimitiveComponent.SetCollisionResponseToChannel` (`self.Surface`) "ECC_GameTraceChannel3" "ECR_Ignore"))))

(fn `UserConstructionScript`)