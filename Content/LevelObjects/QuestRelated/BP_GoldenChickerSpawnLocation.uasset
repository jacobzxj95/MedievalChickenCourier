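; Level actor that plays a golden chicken spawn cutscene with its own camera, spotlight, widget, angel sound and VFX.
; AnimateTheCock disables player input, hides a UI message and fades to the actor's view.
; A timeline brightens the spotlight while moving the given chicken from above the light to the actor's location, spinning it on a random axis and direction.
; A timer then fades back, restoring player view, input and UI.
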(event `self.ReceiveBeginPlay`
  (bind (_returnvalue_x _returnvalue_y _returnvalue_z) (`KismetMathLibrary.BreakVector` (`SceneComponent.K2_GetComponentLocation` (`self.SpotLight`))))
  (set `self.startingLocation` (`KismetMathLibrary.MakeVector` _returnvalue_x _returnvalue_y (+ _returnvalue_z 25.0)))
  (set `self.endingLocation` (`self.K2_GetActorLocation`))
  (`LightComponent.SetIntensity` (`self.SpotLight`) 0.0))

(event `Animate The Cock`
  (params (Actor :type "Actor Object Reference"))
  (bind _camera (`self.Camera`))
  (message `/Game/Utility/Interfaces/BPI_UI.TurnOffUI` (`GameplayStatics.GetGameMode`) "NewEnumerator0")
  (`AudioComponent.Play` (`self._Audio__Angel_-_Sound_Effect_HD`) 0.0)
  (bind _output_get (set `self.GivenChickenActor` Actor))
  (`self.K2_SetActorLocation` _output_get (0.0 0.0 0.0) false false)
  (bind _returnvalue (`|CreateWidget` "/Game/UI/Dialogue/W_GoldenChickenSpawning.W_GoldenChickenSpawning_C"))
  (bind _output_get_2 (set `self.GoldenChickenWidget` _returnvalue))
  (`UserWidget.AddToViewport` _returnvalue 0)
  (`UserWidget.AddToViewport` _output_get_2 0)
  (`self.DisableInput` (`GameplayStatics.GetPlayerCharacter` 0) (`GameplayStatics.GetPlayerController` 0))
  (`PlayerCameraManager.StartCameraFade` :`self` (`GameplayStatics.GetPlayerCameraManager` 0) :`ToAlpha` 1.0 :`Duration` 0.4 :`bShouldFadeAudio` true :`bHoldWhenFinished` true)
  (`KismetSystemLibrary.Delay` 0.6)
  (`PlayerController.SetViewTargetWithBlend` (`GameplayStatics.GetPlayerController` 0) self 0.0 "VTBlend_Linear" 0.0 false)
  (`PlayerCameraManager.StartCameraFade` :`self` (`GameplayStatics.GetPlayerCameraManager` 0) :`FromAlpha` 1.0 :`Duration` 4.0 :`bShouldFadeAudio` true)
  (`KismetSystemLibrary.Delay` 0.6)
  (`self.Pick Rotation`)
  (`self.K2_SetActorLocation` (`self.GivenChickenActor`) (`self.startingLocation`) false false)
  (`NiagaraFunctionLibrary.SpawnSystemAtLocation` "/Game/Art/VFX/VFX_ChickenSpawning.VFX_ChickenSpawning" (+ (* (`SceneComponent.GetForwardVector` _camera) 50.0) (`SceneComponent.K2_GetComponentLocation` _camera)) (struct) (1.0 1.0 1.0) false)
  (`TimelineComponent.SetPlayRate` (`self.MoveTheChicken`) 0.25)
  (bind (_direction _alpha) (`Timeline|MoveTheChicken` :!via `PlayFromStart`)
    (:`Update`
      (`LightComponent.SetIntensity` (`self.SpotLight`) (`KismetMathLibrary.Lerp` 0.0 100000.0 _alpha))
      (`self.K2_SetActorLocation` (`self.GivenChickenActor`) (`KismetMathLibrary.VLerp` (`self.startingLocation`) (`self.endingLocation`) _alpha) false false)
      (`self.K2_SetActorRotation` (`self.GivenChickenActor`) (`KismetMathLibrary.RLerp` (`self.startingRotation`) (`self.endingRotation`) _alpha) false))
    (:`Finished`
      (`KismetSystemLibrary.K2_SetTimer` null "Start Camera Fade Back To Player" 0.5))))

(event `Start Camera Fade Back To Player`
  (`Widget.RemoveFromParent` (`self.GoldenChickenWidget`))
  (`PlayerCameraManager.StartCameraFade` :`self` (`GameplayStatics.GetPlayerCameraManager` 0) :`ToAlpha` 1.0 :`Duration` 0.4 :`bShouldFadeAudio` true :`bHoldWhenFinished` true)
  (`KismetSystemLibrary.Delay` 0.5)
  (`self.Re-enablePlayerController`)
  (`PlayerCameraManager.StartCameraFade` :`self` (`GameplayStatics.GetPlayerCameraManager` 0) :`FromAlpha` 1.0 :`Duration` 0.4 :`bShouldFadeAudio` true)
  (`AudioComponent.Stop` (`self._Audio__Angel_-_Sound_Effect_HD`)))

(fn `Pick Rotation`
  (set `self.RotationAdditive` (* (`self.RotationAdditive`) (`KismetMathLibrary.SelectFloat` 1.0 -1.0 (`KismetMathLibrary.RandomBool`))))
  (switch `int` (`KismetMathLibrary.RandomIntegerInRange` 0 2)
    (:`0`
      (bind _output_get (set `self.startingRotation` (`self.K2_GetActorRotation` (`self.GivenChickenActor`))))
      (set `self.endingRotation` (`KismetMathLibrary.MakeRotator` (.roll _output_get) (.pitch _output_get) (+ (.yaw _output_get) (`self.RotationAdditive`)))))
    (:`1`
      (bind _output_get_2 (set `self.startingRotation` (`self.K2_GetActorRotation` (`self.GivenChickenActor`))))
      (set `self.endingRotation` (`KismetMathLibrary.MakeRotator` (.roll _output_get_2) (+ (.pitch _output_get_2) (`self.RotationAdditive`)) (.yaw _output_get_2))))
    (:`2`
      (bind _output_get_3 (set `self.startingRotation` (`self.K2_GetActorRotation` (`self.GivenChickenActor`))))
      (set `self.endingRotation` (`KismetMathLibrary.MakeRotator` (+ (.roll _output_get_3) (`self.RotationAdditive`)) (.pitch _output_get_3) (.yaw _output_get_3)))))
  (return))

(fn `Re-enablePlayerController`
  (`self.EnableInput` (`GameplayStatics.GetPlayerCharacter` 0) (`GameplayStatics.GetPlayerController` 0))
  (message `/Game/Utility/Interfaces/BPI_UI.TurnOnUI` (`GameplayStatics.GetGameMode`) "NewEnumerator0")
  (`PlayerController.SetViewTargetWithBlend` (`GameplayStatics.GetPlayerController` 0) (`GameplayStatics.GetPlayerCharacter` 0) 0.0 "VTBlend_Linear" 0.0 false))

(fn `UserConstructionScript`)