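; A quest delivery volume that accepts matching items, either carried by the player or overlapping it on their own.
; A quest turn-in component checks each item, then the volume stores it at a drop point or destroys it, spawns confetti and checks turn-in allowance.
; Objective waypoint events toggle the marker widget and whether the volume accepts deliveries.
; When turn-in finishes, it can disable its own collision and marker.
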(event `self.ReceiveBeginPlay`
  (bind _output_get (`/Game/Components/ActorComponents/AC_QuestTurnin.CreateWidget` (`self.AC_QuestTurnin`)))
  (`/Game/UI/Icons/W_MainObjectiveIcon.TurnOnObjectiveIcon` (`/Game/Components/ActorComponents/AC_QuestTurnin.TurninIcon` (`self.AC_QuestTurnin`)) 0)
  (`WidgetComponent.SetWidget` (`self.TurnInMarker`) _output_get)
  (add `/Game/Components/ActorComponents/AC_QuestTurnin.TurninFinished` (`self.AC_QuestTurnin`) (delegate `CustomEvent`)))

(event `CustomEvent`
  (if (`self.ShouldDestroySelf`)
    (`PrimitiveComponent.SetCollisionEnabled` (`self.Box`) "NoCollision")
    (`SceneComponent.SetHiddenInGame` (`self.TurnInMarker`) true false)
    (set `self.IsQuestEnabled` false)
    (`KismetSystemLibrary.PrintString` "delivery volume disabled" true true (struct :`R` 0.998667 :`G` 1.0 :`B` 0.976708 :`A` 1.0) 10.0)))

(event `/Game/Utility/Interfaces/BPI_Quest.TurnOnWaypoints`
  (params (ObjectiveID :type String) (`On/Off` :type Boolean))
  (bind _turninmarker (`self.TurnInMarker`))
  (for _array_element (`/Game/Components/ActorComponents/AC_QuestTurnin.ObjectiveName` (`self.AC_QuestTurnin`))
    (if (`KismetStringLibrary.EqualEqual_StrStr` ObjectiveID _array_element)
      (if `On/Off`
        (`SceneComponent.SetHiddenInGame` _turninmarker false false)
        (set `self.IsQuestEnabled` true)
        (else
          (`SceneComponent.SetHiddenInGame` _turninmarker true false)
          (set `self.IsQuestEnabled` false)
          (`KismetSystemLibrary.PrintString` "delivery volume disabled" true true (struct :`R` 0.998667 :`G` 1.0 :`B` 0.976708 :`A` 1.0) 10.0))))))

(event `self.Box.OnComponentBeginOverlap`
  (params (OverlappedComponent :type "PrimitiveComponent Object Reference") (OtherActor :type "Actor Object Reference") (OtherComp :type "PrimitiveComponent Object Reference") (OtherBodyIndex :type Integer) (bFromSweep :type Boolean) (SweepResult :type "HitResult Structure (by ref)"))
  (if (== (`GameplayStatics.GetObjectClass` OtherActor) "/Game/Characters/BP_PlayerChar.BP_PlayerChar_C")
    (if (`self.IsQuestEnabled`)
      (bind _asbp_player_char (cast `/Game/Characters/BP_PlayerChar` OtherActor))
      (bind _output_get (set `self.Player Character Ref` _asbp_player_char))
      (bind _current_item (`/Game/Characters/BP_ActiveChar.Current Item` _output_get)
        (:`then`
          (set `self.IsPlayerCharacter` true)
          (bind _isquestitem (`/Game/Components/ActorComponents/AC_QuestTurnin.Actor to Check` (`self.AC_QuestTurnin`) _current_item))
          (if (and _isquestitem (not (`self.ActorHasTag` _current_item "Delivered")))
            (`|ExecutionSequence`
              (:`then_0`
                (`KismetSystemLibrary.Delay` 0.2)
                (`/Game/Characters/BP_PlayerChar.ChickenTimer` (`self.Player Character Ref`)))
              (:`then_1`
                (if (`KismetSystemLibrary.DoesImplementInterface` (`self.OverlappedActor`) "/Game/AI/HoningChicken/BPI_Honing.BPI_Honing_C") :!label _label
                  (message `/Game/AI/HoningChicken/BPI_Honing.UnPosses` (`self.OverlappedActor`)))
                (switch `/Game/Utility/Enums/E_TurnInActions` (`/Game/Components/ActorComponents/AC_QuestTurnin.ReactionToTurnin` (`self.AC_QuestTurnin`))
                  (:`NewEnumerator0`
                    (if (`self.IsPlayerCharacter`)
                      (`self.Player Character Ref`
                        (:`then`
                          (`/Game/Components/ActorComponents/AC_QuestTurnin.MoveActorToLocation` (`self.AC_QuestTurnin`) (`SceneComponent.K2_GetComponentLocation` (`self.ChickenMoveToLocation`)) true))
                        (:`else`))
                      (else
                        (`/Game/Components/ActorComponents/AC_QuestTurnin.MoveActorToLocationFunction` (`self.AC_QuestTurnin`) (`self.OverlappedActor`) (`SceneComponent.K2_GetComponentLocation` (`self.ChickenMoveToLocation`)))
                        (if (`KismetSystemLibrary.DoesImplementInterface` (`self.OverlappedActor`) "/Game/AI/HoningChicken/BPI_Honing.BPI_Honing_C")
                          _
                          (else
                            _)))))
                  (:`NewEnumerator1`
                    (if (`self.IsPlayerCharacter`)
                      (bind _player_character_ref (`self.Player Character Ref`)
                        (:`then`
                          (bind _tempcurrentitem1 (`/Game/Characters/BP_ActiveChar.GiveItem` _player_character_ref))
                          (`self.K2_DestroyActor` _tempcurrentitem1))
                        (:`else`))
                      (else
                        (`self.K2_DestroyActor` (`self.OverlappedActor`))))))
                (`NiagaraFunctionLibrary.SpawnSystemAtLocation` "/Game/Art/VFX/VFX_Confetti.VFX_Confetti" (`SceneComponent.K2_GetComponentLocation` (`self.DefaultSceneRoot`)))
                (`/Game/Components/ActorComponents/AC_QuestTurnin.CheckTurninAllowance` (`self.AC_QuestTurnin`))))))
        (:`else`)))
    (elif (`self.IsQuestEnabled`)
      (bind _output_get_2 (set `self.OverlappedActor` OtherActor))
      (bind _isquestitem_2 (`/Game/Components/ActorComponents/AC_QuestTurnin.Actor to Check` (`self.AC_QuestTurnin`) _output_get_2))
      (if _isquestitem_2
        (set `self.IsPlayerCharacter` false)
        (goto _label)))))

(fn `UserConstructionScript`)