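; BP_MainObjectiveIcon is a main objective marker with a chicken icon and an inactive-quest icon, whose initial visibility comes from flags in the construction script.
; A volume hides the chicken icon while the player is inside and reveals it on exit, if IconVisible is set.
; A SetVisibility event toggles the chicken icon directly.
; BeginPlay caches all quest givers, which a QuestActive? macro scans for active quests.
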(event `self.ReceiveBeginPlay`
  (bind _outactors (`GameplayStatics.GetAllActorsOfClass` "/Game/Characters/BP_QuestGiver.BP_QuestGiver_C"))
  (set `self.QuestGivers` _outactors))

(event `SetVisibility`
  (params (`New Visibility` :type Boolean))
  (`SceneComponent.SetVisibility` (`self.ChickenIcon`) `New Visibility` false))

(event `self.Volume.OnComponentBeginOverlap`
  (params (OverlappedComponent :type "PrimitiveComponent Object Reference") (OtherActor :type "Actor Object Reference") (OtherComp :type "PrimitiveComponent Object Reference") (OtherBodyIndex :type Integer) (bFromSweep :type Boolean) (SweepResult :type "HitResult Structure (by ref)"))
  ;[0.7102 0.3209 1] Hide the icon when the player is close or at the objective location
  (if (and (== OtherActor (`GameplayStatics.GetPlayerPawn` 0)) (`self.IconVisible?`))
    (`SceneComponent.SetVisibility` (`self.ChickenIcon`) false false)))

(event `self.Volume.OnComponentEndOverlap`
  (params (OverlappedComponent :type "PrimitiveComponent Object Reference") (OtherActor :type "Actor Object Reference") (OtherComp :type "PrimitiveComponent Object Reference") (OtherBodyIndex :type Integer))
  ;[0.4828 1 0.5202] Reveal the icon when the player is away from the objective location
  (if (and (== (`GameplayStatics.GetPlayerPawn` 0) OtherActor) (`self.IconVisible?`))
    (`SceneComponent.SetVisibility` (`self.ChickenIcon`) true false)))

(fn `UserConstructionScript`
  ;[1 1 1] Hide the chicken icon initially
  (`SceneComponent.SetVisibility` (`self.ChickenIcon`) (`self.IconVisible?`) false)
  (`SceneComponent.SetVisibility` (`self.InactiveQuestIcon`) (`self.InactiveQuestIconVisible?`) false))