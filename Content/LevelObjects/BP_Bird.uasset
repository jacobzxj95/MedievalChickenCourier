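; BP_Bird is a level object that moves between two configurable points, with an arrow component re-aimed as it goes.
; The construction script feeds Location1 and Location2 to InterpToMovement as relative control points and applies Duration as its travel time.
; A looping timer of the same Duration flip-flops the Arrow's rotation between look-at values computed from its forward vector, using world rotation for Location1 and relative for Location2.
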(event `self.ReceiveBeginPlay`
  (`KismetSystemLibrary.K2_SetTimerDelegate` (delegate `SwitchPoints`) (`self.Duration`) true)
  (`SceneComponent.K2_SetRelativeRotation` (`self.Arrow`) (`KismetMathLibrary.FindLookAtRotation` (`SceneComponent.GetForwardVector` (`self.Arrow`)) (`self.Location 2`)) false false))

(event `SwitchPoints`
  (bind _arrow (`self.Arrow`))
  (`/Engine/EditorBlueprintResources/StandardMacros.FlipFlop`
    (:`A`
      (`SceneComponent.K2_SetWorldRotation` _arrow (`KismetMathLibrary.FindLookAtRotation` (`SceneComponent.GetForwardVector` _arrow) (`self.Location 1`)) false false))
    (:`B`
      (`SceneComponent.K2_SetRelativeRotation` _arrow (`KismetMathLibrary.FindLookAtRotation` (`SceneComponent.GetForwardVector` _arrow) (`self.Location 2`)) false false))))

(event `self.ReceiveTick`
  (params (DeltaSeconds :type "Float (single-precision)")))

(event `self.InterpToMovement.OnInterpToStop`
  (params (ImpactResult :type "HitResult Structure (by ref)") (Time :type "Float (single-precision)")))

(fn `UserConstructionScript`
  (bind _interptomovement (`self.InterpToMovement`))
  (set `InterpToMovementComponent.ControlPoints` (`|MakeArray` (make `InterpControlPoint` (`self.Location 1`)) (make `InterpControlPoint` (`self.Location 2`))) _interptomovement)
  (set `InterpToMovementComponent.Duration` (`self.Duration`) _interptomovement))