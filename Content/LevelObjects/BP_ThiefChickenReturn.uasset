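; BP_ThiefChickenReturn is a drop-off point where a thief turns in a carried chicken.
; An overlap on its DropOff component takes the held item from any non-player BP_ActiveChar, destroys it and plays a voice clip.
; If that character is a BP_Thief, it is notified of the return and every BP_QuestManager receives a "SUB" quest update.
; HasGoldenChicken and PickupChicken are empty stubs.
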(event `self.DropOff.OnComponentBeginOverlap`
  (params (OverlappedComponent :type "PrimitiveComponent Object Reference") (OtherActor :type "Actor Object Reference") (OtherComp :type "PrimitiveComponent Object Reference") (OtherBodyIndex :type Integer) (bFromSweep :type Boolean) (SweepResult :type "HitResult Structure (by ref)"))
  (`self.Turned In Actor` OtherActor))

(fn `HasGoldenChicken`
  (return))

(fn `PickupChicken`
  (returns (`Currently being held` :type Boolean))
  (return false))

(fn `Turned In Actor`
  (params (`Overlapped actor` :type "Object Object Reference"))
  (locals (`Overlapped Object` :type "Object Object Reference"))
  (bind _output_get (set `local.Overlapped Object` `Overlapped actor`))
  (bind _asbp_active_char (cast `/Game/Characters/BP_ActiveChar` _output_get))
  (if (!= (`local.Overlapped Object`) (`GameplayStatics.GetPlayerCharacter` 0))
    (`/Engine/EditorBlueprintResources/StandardMacros.IsValid` (`/Game/Characters/BP_ActiveChar.Current Item` _asbp_active_char)
      (:`Is Valid`
        (bind _tempcurrentitem1 (`/Game/Characters/BP_ActiveChar.GiveItem` _asbp_active_char))
        (`self.K2_DestroyActor` _tempcurrentitem1)
        (`GameplayStatics.PlaySoundAtLocation` "/Game/SFX/CharacterSounds/Theif/ES_Voice_Clip_Male_170_-_SFX_Producer.ES_Voice_Clip_Male_170_-_SFX_Producer" (`self.K2_GetActorLocation`) (struct) 1.0 1.0 0.0 null null null null)
        (bind _asbp_thief (cast `/Game/Characters/BP_Thief` (`local.Overlapped Object`))
          (:`then`
            (`/Game/Characters/BP_Thief.ChickenReturned` _asbp_thief)
            (bind _outactors (`GameplayStatics.GetAllActorsOfClass` "/Game/RodgerL/BP_QuestManager.BP_QuestManager_C"))
            (for _array_element _outactors
              (message `/Game/Utility/Interfaces/BPI_Quest.QuestUpdate` _array_element "SUB")))
          (:`CastFailed`
            (`KismetSystemLibrary.PrintString` "ThiefTurnIn: thief cast failed" true true (struct :`R` 1.0 :`G` 0.743918 :`A` 1.0)))))
      (:`Is Not Valid`
        (`KismetSystemLibrary.PrintString` "ThiefeturnIn: Current Item Not Valid" true true (struct :`R` 1.0 :`G` 0.905079 :`A` 1.0) 10.0)))))

(fn `UserConstructionScript`)