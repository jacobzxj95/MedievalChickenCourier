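; BP_TutorialVolume is a level trigger that shows a tutorial popup for a chosen mechanic when the player character enters its box.
; On overlap it looks up that mechanic in the game instance's ShownTutorials map and only prints a message if it was already shown.
; Otherwise it creates a W_TutorialBase widget for that mechanic and saves it as shown through the game instance, so each tutorial appears once.
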(event `self.Box.OnComponentBeginOverlap`
  (params (OverlappedComponent :type "PrimitiveComponent Object Reference") (OtherActor :type "Actor Object Reference") (OtherComp :type "PrimitiveComponent Object Reference") (OtherBodyIndex :type Integer) (bFromSweep :type Boolean) (SweepResult :type "HitResult Structure (by ref)"))
  (if (== OtherActor (`GameplayStatics.GetPlayerCharacter` 0))
    (bind _asbp_game_instance (cast `/Game/Utility/GameModes/BP_GameInstance` (`GameplayStatics.GetGameInstance`)))
    (set `self.As BP Game Instance` _asbp_game_instance)
    (if (`BlueprintMapLibrary.Map_Find` (`/Game/Utility/GameModes/BP_GameInstance.ShownTutorials` _asbp_game_instance) (`self.E_Mechanics`))
      (`KismetSystemLibrary.PrintString` "already shown")
      (else
        (bind _returnvalue (`|CreateWidget` "/Game/UI/W_TutorialBase.W_TutorialBase_C" (`GameplayStatics.GetPlayerController` 0)))
        (bind _output_get (set `/Game/UI/W_TutorialBase.E_Mechanics` (`self.E_Mechanics`) _returnvalue))
        (`UserWidget.AddToViewport` _returnvalue 0)
        (`/Game/Utility/GameModes/BP_GameInstance.SaveTutorialPopups` (`self.As BP Game Instance`) _output_get true)))))

(fn `UserConstructionScript`)