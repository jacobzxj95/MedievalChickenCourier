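; Wall torch level object that switches its point light, flame effect and burning sound on or off through a bound toggle-torches event.
; The construction script matches light visibility to Lit, and each toggle flips that state through paired DoOnce gates.
; Torches tagged StayLit activate their flame at BeginPlay and skip flame, sound and state changes, though the toggle sets point light visibility before that check.
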(event `self.ReceiveBeginPlay`
  (add `self.ToggleTorches` (delegate `TurnOn/OffLights`))
  (if (`self.ActorHasTag` "StayLit")
    (`ActorComponent.Activate` (`self.Flame`) false)))

(event `TurnOn/OffLights`
  (bind _lit_ (`self.Lit?`))
  (bind _burningsound (`self.BurningSound`))
  (bind _flame (`self.Flame`))
  (`SceneComponent.SetHiddenInGame` (`self.PointLight`) _lit_ true)
  (if (`self.ActorHasTag` "StayLit")
    _
    (elif _lit_
      (`|ExecutionSequence`
        (:`then_0`
          (`/Engine/EditorBlueprintResources/StandardMacros.DoOnce` false :!label _label
            (:`Completed`
              (`AudioComponent.Stop` _burningsound)
              (`ActorComponent.Deactivate` _flame)
              (set `self.Lit?` false))))
        (:`then_1`
          (goto _label_2 :!via `Reset`)))
      (else
        (`|ExecutionSequence`
          (:`then_0`
            (goto _label :!via `Reset`))
          (:`then_1`
            (`/Engine/EditorBlueprintResources/StandardMacros.DoOnce` false :!label _label_2
              (:`Completed`
                (`AudioComponent.Play` _burningsound 0.0)
                (`ActorComponent.Activate` _flame true)
                (set `self.Lit?` true)))))))))

(event `self.ReceiveTick`
  (params (DeltaSeconds :type "Float (single-precision)")))

(fn `UserConstructionScript`
  (bind _pointlight (`self.PointLight`))
  (if (`self.Lit?`)
    (`SceneComponent.SetHiddenInGame` _pointlight false true)
    (else
      (`SceneComponent.SetHiddenInGame` _pointlight true true))))