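; BP_WaterSurface is a level object that plays splash feedback when actors enter or leave its box volume.
; Entering plays an enter sound and spawns a splash effect at the actor's location, throttled by a DoOnce that resets after a short delay.
; Leaving plays an exit sound and the same effect unthrottled, oriented by the actor's up vector rather than the sweep impact point used on entry.
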(event `self.Box.OnComponentBeginOverlap`
  (params (OverlappedComponent :type "PrimitiveComponent Object Reference") (OtherActor :type "Actor Object Reference") (OtherComp :type "PrimitiveComponent Object Reference") (OtherBodyIndex :type Integer) (bFromSweep :type Boolean) (SweepResult :type "HitResult Structure (by ref)"))
  (bind _returnvalue (`self.K2_GetActorLocation` OtherActor))
  (`/Engine/EditorBlueprintResources/StandardMacros.DoOnce` false :!label _label
    (:`Completed`
      (`GameplayStatics.PlaySoundAtLocation` "/Game/SFX/Environment/SC_EnterWaterSplash.SC_EnterWaterSplash" _returnvalue (struct) 1.0 1.0 0.0 null null null null)
      (`NiagaraFunctionLibrary.SpawnSystemAtLocation` "/Game/Art/VFX/VFX_WaterSplash.VFX_WaterSplash" _returnvalue (`KismetMathLibrary.MakeRotFromZ` SweepResult_ImpactPoint))
      (`KismetSystemLibrary.Delay` 0.1)
      (`self.ResetDoOnce`))))

(event `ResetDoOnce`
  (goto _label :!via `Reset`))

(event `self.Box.OnComponentEndOverlap`
  (params (OverlappedComponent :type "PrimitiveComponent Object Reference") (OtherActor :type "Actor Object Reference") (OtherComp :type "PrimitiveComponent Object Reference") (OtherBodyIndex :type Integer))
  (bind _returnvalue (`self.K2_GetActorLocation` OtherActor))
  (`GameplayStatics.PlaySoundAtLocation` "/Game/SFX/Environment/SC_ExitWaterSplash.SC_ExitWaterSplash" _returnvalue (struct) 1.0 1.0 0.5 null null null null)
  (`NiagaraFunctionLibrary.SpawnSystemAtLocation` "/Game/Art/VFX/VFX_WaterSplash.VFX_WaterSplash" _returnvalue (`KismetMathLibrary.MakeRotFromZ` (`self.GetActorUpVector` OtherActor))))

(fn `UserConstructionScript`)