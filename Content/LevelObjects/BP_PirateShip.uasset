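; BP_PirateShip is a quest-objective ship that sinks when a catapult-launched AI chicken hits it.
; The impact plays explosion and barrel-break effects, swaps in a sunk mesh, sends the quest ID, and eases the ship down with a tilt.
; It then reports the sinking to the game instance through the game mode and destroys itself.
; An objective-icon widget created by the quest-item component is shown or hidden by matching waypoint IDs.
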(event `self.ReceiveBeginPlay`
  (bind _output_get (`/Game/Components/ActorComponents/AC_Questitem.CreateWidget` (`self.AC_Questitem`)))
  (`WidgetComponent.SetWidget` (`self.Widget`) _output_get)
  (bind _output_get_2 (set `self.MainObjectiveIcon` _output_get))
  (`/Game/UI/Icons/W_MainObjectiveIcon.TurnOnObjectiveIcon` _output_get_2 3))

(event `self.StaticMesh.OnComponentHit`
  (params (HitComponent :type "PrimitiveComponent Object Reference") (OtherActor :type "Actor Object Reference") (OtherComp :type "PrimitiveComponent Object Reference") (NormalImpulse :type "Vector Structure") (Hit :type "HitResult Structure (by ref)"))
  (bind _defaultsceneroot (`self.DefaultSceneRoot`))
  (bind (_returnvalue_x _returnvalue_y) (`KismetMathLibrary.BreakVector` (`SceneComponent.K2_GetComponentLocation` _defaultsceneroot)))
  (if (== "/Game/AI/AICharacters/BP_AI_Chicken.BP_AI_Chicken_C" (`GameplayStatics.GetObjectClass` OtherActor))
    (bind _asbp_ai_chicken (cast `/Game/AI/AICharacters/BP_AI_Chicken` OtherActor))
    (if (`/Game/AI/AICharacters/BP_AI_Chicken.Catapult Launched?` _asbp_ai_chicken)
      (`GameplayStatics.PlaySoundAtLocation` "/Game/SFX/Mechanics/Catapult/SC_ShortExplosion.SC_ShortExplosion" Hit_Location (struct) 1.0 1.0 0.0 null null null null)
      (`NiagaraFunctionLibrary.SpawnSystemAtLocation` "/Game/Art/VFX/VFX_BarrelBreak.VFX_BarrelBreak" Hit_Location (struct) (2.0 2.0 2.0))
      ;[0 0.8924 1] Sink ship
      (`StaticMeshComponent.SetStaticMesh` (`self.StaticMesh`) "/Game/Meshes/Boats/SunkShip__2_.SunkShip__2_")
      (`GameplayStatics.PlaySoundAtLocation` "/Game/SFX/Mechanics/Catapult/SC_LargeExplosion.SC_LargeExplosion" (`self.K2_GetActorLocation`) (struct) 1.0 1.0 0.0 null null null null)
      (`/Game/Components/ActorComponents/AC_Questitem.Send ID` (`self.AC_Questitem`) 0)
      (`KismetSystemLibrary.MoveComponentTo` _defaultsceneroot (`KismetMathLibrary.MakeVector` _returnvalue_x _returnvalue_y -1220.0) (struct :`Pitch` -30.0) true true 3.0)
      ;[1 1 1] Inform the game instance of the sunken ship and then destroy self
      (bind _output_get (set `self.ShipSunk?` true))
      (bind _game_instance (message `/Game/Utility/Interfaces/BPI_UI.Pass Out Game Instance Ref` (`GameplayStatics.GetGameMode`)))
      (message `/Game/Utility/Interfaces/BPI_Objective.PrimaryObjective` _game_instance false false 0 _output_get)
      (`self.K2_DestroyActor`))))

(event `/Game/Utility/Interfaces/BPI_Quest.TurnOnWaypoints`
  (params (ObjectiveID :type String) (`On/Off` :type Boolean))
  (for _array_element (`/Game/Components/ActorComponents/AC_Questitem.ActorQuestIDS` (`self.AC_Questitem`))
    (if (`KismetStringLibrary.EqualEqual_StrStr` ObjectiveID _array_element)
      (if `On/Off`
        (`SceneComponent.SetHiddenInGame` (`self.Widget`) false false)
        (else
          (`SceneComponent.SetHiddenInGame` (`self.Widget`) true false))))))

(fn `UserConstructionScript`)