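; Game mode for the chicken-quest game that acts as the central UI manager and quest-to-HUD relay.
; BeginPlay creates the game's widgets up front, retries until the player character exists, then restores currency and quest data from the game instance and shows a post-loss screen if the last quest failed.
; Enum-driven TurnOn/TurnOffWidget functions handle viewport, pause, cursor and input mode, tracking open widgets in an array.
; Events forward quest, objective and currency updates to the HUD.
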(event `self.ReceiveBeginPlay`
  (bind _returnvalue (`GameplayStatics.GetPlayerController` 0))
  ;[1 0.1309 0.001194] Begin play
  (`|ExecutionSequence`
    (:`then_0`
      (`KismetSystemLibrary.Delay` 1.0 :!label _label)
      (bind _asbp_player_char (cast `/Game/Characters/BP_PlayerChar` (`GameplayStatics.GetPlayerCharacter` 0))
        (:`then`
          (bind _output_get (set `self.PlayerChar` _asbp_player_char))
          (message `/Game/Utility/Interfaces/BPI_UI.TurnOnUI` _output_get "NewEnumerator0")
          (bind _asbp_game_instance (cast `/Game/Utility/GameModes/BP_GameInstance` (`GameplayStatics.GetGameInstance`)))
          (bind _output_get_2 (set `self.Game Instance` _asbp_game_instance))
          (set `self.PlayerStartTag` (`/Game/Utility/GameModes/BP_GameInstance.PlayerStartTag` _output_get_2))
          (bind _asbp_game_instance_2 (cast `/Game/Utility/GameModes/BP_GameInstance` (`GameplayStatics.GetGameInstance`)))
          (if (not (not (`/Game/Utility/GameModes/BP_GameInstance.QuestFailed` _asbp_game_instance_2)))
            (bind _returnvalue_2 (`|CreateWidget` "/Game/UI/WBP_PostlostUI.WBP_PostlostUI_C" _returnvalue))
            (set `/Game/UI/WBP_PostlostUI.LossCondition` (`/Game/Utility/GameModes/BP_GameInstance.LossCondition` _asbp_game_instance_2) _returnvalue_2)
            (`UserWidget.AddToViewport` _returnvalue_2 0)
            (`WidgetBlueprintLibrary.SetInputMode_UIOnlyEx` _returnvalue _returnvalue_2)
            (set `PlayerController.bShowMouseCursor` true _returnvalue)
            (set `/Game/Utility/GameModes/BP_GameInstance.QuestFailed` false _asbp_game_instance_2)
            (`GameplayStatics.SetGamePaused` true)))
        (:`CastFailed`
          (goto _label))))
    (:`then_1`
      (`|ExecutionSequence`
        (:`then_0`
          (bind _returnvalue_3 (`|CreateWidget` "/Game/UI/W_HUD.W_HUD_C" (`GameplayStatics.GetPlayerController` 0)))
          (set `self.PlayerHUD` _returnvalue_3)
          (bind _returnvalue_4 (`|CreateWidget` "/Game/UI/W_Lose.W_Lose_C" (`GameplayStatics.GetPlayerController` 0)))
          (set `self.LossUI` _returnvalue_4))
        (:`then_1`
          (bind _returnvalue_5 (`|CreateWidget` "/Game/UI/W_TemperMeter.W_TemperMeter_C" (`GameplayStatics.GetPlayerController` 0)))
          (set `self.ChickenTemperMeter` _returnvalue_5)
          (bind _returnvalue_6 (`|CreateWidget` "/Game/UI/W_Vendor.W_Vendor_C" (`GameplayStatics.GetPlayerController` 0)))
          (set `self.VendorUI` _returnvalue_6))
        (:`then_2`
          (bind _returnvalue_7 (`|CreateWidget` "/Game/UI/Menus/W_PauseMenu.W_PauseMenu_C" (`GameplayStatics.GetPlayerController` 0)))
          (set `self.PauseUI` _returnvalue_7)
          (bind _returnvalue_8 (`|CreateWidget` "/Game/UI/Dialogue/W_QuestDialogue.W_QuestDialogue_C" (`GameplayStatics.GetPlayerController` 0)))
          (set `self.QuestDialogueUI` _returnvalue_8))
        (:`then_3`
          (bind _returnvalue_9 (`|CreateWidget` "/Game/UI/W_Win.W_Win_C" (`GameplayStatics.GetPlayerController` 0)))
          (set `self.WinUI` _returnvalue_9))
        (:`then_4`
          (bind _returnvalue_10 (`|CreateWidget` "/Game/UI/Icons/W_MainObjectiveIcon.W_MainObjectiveIcon_C" (`GameplayStatics.GetPlayerController` 0)))
          (set `self.MainObjectiveRef` _returnvalue_10)
          (bind _returnvalue_11 (`|CreateWidget` "/Game/UI/W_Wager.W_Wager_C" (`GameplayStatics.GetPlayerController` 0)))
          (set `self.WagerUI_Ref` _returnvalue_11))
        (:`then_5`
          (bind _returnvalue_12 (`|CreateWidget` "/Game/UI/LevelSequences/W_SequencerProgressBar.W_SequencerProgressBar_C" (`GameplayStatics.GetPlayerController` 0)))
          (set `self.SequenceSkipBarRef` _returnvalue_12)
          (bind _returnvalue_13 (`|CreateWidget` "/Game/UI/LevelSequences/W_SequencerSkipText.W_SequencerSkipText_C" (`GameplayStatics.GetPlayerController` 0)))
          (set `self.SequencerSkipText` _returnvalue_13))
        (:`then_6`
          (bind _returnvalue_14 (`|CreateWidget` "/Game/UI/W_KeepMovingPrompt.W_KeepMovingPrompt_C" (`GameplayStatics.GetPlayerController` 0)))
          (set `self.KeepMovingPrompts` _returnvalue_14)
          (bind _returnvalue_15 (`|CreateWidget` "/Game/UI/Dialogue/W_IntroDialogue.W_IntroDialogue_C" (`GameplayStatics.GetPlayerController` 0)))
          (set `self.IntoDialogue` _returnvalue_15))
        (:`then_7`
          (bind _returnvalue_16 (`|CreateWidget` "/Game/UI/Dialogue/W_KingsDialogue.W_KingsDialogue_C" (`GameplayStatics.GetPlayerController` 0)))
          (set `self.KingsDialogueUI` _returnvalue_16)
          (bind _returnvalue_17 (`|CreateWidget` "/Game/UI/Menus/W_Credits.W_Credits_C" (`GameplayStatics.GetPlayerController` 0)))
          (set `self.CreditsUI` _returnvalue_17))
        (:`then_8`
          (bind _returnvalue_18 (`|CreateWidget` "/Game/UI/Icons/WBP_HoningTimer_Icon.WBP_HoningTimer_Icon_C" (`GameplayStatics.GetPlayerController` 0)))
          (set `self.HoningTimer_Icon` _returnvalue_18)
          (bind _returnvalue_19 (`|CreateWidget` "/Game/UI/W_Catapult.W_Catapult_C" (`GameplayStatics.GetPlayerController` 0)))
          (set `self.CatapultUI` _returnvalue_19))
        (:`then_9`
          (bind _returnvalue_20 (`|CreateWidget` "/Game/UI/W_TutorialBase.W_TutorialBase_C" (`GameplayStatics.GetPlayerController` 0)))
          (set `self.TutorialUI` _returnvalue_20))
        (:`then_10`
          (bind _returnvalue_21 (`|CreateWidget` "/Game/UI/W_LevelExitConfirmation.W_LevelExitConfirmation_C" (`GameplayStatics.GetPlayerController` 0)))
          (set `self.LevelExitConfirmation` _returnvalue_21))
        (:`then_11`
          (bind _returnvalue_22 (`|CreateWidget` "/Game/AI/HoningChicken/VFX/WBP_TimerIndicator.WBP_TimerIndicator_C" (`GameplayStatics.GetPlayerController` 0)))
          (set `self.Timing Indicator` _returnvalue_22)
          (bind _current_player_save_data (`self.LoadPlayerData`))
          (`/Game/UI/W_HUD.LoadHudData` (`self.PlayerHUD`) (break `/Game/Utility/Struct/STR_PlayerSaveData` _current_player_save_data))
          (bind _game_instance (`self.Game Instance`)
            (:`then`
              (`self.Loaded` (`/Game/Utility/GameModes/BP_GameInstance.Has Object Been Turned in` _game_instance))
              (bind _returnvalue_23 (`GameplayStatics.GetCurrentLevelName` true))
              (bind (_value _returnvalue_24) (`BlueprintMapLibrary.Map_Find` (`/Game/Utility/GameModes/BP_GameInstance.CompletedQuests` _game_instance) _returnvalue_23))
              (if _returnvalue_24
                (`self.QuestDataLoad` _value)))
            (:`else`)))
        (:`then_12`
          (bind _returnvalue_25 (`|CreateWidget` "/Game/UI/Icons/WBP_Pushback_Cooldown_Icon.WBP_Pushback_Cooldown_Icon_C" (`GameplayStatics.GetPlayerController` 0)))
          (set `self.WBP Pushback` _returnvalue_25))
        (:`then_13`
          (bind _returnvalue_26 (`|CreateWidget` "/Game/UI/WBP_ChickenStolen.WBP_ChickenStolen_C" (`GameplayStatics.GetPlayerController` 0)))
          (set `self.WBP Chicken Stolen` _returnvalue_26))))))

(event `/Game/Utility/Interfaces/BPI_UI.TurnOnUI`
  (params (`UI to turn On` :type "/Game/Utility/Enums/E_UI Enum" :default "NewEnumerator0"))
  ;[0 0.2912 1] Turn on UI
  (bind _currentonui (`self.TurnOnWidget` `UI to turn On`))
  (`KismetArrayLibrary.Array_AddUnique` (`self.CurrentOnWidgets`) _currentonui))

(event `/Game/Utility/Interfaces/BPI_UI.TurnOffUI`
  (params (`UI to turn off` :type "/Game/Utility/Enums/E_UI Enum" :default "NewEnumerator0"))
  ;[0 0.2912 1] Turn off UI
  (`self.TurnOffWidget` `UI to turn off`))

(event `/Game/Utility/Interfaces/BPI_UI.Set Command Points Interface`
  (`/Game/UI/W_HUD.Set command points upon purchase` (`self.PlayerHUD`)))

(event `/Game/Utility/Interfaces/BPI_UI.TurnOffAnyCurrentlyOnUI`
  (bind _currentonwidgets (`self.CurrentOnWidgets`))
  (if (`KismetArrayLibrary.Array_IsNotEmpty` _currentonwidgets)
    (for _array_element _currentonwidgets
      (`/Engine/EditorBlueprintResources/StandardMacros.IsValid` _array_element
        (:`Is Valid`
          (`Widget.RemoveFromParent` _array_element)
          (`self.RemoveWidgetArrayElement` _array_element))))
    (`WidgetBlueprintLibrary.SetInputMode_GameOnly` (`GameplayStatics.GetPlayerController` 0))
    (else
      (`KismetSystemLibrary.PrintString` "array empty"))))

(event `/Game/Utility/Interfaces/BPI_UI.Spend Command Point`
  (`/Game/UI/W_HUD.Spend Command Point ` (`self.PlayerHUD`)))

(event `/Game/Utility/Interfaces/BPI_UI.UpdateCurrency`
  (params (Currency :type Integer))
  (bind _playerhud (`self.PlayerHUD`))
  ;[0 0.2912 1] Update UI currency value
  (`/Game/UI/W_HUD.Add Coins` _playerhud Currency)
  (set `self.Total Currency` (`/Game/UI/W_HUD.CurrencyTotal` _playerhud)))

(event `SetupPlayerHUD`
  (bind _playerhud (`self.PlayerHUD`))
  (bind ((`CurrentChickens_16_1E480401441CFD2FA8B886A1BB233B78` _currentchickens) (`ChickensNeeded_6_F8F4553D4DE63061106E328A97F62BC7` _chickensneeded) (`MyQuestMarker_43_A5DB8E164FBE16167027A0973E042D41` _myquestmarker)) (break `/Game/Utility/Struct/STR_Quest` (`self.ActiveQuestInfo`)))
  ;[0 1 0.05664] PlayerHUD
  (for _array_element _myquestmarker
    (bind _asw_main_objective_icon (cast `/Game/UI/Icons/W_MainObjectiveIcon` (`WidgetComponent.GetWidget` (`/Game/LevelObjects/QuestRelated/BP_MainObjectiveIcon.ChickenIcon` _array_element))))
    (`Widget.SetVisibility` (`/Game/UI/Icons/W_MainObjectiveIcon.ChickenIcon` _asw_main_objective_icon) "Visible")
    (`Widget.SetVisibility` (`/Game/UI/Icons/W_MainObjectiveIcon.InactiveQuestIcon` _asw_main_objective_icon) "Hidden"))
  (set `/Game/UI/W_HUD.ChickensCollected` _currentchickens _playerhud)
  (set `/Game/UI/W_HUD.ChickensTotal` _chickensneeded _playerhud)
  (`Widget.SetVisibility` (`/Game/UI/W_HUD.HorizontalBox_0` (`self.PlayerHUD`)) "Visible"))

(event `/Game/Utility/Interfaces/BPI_UI.UpdatePlayerStats`
  (params (PlayerStats :type "Map of /Game/Utility/Enums/E_PlayerStats Enum to Float (double-precision)" :default _))
  ;[0 1 0.05664] Player Stat's Update
  (set `/Game/UI/W_TemperMeter.HandlingDuration` (`BlueprintMapLibrary.Map_Find` PlayerStats "NewEnumerator2") (`self.ChickenTemperMeter`)))

(event `/Game/Utility/Interfaces/BPI_UI.QuestCompleted`
  (params (IsGoldenChickenQuest :type Boolean))
  ;[1 1 1] Quest Interfaces
  (`/Game/UI/W_HUD.QuestCompleted` (`self.PlayerHUD`))
  (`/Game/UI/Menus/W_PauseMenu.TurnOnGoldenChickenReaction` (`self.PauseUI`) IsGoldenChickenQuest))

(event `/Game/Utility/Interfaces/BPI_UI.QuestStarted`
  (params (`Quest Actor` :type "/Game/RodgerL/BP_QuestManager Object Reference"))
  ;[1 1 1] Quest Interfaces
  (`/Game/UI/W_HUD.QuestBegan` (`self.PlayerHUD`) `Quest Actor`))

(event `/Game/Utility/Interfaces/BPI_UI.Update UI Upon Turnin`
  (params (NewObjectiveNumber :type Integer) (ObjectiveDetails :type "/Game/Utility/Struct/STR_ObjectiveDetails Structure"))
  ;[1 1 1] Quest Interfaces
  (`/Game/UI/W_HUD.UpdateObjective` (`self.PlayerHUD`) NewObjectiveNumber ObjectiveDetails))

(event `/Game/Utility/Interfaces/BPI_UI.StageCompleted`
  (params (`New Stage Details` :type "/Game/Utility/Struct/STR_StageDetails Structure"))
  ;[1 1 1] Quest Interfaces
  (`/Game/UI/W_HUD.Stage Completed` (`self.PlayerHUD`) `New Stage Details`))

(event `/Game/Utility/Interfaces/BPI_UI.ObjectiveCompleted`
  (params (NewObjective :type "/Game/Utility/Struct/STR_ObjectiveDetails Structure"))
  ;[1 1 1] Quest Interfaces
  (`/Game/UI/W_HUD.ObjectiveCompleted` (`self.PlayerHUD`) NewObjective))

(event `/Game/Utility/Interfaces/BPI_UI.QuestFailed`
  ;[1 1 1] Quest Interfaces
  (`self.TurnOffWidget` "NewEnumerator0")
  (`self.TurnOnWidget` "NewEnumerator1"))

(event `/Game/Utility/Interfaces/BPI_UI.LossCondition`
  (params (NewLossState :type Integer))
  (`/Game/UI/W_HUD.LossCondition` (`self.PlayerHUD`) NewLossState))

(fn `GetDefaultPawnClassForController`
  (params (InController :type "Controller Object Reference"))
  (returns (ReturnValue :type "Object Class Reference"))
  (bind _returnvalue (`parent.GetDefaultPawnClassForController` InController))
  (return _returnvalue))

(fn `LoadPlayerData`
  (returns (`Current Player Save Data` :type "/Game/Utility/Struct/STR_PlayerSaveData Structure"))
  (bind _game_instance (`self.Game Instance`)
    (:`then`
      (return (`/Game/Utility/GameModes/BP_GameInstance.PlayerSaveData` _game_instance)))
    (:`else`)))

(fn `Pass Out Game Instance Ref`
  (returns (`Game Instance` :type "/Game/Utility/GameModes/BP_GameInstance Object Reference"))
  (return (`self.Game Instance`)))

(fn `Pass Out Playercharacter ref`
  (returns (PlayerCharacterRef :type "/Game/Characters/BP_PlayerChar Object Reference"))
  (bind _playerchar (`self.PlayerChar`)
    (:`then`
      (return _playerchar))
    (:`else`)))

(fn `RemoveWidgetArrayElement`
  (params (Widget :type "Widget Object Reference (by ref)"))
  (if (`KismetArrayLibrary.Array_Contains` (`self.CurrentOnWidgets`) Widget)
    (bind _returnvalue (`KismetArrayLibrary.Array_RemoveItem` (`self.CurrentOnWidgets`) Widget))
    (`KismetSystemLibrary.PrintString` (`KismetStringLibrary.Concat_StrStr` (`KismetStringLibrary.Conv_BoolToString` _returnvalue) "Widget Array Item Removed"))))

(fn `TurnOffWidget`
  (params (Selection :type "/Game/Utility/Enums/E_UI Enum" :default "NewEnumerator0"))
  (bind _returnvalue (`GameplayStatics.GetPlayerController` 0))
  (bind _returnvalue_2 (`GameplayStatics.GetPlayerController` 0))
  (bind _returnvalue_3 (`GameplayStatics.GetPlayerController` 0))
  (bind _returnvalue_4 (`GameplayStatics.GetPlayerController` 0))
  (bind _returnvalue_5 (`GameplayStatics.GetPlayerController` 0))
  (bind _lossui (`self.LossUI`))
  (bind _pauseui (`self.PauseUI`))
  (bind _winui (`self.WinUI`))
  (switch `/Game/Utility/Enums/E_UI` Selection
    (:`NewEnumerator0`
      (bind _playerhud (`self.PlayerHUD`)
        (:`then`
          (`Widget.RemoveFromParent` _playerhud)
          (set `self.PlayerHUDOFF` true))
        (:`else`)))
    (:`NewEnumerator1`
      (`Widget.RemoveFromParent` _lossui)
      (set `PlayerController.bShowMouseCursor` false _returnvalue)
      (`WidgetBlueprintLibrary.SetInputMode_GameOnly` _returnvalue)
      (`self.RemoveWidgetArrayElement` _lossui))
    (:`NewEnumerator2`
      (bind _chickentempermeter (`self.ChickenTemperMeter`)
        (:`then`
          (`Widget.RemoveFromParent` _chickentempermeter)
          (`self.RemoveWidgetArrayElement` _chickentempermeter))
        (:`else`)))
    (:`NewEnumerator3`
      (bind _vendorui (`self.VendorUI`)
        (:`then`
          (`Widget.RemoveFromParent` _vendorui)
          (`WidgetBlueprintLibrary.SetInputMode_GameOnly` _returnvalue_4)
          (set `PlayerController.bShowMouseCursor` false _returnvalue_4)
          (set `self.VendorUION` false)
          (`self.RemoveWidgetArrayElement` _vendorui))
        (:`else`)))
    (:`NewEnumerator4`
      (`Widget.RemoveFromParent` _pauseui)
      (`GameplayStatics.SetGamePaused` false)
      (set `PlayerController.bShowMouseCursor` false _returnvalue_3)
      (`WidgetBlueprintLibrary.SetInputMode_GameOnly` _returnvalue_3)
      (`self.RemoveWidgetArrayElement` _pauseui))
    (:`NewEnumerator7`
      (`UserWidget.AddToViewport` _winui 0)
      (`GameplayStatics.SetGamePaused` false)
      (set `PlayerController.bShowMouseCursor` false _returnvalue_5)
      (`WidgetBlueprintLibrary.SetInputMode_GameOnly` _returnvalue_5)
      (`self.RemoveWidgetArrayElement` _winui))
    (:`NewEnumerator8`
      (bind _mainobjectiveref (`self.MainObjectiveRef`)
        (:`then`
          (`Widget.RemoveFromParent` _mainobjectiveref)
          (`self.RemoveWidgetArrayElement` _mainobjectiveref))
        (:`else`)))
    (:`NewEnumerator9`
      (bind _wagerui_ref (`self.WagerUI_Ref`)
        (:`then`
          (`Widget.RemoveFromParent` _wagerui_ref)
          (set `PlayerController.bShowMouseCursor` false _returnvalue_2)
          (`WidgetBlueprintLibrary.SetInputMode_GameOnly` _returnvalue_2)
          (`self.RemoveWidgetArrayElement` _wagerui_ref))
        (:`else`)))
    (:`NewEnumerator10`
      (bind _sequenceskipbarref (`self.SequenceSkipBarRef`)
        (:`then`
          (`UserWidget.StopAnimation` _sequenceskipbarref (`/Game/UI/LevelSequences/W_SequencerProgressBar.ProgressBarPercent` _sequenceskipbarref))
          (`Widget.RemoveFromParent` _sequenceskipbarref)
          (`self.RemoveWidgetArrayElement` _sequenceskipbarref))
        (:`else`)))
    (:`NewEnumerator11`
      (bind _sequencerskiptext (`self.SequencerSkipText`)
        (:`then`
          (`UserWidget.StopAnimation` _sequencerskiptext (`/Game/UI/LevelSequences/W_SequencerSkipText.FadeInAndOut` _sequencerskiptext))
          (`Widget.RemoveFromParent` _sequencerskiptext)
          (`self.RemoveWidgetArrayElement` _sequencerskiptext))
        (:`else`)))
    (:`NewEnumerator12`
      (bind _keepmovingprompts (`self.KeepMovingPrompts`)
        (:`then`
          (`Widget.RemoveFromParent` _keepmovingprompts)
          (`self.RemoveWidgetArrayElement` _keepmovingprompts))
        (:`else`)))
    (:`NewEnumerator17`
      (bind _honingtimer_icon (`self.HoningTimer_Icon`)
        (:`then`
          (`Widget.RemoveFromParent` _honingtimer_icon)
          (`self.RemoveWidgetArrayElement` _honingtimer_icon))
        (:`else`)))
    (:`NewEnumerator19`
      (bind _wbp_pushback (`self.WBP Pushback`)
        (:`then`
          (`Widget.RemoveFromParent` _wbp_pushback)
          (`self.RemoveWidgetArrayElement` _wbp_pushback))
        (:`else`)))
    (:`NewEnumerator20`
      (bind _catapultui (`self.CatapultUI`)
        (:`then`
          (`Widget.RemoveFromParent` _catapultui)
          (`self.RemoveWidgetArrayElement` _catapultui))
        (:`else`)))
    (:`NewEnumerator21`
      (bind _wbp_chicken_stolen (`self.WBP Chicken Stolen`)
        (:`then`
          (`Widget.RemoveFromParent` _wbp_chicken_stolen)
          (`self.RemoveWidgetArrayElement` _wbp_chicken_stolen))
        (:`else`)))
    (:`NewEnumerator22`
      (bind _levelexitconfirmation (`self.LevelExitConfirmation`)
        (:`then`
          (`Widget.RemoveFromParent` _levelexitconfirmation)
          (`WidgetBlueprintLibrary.SetInputMode_GameOnly` (`GameplayStatics.GetPlayerController` 0))
          (`self.RemoveWidgetArrayElement` _levelexitconfirmation))
        (:`else`)))
    (:`NewEnumerator23`
      (bind _creditsui (`self.CreditsUI`)
        (:`then`
          (`Widget.RemoveFromParent` _creditsui)
          (`self.RemoveWidgetArrayElement` _creditsui))
        (:`else`)))
    (:`NewEnumerator24`
      (bind _kingsdialogueui (`self.KingsDialogueUI`)
        (:`then`
          (`Widget.RemoveFromParent` _kingsdialogueui)
          (`self.RemoveWidgetArrayElement` _kingsdialogueui))
        (:`else`)))))

(fn `TurnOnWidget`
  (params (Selection :type "/Game/Utility/Enums/E_UI Enum" :default "NewEnumerator0"))
  (returns (CurrentOnUI :type "Widget Object Reference"))
  (bind _returnvalue (`GameplayStatics.GetPlayerController` 0))
  (bind _returnvalue_2 (`GameplayStatics.GetPlayerController` 0))
  (bind _returnvalue_3 (`GameplayStatics.GetPlayerController` 0))
  (bind _returnvalue_4 (`GameplayStatics.GetPlayerController` 0))
  (bind _returnvalue_5 (`GameplayStatics.GetPlayerController` 0))
  (bind _honingtimer_icon (`self.HoningTimer_Icon`))
  (bind _wbp_pushback (`self.WBP Pushback`))
  (bind _pauseui (`self.PauseUI`))
  (bind _vendorui (`self.VendorUI`))
  (bind _wagerui_ref (`self.WagerUI_Ref`))
  (bind _lossui (`self.LossUI`))
  (bind _winui (`self.WinUI`))
  (bind _chickentempermeter (`self.ChickenTemperMeter`))
  (bind _keepmovingprompts (`self.KeepMovingPrompts`))
  (switch `/Game/Utility/Enums/E_UI` Selection
    (:`NewEnumerator0`
      (bind _playerhud (`self.PlayerHUD`)
        (:`then`
          (`UserWidget.AddToViewport` _playerhud 0))
        (:`else`)))
    (:`NewEnumerator1`
      (`UserWidget.AddToViewport` _lossui 0)
      (`GameplayStatics.SetGamePaused` true)
      (set `PlayerController.bShowMouseCursor` true _returnvalue_3)
      (`WidgetBlueprintLibrary.SetInputMode_UIOnlyEx` _returnvalue_3 _lossui)
      (return _lossui))
    (:`NewEnumerator2`
      (`UserWidget.AddToViewport` _chickentempermeter 0)
      (return _chickentempermeter))
    (:`NewEnumerator3`
      (`UserWidget.AddToViewport` _vendorui 0)
      (set `PlayerController.bShowMouseCursor` true _returnvalue_5)
      (`WidgetBlueprintLibrary.SetInputMode_GameAndUIEx` _returnvalue_5 _vendorui)
      (set `self.VendorUION` true)
      (return _vendorui))
    (:`NewEnumerator4`
      (`UserWidget.AddToViewport` _pauseui 0)
      (`GameplayStatics.SetGamePaused` true)
      (set `PlayerController.bShowMouseCursor` true _returnvalue_2)
      (`WidgetBlueprintLibrary.SetInputMode_UIOnlyEx` _returnvalue_2 _pauseui)
      (return _pauseui))
    (:`NewEnumerator7`
      (`UserWidget.AddToViewport` _winui 0)
      (`GameplayStatics.SetGamePaused` true)
      (set `PlayerController.bShowMouseCursor` true _returnvalue_4)
      (`WidgetBlueprintLibrary.SetInputMode_UIOnlyEx` _returnvalue_4 _winui)
      (return _winui))
    (:`NewEnumerator8`
      (`UserWidget.AddToViewport` (`self.MainObjectiveRef`) 0))
    (:`NewEnumerator9`
      (set `/Game/UI/W_Wager.TotalCurrency` (`self.Total Currency`) (`self.WagerUI_Ref`))
      (`UserWidget.AddToViewport` _wagerui_ref 0)
      (set `PlayerController.bShowMouseCursor` true _returnvalue)
      (`WidgetBlueprintLibrary.SetInputMode_GameAndUIEx` _returnvalue _wagerui_ref)
      (return _wagerui_ref))
    (:`NewEnumerator10`
      (bind _sequenceskipbarref (`self.SequenceSkipBarRef`)
        (:`then`
          (`UserWidget.AddToViewport` _sequenceskipbarref 0)
          (return _sequenceskipbarref))
        (:`else`)))
    (:`NewEnumerator11`
      (bind _sequencerskiptext (`self.SequencerSkipText`)
        (:`then`
          (`UserWidget.AddToViewport` _sequencerskiptext 0)
          (return _sequencerskiptext))
        (:`else`)))
    (:`NewEnumerator12`
      (`UserWidget.AddToViewport` _keepmovingprompts 0)
      (return _keepmovingprompts))
    (:`NewEnumerator17`
      (`UserWidget.AddToViewport` _honingtimer_icon 0)
      (return _honingtimer_icon))
    (:`NewEnumerator19`
      (`UserWidget.AddToViewport` _wbp_pushback 0)
      (return _wbp_pushback))
    (:`NewEnumerator20`
      (bind _catapultui (`self.CatapultUI`)
        (:`then`
          (`UserWidget.AddToViewport` _catapultui 0)
          (return _catapultui))
        (:`else`)))
    (:`NewEnumerator21`
      (bind _wbp_chicken_stolen (`self.WBP Chicken Stolen`)
        (:`then`
          (`UserWidget.AddToViewport` _wbp_chicken_stolen 0)
          (return _wbp_chicken_stolen))
        (:`else`)))
    (:`NewEnumerator22`
      (bind _levelexitconfirmation (`self.LevelExitConfirmation`)
        (:`then`
          (`UserWidget.AddToViewport` _levelexitconfirmation 0)
          (`WidgetBlueprintLibrary.SetInputMode_UIOnlyEx` (`GameplayStatics.GetPlayerController` 0) _levelexitconfirmation)
          (return _levelexitconfirmation))
        (:`else`)))
    (:`NewEnumerator23`
      (bind _creditsui (`self.CreditsUI`)
        (:`then`
          (`UserWidget.AddToViewport` _creditsui 0)
          (return _creditsui))
        (:`else`)))
    (:`NewEnumerator24`
      (bind _kingsdialogueui (`self.KingsDialogueUI`)
        (:`then`
          (`UserWidget.AddToViewport` _kingsdialogueui 0)
          (return _kingsdialogueui))
        (:`else`)))))

(fn `UserConstructionScript`)